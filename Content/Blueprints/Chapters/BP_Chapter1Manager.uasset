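; Chapter 1 manager Blueprint that sets up the opening screen fade and soundscape for the first level.
; InitializeLevel1 runs FadeIn on the fade screen component, then spawns night ambience through the level's BP_AmbienceSound and starts people-talking audio on every BP_HouseTalking actor.
; StartGame only casts the player character to BP_FirstPersonCharacter, with no further logic attached.
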(event `Start Game`
  (cast `/Game/FirstPerson/Blueprints/BP_FirstPersonCharacter` (`GameplayStatics.GetPlayerCharacter` 0)))

(event `Initialize Level 1`
  (`/Game/Blueprints/Components/BP_FadeScreenComponent.Fade In` (`self.BP_FadeScreenComponent`) (`self.Player Ref`))
  (`|ExecutionSequence`
    (:`then_0`
      (bind _returnvalue (`GameplayStatics.GetActorOfClass` "/Game/Blueprints/Levels/BP_AmbienceSound.BP_AmbienceSound_C"))
      (bind _output_get (set `self.Ambience` _returnvalue))
      (`/Game/Blueprints/Levels/BP_AmbienceSound.Spawn Night Ambience` _output_get 0.01))
    (:`then_1`
      (bind _outactors (`GameplayStatics.GetAllActorsOfClass` "/Game/Blueprints/EventItems/BP_HouseTalking.BP_HouseTalking_C"))
      (for _array_element _outactors
        (`/Game/Blueprints/EventItems/BP_HouseTalking.Play People Talking` _array_element true)))))

(fn `UserConstructionScript`
  (`parent.UserConstructionScript`))