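; Chapter 5 manager that runs a timed scare script involving Ryan's door, cooking sounds, the television and a peeping Father.
; PlayChapter5 is one linear chain of validity checks and delays, so a missing actor halts the rest.
; It builds to crying, basketball and TV disturbance effects, then silences them and plays the Anim_CrazyDisturbance level sequence.
; When the sequence finishes, PlayNextEvent readies the BasketBallSound event.
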(event `Play Chapter 5`
  ; Door opened mysteriously
  (bind _ryan_sdoor (`self.Ryan'sDoor`)
    (:`then`
      (`/Game/Blueprints/EventItems/BP_RyansRoomsDoor.Close the Door` _ryan_sdoor)
      (`KismetSystemLibrary.Delay` 10.0)
      (`/Game/Blueprints/EventItems/BP_RyansRoomsDoor.Open Door by Event` _ryan_sdoor)
      (`KismetSystemLibrary.Delay` 16.0)
      ; Cooking Sound Effect
      (bind _cookingsfx (`self.CookingSfx`)
        (:`then`
          (`/Game/Blueprints/EventItems/BP_DisturbanceSfx.Play Cooking Sfx` _cookingsfx)
          (`KismetSystemLibrary.Delay` 10.0)
          ; Television Segment
          (bind _television (`self.Television`)
            (:`then`
              (`/Game/Blueprints/EventItems/BP_Television.Turn On TV` _television)
              (`KismetSystemLibrary.Delay` 10.0)
              ; Father Peeping
              (bind _father (`self.Father`)
                (:`then`
                  (`/Game/Blueprints/EventItems/BP_FatherPeepingDoor.Peep` _father)
                  (`KismetSystemLibrary.Delay` 10.0)
                  (`/Game/Blueprints/EventItems/BP_FatherPeepingDoor.Return from peep` _father)
                  (`KismetSystemLibrary.Delay` 10.0)
                  (`/Game/Blueprints/EventItems/BP_Television.Turn Off TV` _television)
                  (`KismetSystemLibrary.Delay` 5.0)
                  (`/Game/Blueprints/EventItems/BP_DisturbanceSfx.Play Crying Sfx` _cookingsfx)
                  (`/Game/Blueprints/EventItems/BP_Television.Play Crazy Disturbance` _television)
                  (`/Game/Blueprints/EventItems/BP_DisturbanceSfx.Play Basketball Sfx` _cookingsfx)
                  (`KismetSystemLibrary.Delay` 20.0)
                  (`|ExecutionSequence`
                    (:`then_0`
                      (`/Game/Blueprints/EventItems/BP_DisturbanceSfx.Stop All Sounds` _cookingsfx))
                    (:`then_1`
                      (`/Game/Blueprints/EventItems/BP_Television.Turn Off TV` _television))
                    (:`then_2`
                      (bind (_outactor _returnvalue) (`LevelSequencePlayer.CreateLevelSequencePlayer` "/Game/Animation/Anim_CrazyDisturbance.Anim_CrazyDisturbance"))
                      (`MovieSceneSequencePlayer.Play` _returnvalue)
                      (add `MovieSceneSequencePlayer.OnFinished` _returnvalue (delegate `Play Next Event`)))))
                (:`else`)))
            (:`else`)))
        (:`else`)))
    (:`else`)))

(event `Play Next Event`
  (bind _basketballsound (`self.BasketBallSound`)
    (:`then`
      (`/Game/Blueprints/EventItems/BP_BasketballSoundInTheRoom.Set Event Ready` _basketballsound))
    (:`else`)))

(fn `UserConstructionScript`
  (`parent.UserConstructionScript`))