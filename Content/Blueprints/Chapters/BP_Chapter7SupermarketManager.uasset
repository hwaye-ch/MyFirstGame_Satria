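; Chapter 7 supermarket manager Blueprint that sets up the player's start in the supermarket level.
; On InitializeChapter7Supermarket, it runs a black-screen fade-in through the BPFadeScreenComponent for the player.
; It then teleports the player to the location and rotation of the SpawnArea_Kasir actor found in the level, keeping the player's own scale.
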(event `Initialize Chapter 7 Supermarket`
  (bind _player_ref (`self.Player Ref`))
  (`|ExecutionSequence`
    (:`then_0`
      (`/Game/Blueprints/Components/BP_FadeScreenComponent.Black Screen then Fade In` (`self.BP_FadeScreenComponent`) (`self.Player Ref`) 3.0)
      (bind _returnvalue (`GameplayStatics.GetActorOfClass` "/Game/Blueprints/Levels/SpawnArea_Kasir.SpawnArea_Kasir_C"))
      (bind (_returnvalue_location _returnvalue_rotation) (`KismetMathLibrary.BreakTransform` (`self.GetTransform` _returnvalue)))
      (`self.K2_SetActorTransform` _player_ref (`KismetMathLibrary.MakeTransform` _returnvalue_location _returnvalue_rotation (`self.GetActorScale3D` _player_ref)) false true))))

(fn `UserConstructionScript`
  (`parent.UserConstructionScript`))