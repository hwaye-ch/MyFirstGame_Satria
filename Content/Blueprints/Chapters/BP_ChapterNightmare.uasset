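; Nightmare chapter controller that fades in the player at a spawn area with running disabled and scripts events across a sequence of blocks.
; Each SpawnStuff call receives new and current blocks, places story pickups at certain counts, advances SpawnCount and opens the new block's wall.
; Count milestones spawn a crawling Mother with pawn sensing, later destroy her, and finally restore the wall and spawn a sitting evil Mikey.
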(event `Initiate Nightmare`
  (bind _player_ref (`self.Player Ref`))
  (`|ExecutionSequence`
    (:`then_0`
      (`/Game/Blueprints/Components/BP_FadeScreenComponent.Black Screen then Fade In` (`self.BP_FadeScreenComponent`) (`self.Player Ref`) 3.0)
      (set `/Game/FirstPerson/Blueprints/BP_FirstPersonCharacter.Can Jump?` true _player_ref)
      (set `/Game/FirstPerson/Blueprints/BP_FirstPersonCharacter.Can Crouch?` true _player_ref)
      (set `/Game/FirstPerson/Blueprints/BP_FirstPersonCharacter.Can Run?` false _player_ref))
    (:`then_1`
      (bind _player_spawn_area (`self.Player Spawn Area`)
        (:`then`
          (bind (_returnvalue_location _returnvalue_rotation) (`KismetMathLibrary.BreakTransform` (`self.GetTransform` _player_spawn_area)))
          (`self.K2_SetActorLocation` (`self.Player Ref`) _returnvalue_location false false)
          (`Controller.SetControlRotation` (`GameplayStatics.GetPlayerController` 0) _returnvalue_rotation))
        (:`else`)))))

(event `Spawn Stuff`
  (params (`New Block` :type "/Game/Blueprints/Items/Area_EndlessNightmare Object Reference") (`Current Block` :type "/Game/Blueprints/Items/Area_EndlessNightmare Object Reference"))
  (bind _returnvalue (`SceneComponent.K2_GetComponentToWorld` (`/Game/Blueprints/Items/Area_EndlessNightmare.SpawnStuffArea` (`self.NewBlock`))))
  (set `self.CurrentBlock` `Current Block`)
  (set `self.NewBlock` `New Block`)
  (switch `int` (`self.Spawn Count`)
    (:`Default`
      (`self.Setups` :!label _label))
    (:`0`
      (goto _label))
    (:`1`
      (goto _label))
    (:`2`
      (bind _returnvalue_2 (`|SpawnActorFromClass` "/Game/Blueprints/EventItems/BP_Koran.BP_Koran_C" _returnvalue "Undefined" "MultiplyWithRoot" null true null))
      (`KismetSystemLibrary.PrintString` (`KismetStringLibrary.Concat_StrStr` "Spawning " (`KismetSystemLibrary.GetDisplayName` _returnvalue_2)))
      (`SceneComponent.SetVisibility` (`/Game/Blueprints/Items/Area_EndlessNightmare.SpawnStuffArea` (`self.NewBlock`)) true true :!label _label_2)
      (`self.Setups`))
    (:`3`
      (goto _label))
    (:`4`
      (bind _returnvalue_3 (`|SpawnActorFromClass` "/Game/Blueprints/EventItems/BP_ConsultationLetterFromSarah.BP_ConsultationLetterFromSarah_C" _returnvalue "Undefined" "MultiplyWithRoot" null true null))
      (`KismetSystemLibrary.PrintString` (`KismetStringLibrary.Concat_StrStr` (`KismetSystemLibrary.GetDisplayName` _returnvalue_3) (`KismetSystemLibrary.GetDisplayName` null)))
      (goto _label_2))
    (:`5`
      (goto _label))
    (:`6`
      (bind _returnvalue_4 (`|SpawnActorFromClass` "/Game/Blueprints/EventItems/BP_Rontgen.BP_Rontgen_C" _returnvalue "Undefined" "MultiplyWithRoot" null true null))
      (`KismetSystemLibrary.PrintString` (`KismetStringLibrary.Concat_StrStr` (`KismetSystemLibrary.GetDisplayName` _returnvalue_4) (`KismetSystemLibrary.GetDisplayName` null)))
      (goto _label_2))))

(event `Setups`
  (bind _wall (`/Game/Blueprints/Items/Area_EndlessNightmare.Wall` (`self.NewBlock`)))
  (bind _wall_2 (`/Game/Blueprints/Items/Area_EndlessNightmare.Wall` (`self.NewBlock`)))
  (bind _result (`/Engine/EditorBlueprintResources/StandardMacros.IncrementInt` (`self.Spawn Count`))
    (:`  `
      (`KismetSystemLibrary.PrintString` (`KismetStringLibrary.Concat_StrStr` "Spawn Count: " (`KismetStringLibrary.Conv_IntToString` _result)))
      (`SceneComponent.SetVisibility` _wall false false)
      (`PrimitiveComponent.SetCollisionEnabled` _wall "NoCollision")
      (if (== (`self.Spawn Count`) 10)
        (`self.Spawn Mom`)
        (elif (== (`self.Spawn Count`) 24)
          (bind _mother (`self.Mother`)
            (:`then`
              (`self.K2_DestroyActor` _mother))
            (:`else`))
          (elif (== (`self.Spawn Count`) 30)
            (`KismetSystemLibrary.PrintString` "Spawning Michael")
            (`SceneComponent.SetVisibility` _wall_2 true true)
            (`PrimitiveComponent.SetCollisionEnabled` _wall_2 "QueryAndPhysics")
            (`|SpawnActorFromClass` "/Game/Blueprints/Characters/BP_MikeyEvilSitting.BP_MikeyEvilSitting_C" (`SceneComponent.K2_GetComponentToWorld` (`/Game/Blueprints/Items/Area_EndlessNightmare.MikeyLocation` (`self.CurrentBlock`))) "Undefined" "MultiplyWithRoot" null null)))))))

(event `Spawn Mom`
  (bind _returnvalue (`|SpawnActorFromClass` "/Game/Blueprints/Characters/BP_MomCrawling.BP_MomCrawling_C" (`SceneComponent.K2_GetComponentToWorld` (`/Game/Blueprints/Items/Area_EndlessNightmare.SpawnAreaMother` (`self.CurrentBlock`))) "Undefined" "MultiplyWithRoot" null null))
  (bind _output_get (set `self.Mother` _returnvalue))
  (`PawnSensingComponent.SetSensingUpdatesEnabled` (`/Game/Blueprints/Characters/BP_MomCrawling.PawnSensing` _output_get) true))

(fn `UserConstructionScript`
  (`parent.UserConstructionScript`))