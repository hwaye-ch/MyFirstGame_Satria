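; Supermarket customer NPC that brings frozen food to the counter, holds a one-time checkout dialogue, then takes the item home.
; Level sequences bound to this actor at runtime drive the buying and leaving animations.
; TakeAction spawns the food if needed and attaches it to the right hand; finishing the buying sequence moves it to the drop area.
; Dialogue callbacks play the cash-register sound and trigger pickup and exit.
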(event `self.ReceiveBeginPlay`
  (`parent.ReceiveBeginPlay`)
  (bind _returnvalue (`GameplayStatics.GetActorOfClass` "/Game/Blueprints/Chapters/BP_Chapter2SupermarketManager.BP_Chapter2SupermarketManager_C"))
  (set `self.Chapter2Manager` _returnvalue))

(event `self.TalkWithObject`
  (bind _bp_dialoguecomponent (`self.BP_DialogueComponent`))
  (`/Engine/EditorBlueprintResources/StandardMacros.DoOnce` false
    (:`Completed`
      (add `/Game/Blueprints/Components/BP_DialogueComponent.OnActionDuringDialogue` _bp_dialoguecomponent (delegate `OnAction_Event`))
      (add `/Game/Blueprints/Components/BP_DialogueComponent.OnDialogueEnded` _bp_dialoguecomponent (delegate `OnDialogueEnded_Event`))
      (bind _dialoguecomponent (`/Game/Blueprints/Components/BP_DialogueComponent.Construct Dialogue` _bp_dialoguecomponent "ch1_customer2" "/Game/Dialogue/Chapter1_Dialogue.Chapter1_Dialogue" true true))
      (`/Game/Blueprints/Interface/BPI_Dialogue.ShowDialogue` _dialoguecomponent (`self.PlayerRef`) self))))

(event `OnDialogueEnded_Event`
  (`KismetSystemLibrary.Delay` 2.0)
  (`self.K2_DetachFromActor` (`self.Nasi`) "KeepWorld" "KeepWorld" "KeepWorld")
  (`self.Take Action`)
  (`KismetSystemLibrary.DelayUntilNextTick`)
  (bind (_outactor _returnvalue) (`LevelSequencePlayer.CreateLevelSequencePlayer` "/Game/Animation/Anim_CustomerGoHome.Anim_CustomerGoHome"))
  (`LevelSequenceActor.AddBinding` _outactor (`|GetSequenceBinding` null) self false)
  (`MovieSceneSequencePlayer.Play` _returnvalue))

(event `OnAction_Event`
  (`GameplayStatics.PlaySound2D` "/Game/Sounds/sfx_kaching.sfx_kaching" 1.0 1.0 0.0 null null))

(event `Start Sequence Customer 3`
  (bind (_outactor _returnvalue) (`LevelSequencePlayer.CreateLevelSequencePlayer` "/Game/Animation/Anim_CustomerBuyingFromLeft.Anim_CustomerBuyingFromLeft"))
  (`LevelSequenceActor.AddBinding` _outactor (`|GetSequenceBinding` null) self false)
  (add `MovieSceneSequencePlayer.OnFinished` _returnvalue (delegate `OnFinished_Event`))
  (`MovieSceneSequencePlayer.Play` _returnvalue))

(event `OnFinished_Event`
  (bind _returnvalue (`GameplayStatics.GetActorOfClass` "/Game/Blueprints/Levels/Area_DropStuff.Area_DropStuff_C"))
  (bind _output_get (set `self.Area_Drop` _returnvalue))
  (`self.K2_AttachToComponent` (`self.Nasi`) (`/Game/Blueprints/ModularItems/BP_SpawnLocation.DefaultSceneRoot` _output_get) "None" "SnapToTarget" "SnapToTarget" "KeepWorld" true))

(event `self.Take Action`
  (`self.Nasi`
    (:`then`
      _)
    (:`else`
      (bind _returnvalue (`|SpawnActorFromClass` "/Game/Blueprints/EventItems/BP_FrozenFood.BP_FrozenFood_C" (`SceneComponent.GetSocketTransform` (`self.Mesh`) "RightHandSocket" "RTS_World") "Undefined" "MultiplyWithRoot" null null))
      (set `self.Nasi` _returnvalue)))
  (`self.K2_AttachToComponent` (`self.Nasi`) (`self.Mesh`) "RightHandSocket" "SnapToTarget" "SnapToTarget" "KeepWorld" true))

(fn `UserConstructionScript`
  (`parent.UserConstructionScript`))