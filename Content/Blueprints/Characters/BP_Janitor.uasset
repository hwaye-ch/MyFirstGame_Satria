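; BP_Janitor is an NPC that can be moved behind the player and talked to.
; On BeginPlay it binds both actions to events on an Enabler reference, which drives when they happen.
; The move snaps the janitor to the location and rotation of a TeleportLocation actor.
; Interaction shows dialogue through BPDialogueComponent, then calls ActivateLaptop straight away.
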(event `self.ReceiveBeginPlay`
  (bind _enabler (`self.Enabler`))
  (`parent.ReceiveBeginPlay`)
  (`/Engine/EditorBlueprintResources/StandardMacros.IsValid` _enabler
    (:`Is Valid`
      (add `/Game/Blueprints/EventItems/BP_MysteriousBasketballSound.MoveJanitor` _enabler (delegate `Move Janitor Behind Player`))
      (add `/Game/Blueprints/EventItems/BP_MysteriousBasketballSound.TalkToJanitor` _enabler (delegate `Interact With Janitor`)))))

(event `Move Janitor Behind Player`
  (bind _teleportlocation (`self.TeleportLocation`))
  (`/Engine/EditorBlueprintResources/StandardMacros.IsValid` _teleportlocation
    (:`Is Valid`
      (`self.K2_SetActorLocationAndRotation` (`self.K2_GetActorLocation` _teleportlocation) (`self.K2_GetActorRotation` _teleportlocation)))))

(event `Interact With Janitor`
  (params (`Player Pref` :type "/Game/FirstPerson/Blueprints/BP_FirstPersonCharacter Object Reference"))
  (`/Game/Blueprints/Interface/BPI_Dialogue.ShowDialogue` (`self.BP_DialogueComponent`) `Player Pref` self)
  (`self.ActivateLaptop`))

(fn `UserConstructionScript`
  (`parent.UserConstructionScript`))