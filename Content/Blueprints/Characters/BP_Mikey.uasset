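; BP_Mikey is the Blueprint for Mikey, a character that the player can have a dialogue with.
; On BeginPlay it binds handlers to the start and end events of its BPDialogueComponent.
; Dialogue start switches on the talk state through CallToggleIdleToTalk, while dialogue end switches it off and calls CallUnblockBarrier.
; Both handlers print debug strings, and the construction script only runs the parent's.
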(event `self.ReceiveBeginPlay`
  (bind _bp_dialoguecomponent (`self.BP_DialogueComponent`))
  (add `/Game/Blueprints/Components/BP_DialogueComponent.OnDialogueEnded` _bp_dialoguecomponent (delegate `Dialogue Ends`))
  (add `/Game/Blueprints/Components/BP_DialogueComponent.OnDialogStarted` _bp_dialoguecomponent (delegate `Dialogue Starts`)))

(event `Dialogue Ends`
  (`KismetSystemLibrary.PrintString` "Dialogue with Mikey Finished")
  (`self.UnblockBarrier`)
  (`self.ToggleIdleToTalk` false))

(event `Dialogue Starts`
  (`KismetSystemLibrary.PrintString` "Starting doing things while talking")
  (`self.ToggleIdleToTalk` true))

(fn `UserConstructionScript`
  (`parent.UserConstructionScript`))