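; BP_MomNormal is a Mom character that relocates when the window camera signals it.
; On BeginPlay it finds the BP_WindowCamera and binds to its MoveMomDadMikey dispatcher.
; When that fires, it snaps to the location and rotation of the SpawnArea_Mom actor and sets IsStanding to true.
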(event `self.ReceiveBeginPlay`
  (`parent.ReceiveBeginPlay`)
  (bind _returnvalue (`GameplayStatics.GetActorOfClass` "/Game/Blueprints/LevelCameras/BP_WindowCamera.BP_WindowCamera_C"))
  (add `/Game/Blueprints/LevelCameras/BP_WindowCamera.MoveMomDadMikey` _returnvalue (delegate `MoveMomDadMikey_Event`)))

(event `MoveMomDadMikey_Event`
  (bind _returnvalue (`GameplayStatics.GetActorOfClass` "/Game/Blueprints/Levels/SpawnArea_Mom.SpawnArea_Mom_C"))
  (`self.K2_SetActorLocationAndRotation` (`self.K2_GetActorLocation` _returnvalue) (`self.K2_GetActorRotation` _returnvalue))
  (set `self.IsStanding` true))

(fn `UserConstructionScript`
  (`parent.UserConstructionScript`))