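; Actor component that shows a choice dialogue widget and relays the player's chosen option through an ExecuteOption dispatcher.
; Opening it creates WBP_ChoiceDialogue, binds its option-pressed event, switches to UI-only input with a cursor and disables the passed-in player's movement and look.
; A selection broadcasts immediately, then after a short delay removes the widget and restores player control, game-only input and the hidden cursor.
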(event `Construct Choice Dialogue`
  (params (`Player Pref` :type "/Game/FirstPerson/Blueprints/BP_FirstPersonCharacter Object Reference"))
  (bind _returnvalue (`GameplayStatics.GetPlayerController` 0))
  (set `self.Player Pref` `Player Pref`)
  (bind _returnvalue_2 (`|CreateWidget` "/Game/Blueprints/Widgets/WBP_ChoiceDialogue.WBP_ChoiceDialogue_C"))
  (set `self.Dialogue Widget` _returnvalue_2)
  (add `/Game/Blueprints/Widgets/WBP_ChoiceDialogue.OnOptionPressed` (`self.Dialogue Widget`) (delegate `Option Listener`))
  (`UserWidget.AddToViewport` (`self.Dialogue Widget`) 0)
  (`WidgetBlueprintLibrary.SetInputMode_UIOnlyEx` _returnvalue (`self.Dialogue Widget`))
  (set `PlayerController.bShowMouseCursor` true _returnvalue)
  (`/Game/FirstPerson/Blueprints/BP_FirstPersonCharacter.Disable Movement and Look` (`self.Player Pref`)))

(event `Destroy Choice Dialogue`
  (`/Engine/EditorBlueprintResources/StandardMacros.IsValid` (`self.Dialogue Widget`)
    (:`Is Valid`
      (`Widget.RemoveFromParent` (`self.Dialogue Widget`)))))

(event `Option Listener`
  (params (ChosenOption :type "/Game/Blueprints/Enumerations/E_ChoiceDialogue Enum" :default "NewEnumerator0"))
  (bind _returnvalue (`GameplayStatics.GetPlayerController` 0))
  (`self.ExecuteOption` ChosenOption)
  (`KismetSystemLibrary.Delay` 0.5)
  (`self.Destroy Choice Dialogue`)
  (`/Game/FirstPerson/Blueprints/BP_FirstPersonCharacter.Enable Look and Movement` (`self.Player Pref`))
  (`WidgetBlueprintLibrary.SetInputMode_GameOnly` _returnvalue)
  (set `PlayerController.bShowMouseCursor` false _returnvalue))