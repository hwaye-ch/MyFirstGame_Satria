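; Actor component that shows data-table-driven dialogue in a WBP_Dialogue widget, either player-triggered or self-advancing.
; Each row supplies the text, next row, next table and end flag, so conversations can chain across tables.
; ShowDialogue optionally blocks player movement and look and stores dialogue state on the player, while completion notifies the trigger actor.
; ShowAutoDestroyDialogue re-calls itself after a timed delay until the end row removes the widget.
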(event `/Game/Blueprints/Interface/BPI_Dialogue.ClearDialogue`
  (bind _player_pref (`self.Player Pref`))
  (`/Engine/EditorBlueprintResources/StandardMacros.IsValid` (`self.DialogueWidget`)
    (:`Is Valid`
      (`Widget.RemoveFromParent` (`self.DialogueWidget`))
      (`/Engine/EditorBlueprintResources/StandardMacros.IsValid` _player_pref
        (:`Is Valid`
          (set `/Game/FirstPerson/Blueprints/BP_FirstPersonCharacter.DialogueWidget` null _player_pref))))
    (:`Is Not Valid`
      _))
  (`self.Reset Movement`))

(event `Modify Movement`
  (params (PlayerPref :type "/Game/FirstPerson/Blueprints/BP_FirstPersonCharacter Object Reference"))
  (`/Engine/EditorBlueprintResources/StandardMacros.IsValid` PlayerPref
    (:`Is Valid`
      (bind _output_get (set `self.Player Pref` PlayerPref))
      (if (`self.BlockMovement`)
        (`/Game/FirstPerson/Blueprints/BP_FirstPersonCharacter.Disable Movement` _output_get))
      (if (`self.BlockLook`)
        (`/Game/FirstPerson/Blueprints/BP_FirstPersonCharacter.Disable Look` (`self.Player Pref`))))))

(event `Reset Movement`
  (bind _player_pref (`self.Player Pref`))
  (`/Engine/EditorBlueprintResources/StandardMacros.IsValid` _player_pref
    (:`Is Valid`
      (`/Game/FirstPerson/Blueprints/BP_FirstPersonCharacter.Enable Look and Movement` _player_pref))))

(event `/Game/Blueprints/Interface/BPI_Dialogue.FillDialogue`
  (bind _dialoguewidget (`self.DialogueWidget`))
  (`/Engine/EditorBlueprintResources/StandardMacros.IsValid` _dialoguewidget
    (:`Is Valid`
      (`/Game/Blueprints/Widgets/WBP_Dialogue.Fill Dialogue Text` _dialoguewidget))))

(event `/Game/Blueprints/Interface/BPI_Dialogue.FinishDialogue`
  (bind _player_pref (`self.Player Pref`))
  (`/Engine/EditorBlueprintResources/StandardMacros.IsValid` _player_pref
    (:`Is Valid`
      (set `/Game/FirstPerson/Blueprints/BP_FirstPersonCharacter.IsDialogueTextComplete` true _player_pref)
      (message `/Game/Blueprints/Interface/BPI_Dialogue.FinishDialogue` (`self.DialogueActorTrigger`)))))

(event `/Game/Blueprints/Interface/BPI_Dialogue.ShowAutoDestroyDialogue`
  (bind _dialoguewidget (`self.DialogueWidget`))
  (`|ExecutionSequence`
    (:`then_0`
      (set `self.DialogueTable` (`self.DialogueTable`)))
    (:`then_1`
      (`/Engine/EditorBlueprintResources/StandardMacros.IsValid` (`self.DialogueWidget`)
        (:`Is Valid`
          (bind _returnvalue (`|GetDataTableRow` (`self.DialogueTable`) (`self.DialogueCode`))
            (:`then`
              (bind (_dialogue _nextrow _datatable _enddialogue_) (break `/Game/Dialogue/Dialogue_Structure` _returnvalue))
              (`/Game/Blueprints/Widgets/WBP_Dialogue.Update Dialogue` (`self.DialogueWidget`) _dialogue self)
              (set `self.DialogueCode` _nextrow)
              (set `self.DialogueTable` _datatable)
              (set `self.IsDialogueEnded` _enddialogue_)
              (`KismetSystemLibrary.Delay` (`self.DisplayDialogueDuration`) :!label _label)
              (if (`self.IsDialogueEnded`)
                (`/Game/Blueprints/Interface/BPI_Dialogue.ClearDialogue`)
                (`/Engine/EditorBlueprintResources/StandardMacros.IsValid` _dialoguewidget
                  (:`Is Valid`
                    (`Widget.RemoveFromParent` _dialoguewidget)
                    (set `self.DialogueWidget` null)))
                (else
                  (`self.ShowAutoDestroyDialogue`))))
            (:`RowNotFound`
              (`KismetSystemLibrary.PrintString` "Wrong Dialogue Code" :!label _label_2))))
        (:`Is Not Valid`
          (bind _returnvalue_2 (`|GetDataTableRow` (`self.DialogueTable`) (`self.DialogueCode`))
            (:`then`
              (bind (_dialogue_2 _nextrow_2 _datatable_2 _enddialogue__2) (break `/Game/Dialogue/Dialogue_Structure` _returnvalue_2))
              (bind _returnvalue_3 (`|CreateWidget` "/Game/Blueprints/Widgets/WBP_Dialogue.WBP_Dialogue_C" null (`self.Actor Name`) _dialogue_2 self))
              (`UserWidget.AddToViewport` _returnvalue_3 0)
              (set `self.DialogueWidget` _returnvalue_3)
              (set `self.DialogueCode` _nextrow_2)
              (set `self.DialogueTable` _datatable_2)
              (set `self.IsDialogueEnded` _enddialogue__2)
              (goto _label))
            (:`RowNotFound`
              (goto _label_2))))))))

(fn `ShowDialogue`
  (params (PlayerPref :type "/Game/FirstPerson/Blueprints/BP_FirstPersonCharacter Object Reference") (DialogueActorTrigger :type "Actor Object Reference"))
  (set `self.Player Pref` PlayerPref)
  (`|ExecutionSequence`
    (:`then_0`
      (`self.Modify Movement` (`self.Player Pref`))
      (set `self.DialogueTable` (`self.DialogueTable`))
      (set `/Game/FirstPerson/Blueprints/BP_FirstPersonCharacter.IsDialogueTextComplete` false (`self.Player Pref`))
      (set `/Game/FirstPerson/Blueprints/BP_FirstPersonCharacter.IsTriggeringDialogue` true (`self.Player Pref`))
      (set `self.DialogueActorTrigger` DialogueActorTrigger)
      (set `self.DialogueWidget` (`/Game/FirstPerson/Blueprints/BP_FirstPersonCharacter.DialogueWidget` (`self.Player Pref`))))
    (:`then_1`
      (`/Engine/EditorBlueprintResources/StandardMacros.IsValid` (`self.DialogueWidget`)
        (:`Is Valid`
          (bind _returnvalue (`|GetDataTableRow` (`self.DialogueTable`) (`self.DialogueCode`))
            (:`then`
              (bind (_dialogue _nextrow _datatable _enddialogue_) (break `/Game/Dialogue/Dialogue_Structure` _returnvalue))
              (`/Game/Blueprints/Widgets/WBP_Dialogue.Update Dialogue` (`self.DialogueWidget`) _dialogue self)
              (set `/Game/FirstPerson/Blueprints/BP_FirstPersonCharacter.IsDialogueEnded` _enddialogue_ (`self.Player Pref`))
              (set `self.DialogueCode` _nextrow)
              (set `self.DialogueTable` _datatable)
              (set `/Game/FirstPerson/Blueprints/BP_FirstPersonCharacter.DialogueActorComponent` self (`self.Player Pref`))
              (return))
            (:`RowNotFound`
              _)))
        (:`Is Not Valid`
          (bind _returnvalue_2 (`|GetDataTableRow` (`self.DialogueTable`) (`self.DialogueCode`))
            (:`then`
              (bind (_dialogue_2 _nextrow_2 _datatable_2 _enddialogue__2) (break `/Game/Dialogue/Dialogue_Structure` _returnvalue_2))
              (bind _returnvalue_3 (`|CreateWidget` "/Game/Blueprints/Widgets/WBP_Dialogue.WBP_Dialogue_C" null (`self.Actor Name`) _dialogue_2 self))
              (`UserWidget.AddToViewport` _returnvalue_3 0)
              (set `/Game/FirstPerson/Blueprints/BP_FirstPersonCharacter.DialogueWidget` _returnvalue_3 (`self.Player Pref`))
              (set `self.DialogueWidget` _returnvalue_3)
              (set `self.DialogueCode` _nextrow_2)
              (set `self.DialogueTable` _datatable_2)
              (set `/Game/FirstPerson/Blueprints/BP_FirstPersonCharacter.DialogueActorComponent` self (`self.Player Pref`))
              (set `/Game/FirstPerson/Blueprints/BP_FirstPersonCharacter.IsDialogueEnded` _enddialogue__2 (`self.Player Pref`))
              (return))
            (:`RowNotFound`
              _))))
      (`KismetSystemLibrary.PrintString` "Wrong Dialogue Code"))))