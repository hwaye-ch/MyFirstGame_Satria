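; BP_DisplayChatDialogue displays a chat dialogue popup on screen using the WBP_Chat widget.
; ShowChatWidget creates the widget with the supplied image, adds it to the viewport and plays its DisplayMessage animation.
; When that animation ends, it fires the OnAnimationFinished dispatcher and removes the widget from its parent.
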(event `Show Chat Widget`
  (params (Image :type "Texture2D Object Reference"))
  (bind _widget (`self.Widget`))
  (bind _displaymessage (`/Game/Blueprints/Widgets/WBP_Chat.DisplayMessage` _widget))
  (bind _returnvalue (`|CreateWidget` "/Game/Blueprints/Widgets/WBP_Chat.WBP_Chat_C" null Image))
  (bind _output_get (set `self.Widget` _returnvalue))
  (`UserWidget.AddToViewport` _output_get 0)
  (`UserWidget.PlayAnimation` _widget _displaymessage 0.0 1 "Forward" 1.0 false)
  (`UserWidget.BindToAnimationFinished` (`self.Widget`) _displaymessage (delegate `Call On Finished Animation`)))

(event `Call On Finished Animation`
  (`self.OnAnimationFinished`)
  (`Widget.RemoveFromParent` (`self.Widget`)))