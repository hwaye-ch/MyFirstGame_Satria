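; Actor component that runs screen fades through WBP_FadeScreen widget animations, locking player movement and look during fade-outs.
; FadeEvent chains timed fade-out, black-screen hold and fade-in via parallel delayed Sequence branches, with FadeIn restoring player control.
; It fires OnFadeEventFinished after the black-screen hold, then clears all bindings next tick, making listeners one-shot.
; FadeInScreen offers a standalone fade-in that leaves player control untouched.
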(event `Fade In Screen`
  (params (PlayerPref :type "/Game/FirstPerson/Blueprints/BP_FirstPersonCharacter Object Reference"))
  (set `self.Player Ref` PlayerPref)
  (bind _returnvalue (`|CreateWidget` "/Game/Blueprints/Widgets/WBP_FadeScreen.WBP_FadeScreen_C"))
  (bind _output_get (set `self.FadeInWidget` _returnvalue))
  (`UserWidget.AddToViewport` _output_get 0)
  (`UserWidget.PlayAnimation` (`self.FadeInWidget`) (`/Game/Blueprints/Widgets/WBP_FadeScreen.FadeInSequence` (`self.FadeInWidget`)) 0.0 1 "Forward" 1.0 false)
  (`KismetSystemLibrary.Delay` 2.0)
  (`Widget.RemoveFromParent` (`self.FadeInWidget`)))

(event `Fade Out`
  (params (`Fade Out Duration` :type "Float (double-precision)") (PlayerPref :type "/Game/FirstPerson/Blueprints/BP_FirstPersonCharacter Object Reference"))
  (set `self.Fade Out Duration` `Fade Out Duration`)
  (set `self.Player Ref` PlayerPref)
  (`/Game/FirstPerson/Blueprints/BP_FirstPersonCharacter.Disable Movement and Look` (`self.Player Ref`))
  (bind _returnvalue (`|CreateWidget` "/Game/Blueprints/Widgets/WBP_FadeScreen.WBP_FadeScreen_C"))
  (set `self.FadeOutWidget` _returnvalue)
  (`UserWidget.AddToViewport` (`self.FadeOutWidget`) 0)
  (`UserWidget.PlayAnimation` (`self.FadeOutWidget`) (`/Game/Blueprints/Widgets/WBP_FadeScreen.FadeOutSequence` (`self.FadeOutWidget`)) 0.0 1 "Forward" 1.0 false)
  (`KismetSystemLibrary.Delay` (`self.Fade Out Duration`))
  (`Widget.RemoveFromParent` (`self.FadeOutWidget`)))

(event `Black Screen`
  (bind _returnvalue (`|CreateWidget` "/Game/Blueprints/Widgets/WBP_FadeScreen.WBP_FadeScreen_C"))
  (bind _output_get (set `self.BlackScreenWidget` _returnvalue))
  (`UserWidget.AddToViewport` _output_get 0)
  (`UserWidget.PlayAnimation` (`self.BlackScreenWidget`) (`/Game/Blueprints/Widgets/WBP_FadeScreen.BlackScreen` (`self.BlackScreenWidget`)) 0.0 1 "Forward" 1.0 false)
  (`KismetSystemLibrary.Delay` (`self.Duration`)))

(event `Fade Event`
  (params (Duration :type "Float (single-precision)") (`Player Pref` :type "/Game/FirstPerson/Blueprints/BP_FirstPersonCharacter Object Reference") (`Delay Before Fade In` :type "Float (double-precision)"))
  (bind _returnvalue (`KismetMathLibrary.SignOfFloat` 3.0))
  (if (== `Delay Before Fade In` 0.0)
    (set `self.Delay Before Fade In` 2.0)
    (else
      (set `self.Delay Before Fade In` `Delay Before Fade In`)))
  (set `self.Duration` Duration)
  (set `self.Player Ref` `Player Pref`)
  (`/Game/FirstPerson/Blueprints/BP_FirstPersonCharacter.Disable Movement and Look` (`self.Player Ref`))
  (`|ExecutionSequence`
    (:`then_0`
      (`self.Fade Out` _returnvalue (`self.Player Ref`)))
    (:`then_1`
      (`KismetSystemLibrary.Delay` _returnvalue)
      (`self.Black Screen`)
      (`KismetSystemLibrary.Delay` (`self.Duration`))
      (`self.OnFadeEventFinished`)
      (`KismetSystemLibrary.DelayUntilNextTick`)
      (clear `self.OnFadeEventFinished`))
    (:`then_2`
      (`KismetSystemLibrary.Delay` (+ (- (`self.Duration`) 0.1) (`self.Delay Before Fade In`)))
      (`Widget.RemoveFromParent` (`self.BlackScreenWidget`))
      (`self.Fade In` (`self.Player Ref`)))))

(event `Fade In`
  (params (`Player Pref` :type "/Game/FirstPerson/Blueprints/BP_FirstPersonCharacter Object Reference"))
  (set `self.Player Ref` `Player Pref`)
  (bind _returnvalue (`|CreateWidget` "/Game/Blueprints/Widgets/WBP_FadeScreen.WBP_FadeScreen_C"))
  (bind _output_get (set `self.FadeInWidget` _returnvalue))
  (`UserWidget.AddToViewport` _output_get 0)
  (`UserWidget.PlayAnimation` (`self.FadeInWidget`) (`/Game/Blueprints/Widgets/WBP_FadeScreen.FadeInSequence` (`self.FadeInWidget`)) 0.0 1 "Forward" 1.0 false)
  (`KismetSystemLibrary.Delay` 2.0)
  (`Widget.RemoveFromParent` (`self.FadeInWidget`))
  (`/Game/FirstPerson/Blueprints/BP_FirstPersonCharacter.Enable Look and Movement` (`self.Player Ref`)))