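; BP_ReadableComponent is a component that shows a readable object's description on screen.
; ShowObjectDescription looks up its Keyword in a DataTable and picks the localized text column matching the game instance's Language setting.
; It creates a WBP_ReadItemDescription widget with that text, adds it to the viewport and returns it, or prints a message if the row is missing.
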(fn `Show Object Description`
  (returns (ReturnValue :type "/Game/Blueprints/Widgets/WBP_ReadItemDescription Object Reference"))
  (locals (NewLocalVar :type "/Game/Dialogue/Description_Structure Structure"))
  (bind _returnvalue (`|GetDataTableRow` (`self.DataTable`) (`self.Keyword`))
    (:`then`
      (bind _ashwy_game_instance (cast `/Game/System/HwyGameInstance` (`GameplayStatics.GetGameInstance`)))
      (bind (_id _jp _en _kr _th _ch _sunda) (break `/Game/Dialogue/Description_Structure` _returnvalue))
      (bind _returnvalue_2 (`|CreateWidget` "/Game/Blueprints/Widgets/WBP_ReadItemDescription.WBP_ReadItemDescription_C" null (select `/Game/Blueprints/Enumerations/E_Language` (`/Game/System/HwyGameInstance.Language` _ashwy_game_instance) :`NewEnumerator0` _id :`NewEnumerator1` _jp :`NewEnumerator2` _en :`NewEnumerator3` _kr :`NewEnumerator4` _th :`NewEnumerator5` _ch :`NewEnumerator6` _sunda)))
      (bind _output_get (set `self.Widget` _returnvalue_2))
      (`UserWidget.AddToViewport` _output_get 0)
      (return (`self.Widget`)))
    (:`RowNotFound`
      (`KismetSystemLibrary.PrintString` "Description not found"))))