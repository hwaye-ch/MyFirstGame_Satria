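; BP_TextRelatedComponent provides localized text lookup and displays object descriptions on screen.
; ExtractText finds the Keyword row in a DataTable and selects the column matching the HwyGameInstance language, printing an error if the row is missing.
; ShowObjectDescription passes that text into a new WBP_ReadItemDescription widget, adds it to the viewport and returns it.
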(fn `Extract Text`
  (params (DataTable :type "DataTable Object Reference") (Keyword :type Name))
  (returns (`Extracted Text` :type Text))
  (bind _returnvalue (`|GetDataTableRow` DataTable Keyword)
    (:`then`
      (bind _ashwy_game_instance (cast `/Game/System/HwyGameInstance` (`GameplayStatics.GetGameInstance`)))
      (bind (_id _jp _en _kr _th _ch _sunda) (break `/Game/Dialogue/Description_Structure` _returnvalue))
      (return (select `/Game/Blueprints/Enumerations/E_Language` (`/Game/System/HwyGameInstance.Language` _ashwy_game_instance) :`NewEnumerator0` _id :`NewEnumerator1` _jp :`NewEnumerator2` _en :`NewEnumerator3` _kr :`NewEnumerator4` _th :`NewEnumerator5` _ch :`NewEnumerator6` _sunda)))
    (:`RowNotFound`
      (`KismetSystemLibrary.PrintString` "Keyword not found"))))

(fn `Show Object Description`
  (returns (ReturnValue :type "/Game/Blueprints/Widgets/WBP_ReadItemDescription Object Reference"))
  (locals (NewLocalVar :type "/Game/Dialogue/Description_Structure Structure"))
  (bind _extracted_text (`self.Extract Text` (`self.DataTable`) (`self.Keyword`)))
  (bind _returnvalue (`|CreateWidget` "/Game/Blueprints/Widgets/WBP_ReadItemDescription.WBP_ReadItemDescription_C" null _extracted_text))
  (bind _output_get (set `self.Widget` _returnvalue))
  (`UserWidget.AddToViewport` _output_get 0)
  (return (`self.Widget`)))