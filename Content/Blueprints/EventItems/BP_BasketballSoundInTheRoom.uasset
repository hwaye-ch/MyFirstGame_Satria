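; Event item that plays a basketball dribbling sound in the room until the player has looked at it long enough.
; SetReady enables the cube's collision and spawns the attenuated sound at the actor's location.
; Tick adds a fixed, frame-based increment while the player's HitActor is tagged "Basket".
; At the threshold it displays BP_MomOnBed, readies BP_LookAtMom, then after a delay stops the sound and destroys itself.
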(event `self.ReceiveBeginPlay`
  (`parent.ReceiveBeginPlay`)
  (`PrimitiveComponent.SetCollisionEnabled` (`self.Cube`) "NoCollision"))

(event `self.ReceiveTick`
  (params (DeltaSeconds :type "Float (single-precision)"))
  (`KismetSystemLibrary.DelayUntilNextTick`)
  (`self.IsEventReady?`
    (:`then`
      (`self.IsLookAtAlreadyFull`
        (:`then`)
        (:`else`
          (bind _hit_actor (`/Game/FirstPerson/Blueprints/BP_FirstPersonCharacter.Hit Actor` (`self.Player Pref`))
            (:`then`
              (if (`self.ActorHasTag` _hit_actor "Basket")
                (bind _output_get (set `self.LookAtLength` (+ (`self.LookAtLength`) 0.01)))
                (`KismetSystemLibrary.PrintString` (`KismetStringLibrary.Conv_DoubleToString` _output_get))
                (if (>= (`self.LookAtLength`) (`self.LookAtMax`))
                  (set `self.IsLookAtAlreadyFull` true)
                  (bind _returnvalue (`GameplayStatics.GetActorOfClass` "/Game/Blueprints/EventItems/BP_MomOnBed.BP_MomOnBed_C"))
                  (`/Game/Blueprints/EventItems/BP_MomOnBed.Display Mom` _returnvalue)
                  (bind _returnvalue_2 (`GameplayStatics.GetActorOfClass` "/Game/Blueprints/Levels/BP_LookAtMom.BP_LookAtMom_C"))
                  (set `/Game/Blueprints/Levels/BP_LookAtMom.IsReady?` true _returnvalue_2)
                  (`KismetSystemLibrary.Delay` 5.0)
                  (bind _basketballsound (`self.BasketballSound`)
                    (:`then`
                      (`AudioComponent.Stop` _basketballsound))
                    (:`else`
                      _))
                  (`self.K2_DestroyActor`))))
            (:`else`)))))
    (:`else`)))

(event `Set Event Ready`
  (set `self.IsEventReady?` true)
  (`PrimitiveComponent.SetCollisionEnabled` (`self.Cube`) "QueryAndPhysics")
  (bind _returnvalue (`GameplayStatics.SpawnSoundAtLocation` "/Game/Sounds/BasketballBounce/sfx_basketball_dribbling.sfx_basketball_dribbling" (`self.K2_GetActorLocation` self) (struct) 1.0 1.0 0.0 "/Game/Sounds/BasketballBounce/SA_ProximitySound.SA_ProximitySound" null))
  (set `self.BasketballSound` _returnvalue))

(fn `UserConstructionScript`
  (`parent.UserConstructionScript`))