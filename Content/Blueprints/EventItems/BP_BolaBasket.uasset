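; Event item for a mysterious basketball that gets thrown when its Enabler fires the ThrowMysteriousBall event.
; The event makes the ball visible, enables collision and physics, and launches it with an impulse.
; Hits play a bounce sound with speed-scaled volume through a gate that closes after each bounce and reopens when CamouflageSphere ends an overlap.
; In chapter 3, the first bounce also triggers dialogue once after a short delay.
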(event `self.ReceiveBeginPlay`
  (bind _enabler (`self.Enabler`))
  (`parent.ReceiveBeginPlay`)
  (`/Engine/EditorBlueprintResources/StandardMacros.IsValid` _enabler
    (:`Is Valid`
      (add `/Game/Blueprints/Levels/Trigger_Bola_1.Throw Mysterious Ball` _enabler (delegate `/Game/Blueprints/Interface/BPI_Executable.Execute`))
      (`PrimitiveComponent.SetCollisionEnabled` (`self.Property Item`) "NoCollision"))))

(event `/Game/Blueprints/Interface/BPI_Executable.Execute`
  (`PrimitiveComponent.SetCollisionEnabled` (`self.Property Item`) "QueryAndPhysics")
  (`SceneComponent.SetVisibility` (`self.Property Item`) true false)
  (`PrimitiveComponent.SetSimulatePhysics` (`self.Property Item`) true)
  (`PrimitiveComponent.AddImpulse` (`self.Property Item`) (0.0 300.0 500.0) "None" true))

(event `self.Property Item.OnComponentHit`
  (params (HitComponent :type "PrimitiveComponent Object Reference") (OtherActor :type "Actor Object Reference") (OtherComp :type "PrimitiveComponent Object Reference") (NormalImpulse :type "Vector Structure") (Hit :type "HitResult Structure (by ref)"))
  (bind _returnvalue (`PrimitiveComponent.GetPhysicsLinearVelocity` (`self.Property Item`) "None"))
  (`/Engine/EditorBlueprintResources/StandardMacros.Gate` false :!label _label
    (:`Exit`
      (`GameplayStatics.PlaySoundAtLocation` "/Game/Sounds/BasketballBounce/sfx_basketball_bounce_cue.sfx_basketball_bounce_cue" (`SceneComponent.K2_GetComponentLocation` (`self.Property Item`)) (struct) (`KismetMathLibrary.MapRangeClamped` (`KismetMathLibrary.VSize` _returnvalue) 10.0 100.0 0.1 0.5) (`KismetMathLibrary.MapRangeClamped` (`KismetMathLibrary.VSize` (0.0 0.0 0.0)) 50.0 5000.0 0.9 1.1) 0.0 "/Game/Sounds/BasketballBounce/SA_ProximitySound.SA_ProximitySound" null null null)
      (`|ExecutionSequence`
        (:`then_0`
          (if (== (`/Game/FirstPerson/Blueprints/BP_FirstPersonCharacter.CurrentChapter` (`self.Player Ref`)) 3)
            (`/Engine/EditorBlueprintResources/StandardMacros.DoOnce` false
              (:`Completed`
                (`KismetSystemLibrary.Delay` 2.0)
                (`/Game/Blueprints/Components/BP_DialogueComponent.ShowDialogue` (`self.BP_DialogueComponent`) (`self.Player Ref`) self)))))
        (:`then_1`
          (goto _label :!via `Close`))))))

(event `self.CamouflageSphere.OnComponentEndOverlap`
  (params (OverlappedComponent :type "PrimitiveComponent Object Reference") (OtherActor :type "Actor Object Reference") (OtherComp :type "PrimitiveComponent Object Reference") (OtherBodyIndex :type Integer))
  (goto _label :!via `Open`))

(fn `UserConstructionScript`
  (`parent.UserConstructionScript`))