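; Bus event actor that plays a scripted bus ride cinematic and later returns the player from the bus camera.
; Execute teleports the bus to its cached BeginPlay location, initializes its child-actor BP_BusCamera as the level camera without blending, then plays the Anim_Bus level sequence.
; TakeOffBus triggers a screen fade and binds EndBusCamera to its completion, which ends the level camera.
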(event `self.ReceiveBeginPlay`
  (`parent.ReceiveBeginPlay`)
  (set `self.Initial Location` (`self.K2_GetActorLocation`)))

(event `/Game/Blueprints/Interface/BPI_Executable.Execute`
  (`self.K2_SetActorLocation` (`self.Initial Location`) false true)
  (bind _asbp_bus_camera (cast `/Game/Blueprints/LevelCameras/BP_BusCamera` (`ChildActorComponent.ChildActor` (`self.ChildActor`))))
  (bind _output_get (set `self.As BP Bus Camera` _asbp_bus_camera))
  (`/Game/Blueprints/ModularItems/BP_LevelCamera.Initialize Level Camera` _output_get (`self.Player Pref`) 0.0)
  (bind (_outactor _returnvalue) (`LevelSequencePlayer.CreateLevelSequencePlayer` "/Game/Animation/Anim_Bus.Anim_Bus"))
  (`MovieSceneSequencePlayer.Play` _returnvalue))

(event `Take Off Bus`
  (bind _bp_fadescreencomponent (`self.BP_FadeScreenComponent`))
  (`/Game/Blueprints/Components/BP_FadeScreenComponent.Fade Event` _bp_fadescreencomponent 3.0 (`self.Player Pref`) 0.0)
  (add `/Game/Blueprints/Components/BP_FadeScreenComponent.OnFadeEventFinished` _bp_fadescreencomponent (delegate `End Bus Camera`)))

(event `End Bus Camera`
  (bind _as_bp_bus_camera (`self.As BP Bus Camera`)
    (:`then`
      (`/Game/Blueprints/ModularItems/BP_LevelCamera.End Level Camera` _as_bp_bus_camera))
    (:`else`)))

(fn `UserConstructionScript`
  (`parent.UserConstructionScript`))