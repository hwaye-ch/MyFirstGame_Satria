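; Event item actor that plays one-shot ambient sounds, despite its name covering more than cooking.
; Three custom events spawn cooking, woman crying or basketball dribbling sounds at the location of its PropertyItem component.
; Each sound uses the shared SA_ProximitySound attenuation with a fixed volume, with cooking quieter than the others.
; The actor holds no other logic, as BeginPlay is disabled and the construction script only calls its parent.
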(event `Play Cooking Sfx`
  (`GameplayStatics.SpawnSoundAtLocation` "/Game/Sounds/sfx_cooking.sfx_cooking" (`SceneComponent.K2_GetComponentLocation` (`self.Property Item`)) (struct) 0.3 1.0 0.0 "/Game/Sounds/BasketballBounce/SA_ProximitySound.SA_ProximitySound" null))

(event `Play Crying Sfx`
  (`GameplayStatics.SpawnSoundAtLocation` "/Game/Sounds/sfx_woman-crying.sfx_woman-crying" (`SceneComponent.K2_GetComponentLocation` (`self.Property Item`)) (struct) 0.7 1.0 0.0 "/Game/Sounds/BasketballBounce/SA_ProximitySound.SA_ProximitySound" null))

(event `Play Basketball Sfx`
  (`GameplayStatics.SpawnSoundAtLocation` "/Game/Sounds/BasketballBounce/sfx_basketball_dribbling.sfx_basketball_dribbling" (`SceneComponent.K2_GetComponentLocation` (`self.Property Item`)) (struct) 0.7 1.0 0.0 "/Game/Sounds/BasketballBounce/SA_ProximitySound.SA_ProximitySound" null))

(fn `UserConstructionScript`
  (`parent.UserConstructionScript`))