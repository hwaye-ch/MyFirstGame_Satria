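; BP_DadNormal is the father NPC for Chapter 7, a talkable character driven by BP_Chapter7AManager.
; When the manager's move event fires, he teleports to SpawnArea_Dad, stands, builds his movement- and look-blocking dialogue, and binds to the enable-dialogue event.
; A matching enum from that event marks him ready.
; Talking to him is gated on that flag, shows the dialogue, and signals the manager once with another enum value to chain NPC conversations.
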(event `self.ReceiveBeginPlay`
  (`parent.ReceiveBeginPlay`)
  (bind _returnvalue (`GameplayStatics.GetActorOfClass` "/Game/Blueprints/Items/BP_Chapter7AManager.BP_Chapter7AManager_C"))
  (bind _output_get (set `self.ChapterManager` _returnvalue))
  (add `/Game/Blueprints/Items/BP_Chapter7AManager.MoveNPCs` _output_get (delegate `MoveNPCs_Event`)))

(event `MoveNPCs_Event`
  (bind _returnvalue (`GameplayStatics.GetActorOfClass` "/Game/Blueprints/Levels/SpawnArea_Dad.SpawnArea_Dad_C"))
  (`self.K2_SetActorLocationAndRotation` (`self.K2_GetActorLocation` _returnvalue) (`self.K2_GetActorRotation` _returnvalue))
  (set `self.IsStanding` true)
  (`/Game/Blueprints/Components/BP_DialogueComponent.Construct Dialogue` (`self.BP_DialogueComponent`) "ch7_father_0" "/Game/Dialogue/Chapter7_Dialogue.Chapter7_Dialogue" true true)
  (add `/Game/Blueprints/Items/BP_Chapter7AManager.EnableDialogue` (`self.ChapterManager`) (delegate `EnableDialogue_Event`)))

(event `EnableDialogue_Event`
  (params (NPC :type "/Game/Blueprints/Enumerations/E_NPC Enum" :default "NewEnumerator0"))
  (if (`|EnumEquality` NPC "NewEnumerator1")
    (set `self.IsEventReady` true)))

(event `/Game/Blueprints/Interface/BPI_Talk.TalkWithObject`
  (`self.IsEventReady`
    (:`then`
      (`/Game/Blueprints/Components/BP_DialogueComponent.ShowDialogue` (`self.BP_DialogueComponent`) (`self.PlayerRef`) self)
      (`/Engine/EditorBlueprintResources/StandardMacros.DoOnce` false
        (:`Completed`
          (`/Game/Blueprints/Items/BP_Chapter7AManager.EnableDialogue` (`self.ChapterManager`) "NewEnumerator0"))))
    (:`else`)))

(fn `UserConstructionScript`
  (`parent.UserConstructionScript`))