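; Dining table event item that plays a one-time eating sequence and then hands progression on to the shower.
; An Enabler dispatcher marks the table ready and passes in the HeatedFood actor.
; Interaction shows an eating fade widget if ready, but regardless of readiness locks the player, waits, destroys the food and restores control.
; A delayed auto dialogue follows, then the EnableShower dispatcher fires.
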(event `/Game/Blueprints/Interface/BPI_Actionable.OnInteract`
  (bind _heated_food (`self.Heated Food`))
  (`/Engine/EditorBlueprintResources/StandardMacros.DoOnce` false
    (:`Completed`
      (`|ExecutionSequence`
        (:`then_0`
          (if (`/Game/Blueprints/Components/BP_EnablerComponent.IsReadyToInteract` (`self.BP_EnablerComponent`))
            (`/Engine/EditorBlueprintResources/StandardMacros.DoOnce` false
              (:`Completed`
                (bind _returnvalue (`|CreateWidget` "/Game/Blueprints/Widgets/WBP_FadeScreen.WBP_FadeScreen_C"))
                (`UserWidget.AddToViewport` _returnvalue 0)
                (`UserWidget.PlayAnimation` _returnvalue (`/Game/Blueprints/Widgets/WBP_FadeScreen.EatSequence` _returnvalue) 0.0 1 "Forward" 1.0 false)))))
        (:`then_1`
          (`/Game/FirstPerson/Blueprints/BP_FirstPersonCharacter.Disable Movement and Look` (`self.Player Pref`))
          (`KismetSystemLibrary.Delay` (`self.ActionDuration`))
          (`KismetSystemLibrary.PrintString` "Mackan")
          (`/Engine/EditorBlueprintResources/StandardMacros.IsValid` _heated_food
            (:`Is Valid`
              (`self.K2_DestroyActor` _heated_food))
            (:`Is Not Valid`
              _))
          (set `/Game/FirstPerson/Blueprints/BP_FirstPersonCharacter.IsInteractionBlocked` false (`self.Player Pref`))
          (`/Game/FirstPerson/Blueprints/BP_FirstPersonCharacter.Enable Look and Movement` (`self.Player Pref`))
          (`self.Show Dialogue After Eating`))))))

(event `self.ReceiveBeginPlay`
  (bind _enabler (`self.Enabler`))
  (`/Engine/EditorBlueprintResources/StandardMacros.IsValid` _enabler
    (:`Is Valid`
      (add `/Game/Blueprints/EventItems/BP_Microwave.EnableDiningTable` _enabler (delegate `Enable Dining Table`)))))

(event `Enable Dining Table`
  (params (HeatedFood :type "/Game/Blueprints/EventItems/BP_HeatedFood Object Reference"))
  (set `/Game/Blueprints/Components/BP_EnablerComponent.IsReadyToInteract` true (`self.BP_EnablerComponent`))
  (`KismetSystemLibrary.PrintString` "Ammm enak bous kenyank")
  (set `self.Heated Food` HeatedFood))

(event `Show Dialogue After Eating`
  (`KismetSystemLibrary.Delay` (`self.DurationBeforeDialogue`))
  (message `/Game/Blueprints/Interface/BPI_Dialogue.DisplayAutoDialogue` (`self.BP_DialogueComponent`))
  (`self.EnableShower`))

(fn `UserConstructionScript`)