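; BP_DisturbanceSfx is an event actor that plays disturbance sounds in the world: cooking, a woman crying and basketball dribbling.
; Each sound has its own event, which spawns it at PropertyItem's location with proximity attenuation and stores the audio component.
; StopAllSounds stops any valid components, but only the valid basketball branch goes on to destroy the actor after a short delay.
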(event `Play Cooking Sfx`
  (bind _returnvalue (`GameplayStatics.SpawnSoundAtLocation` "/Game/Sounds/sfx_cooking.sfx_cooking" (`SceneComponent.K2_GetComponentLocation` (`self.Property Item`)) (struct) 0.3 1.0 0.0 "/Game/Sounds/BasketballBounce/SA_ProximitySound.SA_ProximitySound" null))
  (set `self.Cooking Sfx` _returnvalue))

(event `Play Crying Sfx`
  (bind _returnvalue (`GameplayStatics.SpawnSoundAtLocation` "/Game/Sounds/sfx_woman-crying.sfx_woman-crying" (`SceneComponent.K2_GetComponentLocation` (`self.Property Item`)) (struct) 0.7 1.0 0.0 "/Game/Sounds/BasketballBounce/SA_ProximitySound.SA_ProximitySound" null))
  (set `self.Crying Sfx` _returnvalue))

(event `Play Basketball Sfx`
  (bind _returnvalue (`GameplayStatics.SpawnSoundAtLocation` "/Game/Sounds/BasketballBounce/sfx_basketball_dribbling.sfx_basketball_dribbling" (`SceneComponent.K2_GetComponentLocation` (`self.Property Item`)) (struct) 0.7 1.0 0.0 "/Game/Sounds/BasketballBounce/SA_ProximitySound.SA_ProximitySound" null))
  (set `self.Basketball Sfx` _returnvalue))

(event `Stop All Sounds`
  (bind _cooking_sfx (`self.Cooking Sfx`)
    (:`then`
      (`AudioComponent.Stop` _cooking_sfx))
    (:`else`
      _))
  (bind _crying_sfx (`self.Crying Sfx`)
    (:`then`
      (`AudioComponent.Stop` _crying_sfx))
    (:`else`
      _))
  (bind _basketball_sfx (`self.Basketball Sfx`)
    (:`then`
      (`AudioComponent.Stop` _basketball_sfx)
      (`KismetSystemLibrary.Delay` 5.0)
      (`self.K2_DestroyActor`))
    (:`else`)))

(fn `UserConstructionScript`
  (`parent.UserConstructionScript`))