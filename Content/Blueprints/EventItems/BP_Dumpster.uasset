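; BP_Dumpster is an event item that takes trash the player holds and tracks a trash-collection mission.
; An Enabler event shows the mission widget with a collected/max progress count.
; Each combine destroys the held item, increments the collectible component's count, plays a dump sound and refreshes the widget.
; When the count reaches the maximum, it removes the widget after a short delay and calls the Mikey room activation event.
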(event `self.ReceiveBeginPlay`
  (bind _enabler (`self.Enabler`))
  (`parent.ReceiveBeginPlay`)
  (`/Engine/EditorBlueprintResources/StandardMacros.IsValid` _enabler
    (:`Is Valid`
      (add `/Game/Blueprints/Levels/Trigger_Welcome.StartCountingTrash` _enabler (delegate `Display GUI Counting Trash`))
      (`self.Construct Collectible`))))

(event `Display GUI Counting Trash`
  (bind _returnvalue (`|CreateWidget` "/Game/Blueprints/Widgets/WBP_MissionWidget.WBP_MissionWidget_C" null (`self.TempCollectibleText`) (`self.Mission Text`)))
  (set `self.Mission Widget` _returnvalue)
  (`UserWidget.AddToViewport` _returnvalue 0))

(event `/Game/Blueprints/Interface/BPI_Combine.OnCombineObject`
  (bind _bp_collectiblecomponent (`self.BP_CollectibleComponent`))
  (bind _bp_collectiblecomponent_2 (`self.BP_CollectibleComponent`))
  (`KismetSystemLibrary.PrintString` "Aku siap menampung sampah")
  (`/Game/FirstPerson/Blueprints/BP_FirstPersonCharacter.Destroy Holding Item` (`self.Player Pref`))
  (set `/Game/Blueprints/Components/BP_CollectibleComponent.CurrentCollectedItem` (+ (`/Game/Blueprints/Components/BP_CollectibleComponent.CurrentCollectedItem` _bp_collectiblecomponent_2) 1) _bp_collectiblecomponent_2)
  (`self.Construct Collectible`)
  (`GameplayStatics.PlaySound2D` "/Game/Sounds/sfx_dump_trash.sfx_dump_trash" 1.0 1.0 0.0 null null)
  (`/Game/Blueprints/Widgets/WBP_MissionWidget.Update Collectible` (`self.Mission Widget`) (`self.TempCollectibleText`) (`self.Mission Text`))
  (if (== (`/Game/Blueprints/Components/BP_CollectibleComponent.CurrentCollectedItem` _bp_collectiblecomponent) (`/Game/Blueprints/Components/BP_CollectibleComponent.MaxCollectibleItem` _bp_collectiblecomponent))
    (`KismetSystemLibrary.PrintString` "Congrats!!!")
    (`KismetSystemLibrary.Delay` 3.0)
    (`Widget.RemoveFromParent` (`self.Mission Widget`))
    (`self.ActivateMikeyRoomEvent`)))

(event `Construct Collectible`
  (bind _bp_collectiblecomponent (`self.BP_CollectibleComponent`))
  (set `self.TempCollectibleText` (`KismetStringLibrary.Concat_StrStr` (`KismetStringLibrary.Conv_IntToString` (`/Game/Blueprints/Components/BP_CollectibleComponent.CurrentCollectedItem` _bp_collectiblecomponent)) " / " (`KismetStringLibrary.Conv_IntToString` (`/Game/Blueprints/Components/BP_CollectibleComponent.MaxCollectibleItem` _bp_collectiblecomponent)))))

(fn `UserConstructionScript`
  (`parent.UserConstructionScript`))