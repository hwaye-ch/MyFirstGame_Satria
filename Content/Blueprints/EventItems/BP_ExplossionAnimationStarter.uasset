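; Event actor that plays the basketball-scene Level Sequence and stages an explosion with fire.
; CutsceneEnabler triggers the cutscene, which locks player movement and look, then restores look and repositions the car beside this actor on finish.
; A separate Ledakkan! event fires the explosion and delayed fire effects, then moves the player to SpawnArea, aimed toward this actor with a downward pitch offset.
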(event `self.ReceiveBeginPlay`
  (bind _cutsceneenabler (`self.CutsceneEnabler`))
  (`parent.ReceiveBeginPlay`)
  (`/Engine/EditorBlueprintResources/StandardMacros.IsValid` _cutsceneenabler
    (:`Is Valid`
      (add `/Game/Blueprints/Levels/Trigger_CarCrashScene.PlayCutsceneAnimation` _cutsceneenabler (delegate `/Game/Blueprints/Interface/BPI_Executable.Execute`))
      (`ActorComponent.SetActive` (`self.NS_Explossion`) false false)
      (`KismetSystemLibrary.Delay` 1.0)
      (`ActorComponent.SetActive` (`self.NS_Fire`) false false))))

(event `/Game/Blueprints/Interface/BPI_Executable.Execute`
  (`KismetSystemLibrary.PrintString` "Playing Cutscene" true true (struct :`R` 1.0 :`B` 0.175299 :`A` 1.0))
  (bind (_outactor _returnvalue) (`LevelSequencePlayer.CreateLevelSequencePlayer` "/Game/Animation/Anim_BasketballScene.Anim_BasketballScene"))
  (`MovieSceneSequencePlayer.Play` _returnvalue)
  (`/Game/FirstPerson/Blueprints/BP_FirstPersonCharacter.Disable Movement and Look` (`self.Player Pref`))
  (add `MovieSceneSequencePlayer.OnFinished` _returnvalue (delegate `OnFinishedCutscene`)))

(event `OnFinishedCutscene`
  (bind (_returnvalue_roll _returnvalue_pitch _returnvalue_yaw) (`KismetMathLibrary.BreakRotator` (`self.K2_GetActorRotation` self)))
  (`/Game/FirstPerson/Blueprints/BP_FirstPersonCharacter.Enable Look` (`self.Player Pref`))
  (`self.K2_SetActorLocationAndRotation` (`self.CarActor`) (+ (`self.K2_GetActorLocation` self) (0.0 -150.0 100.0)) (`KismetMathLibrary.MakeRotator` _returnvalue_roll _returnvalue_pitch (- _returnvalue_yaw 90.0)) false true))

(event `Ledakkan!`
  (bind (_returnvalue_roll _returnvalue_pitch _returnvalue_yaw) (`KismetMathLibrary.BreakRotator` (`KismetMathLibrary.FindLookAtRotation` (`self.K2_GetActorLocation` (`self.Player Pref`)) (`self.K2_GetActorLocation` self))))
  (`ActorComponent.SetActive` (`self.NS_Explossion`) true false)
  (`KismetSystemLibrary.Delay` 1.0)
  (`ActorComponent.SetActive` (`self.NS_Fire`) true false)
  (`KismetSystemLibrary.Delay` 2.0)
  (`self.K2_SetActorLocation` (`self.Player Pref`) (`self.K2_GetActorLocation` (`self.SpawnArea`)) false false)
  (`Controller.SetControlRotation` (`GameplayStatics.GetPlayerController` 0) (`KismetMathLibrary.MakeRotator` _returnvalue_roll (+ _returnvalue_pitch -50.0) _returnvalue_yaw)))

(fn `UserConstructionScript`
  (`parent.UserConstructionScript`))