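; BP_FatherOnBed is an event item that reveals the father's skeletal mesh on the bed and turns the bed camera toward him.
; The mesh is hidden at BeginPlay until ShowDanonBed makes it visible.
; After a short delay, a timeline lerps the BP_BedCamera camera from its current rotation toward the mesh's look-at rotation, changing only yaw.
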(event `self.ReceiveBeginPlay`
  (`parent.ReceiveBeginPlay`)
  (`SceneComponent.SetVisibility` (`self.SkeletalMesh`) false false))

(event `Show Dan on Bed`
  (`SceneComponent.SetVisibility` (`self.SkeletalMesh`) true false)
  (`KismetSystemLibrary.Delay` 3.0)
  (bind _returnvalue (`GameplayStatics.GetActorOfClass` "/Game/Blueprints/LevelCameras/BP_BedCamera.BP_BedCamera_C"))
  (bind (_direction _newtrack_0) (`Timeline|Timeline` :!via `PlayFromStart`)
    (:`Update`
      (bind _camera (`/Game/Blueprints/ModularItems/BP_LevelCamera.Camera` _returnvalue))
      (bind (_returnvalue_roll _returnvalue_pitch) (`KismetMathLibrary.BreakRotator` (`SceneComponent.K2_GetComponentRotation` _camera)))
      (bind (_returnvalue_roll_2 _returnvalue_pitch_2 _returnvalue_yaw) (`KismetMathLibrary.BreakRotator` (`KismetMathLibrary.RLerp` (`SceneComponent.K2_GetComponentRotation` _camera) (`KismetMathLibrary.FindLookAtRotation` (`SceneComponent.K2_GetComponentLocation` _camera) (`SceneComponent.K2_GetComponentLocation` (`self.SkeletalMesh`))) _newtrack_0)))
      (`SceneComponent.K2_SetWorldRotation` _camera (`KismetMathLibrary.MakeRotator` _returnvalue_roll _returnvalue_pitch _returnvalue_yaw) false false))))

(fn `UserConstructionScript`
  (`parent.UserConstructionScript`))