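; BP_FatherPeepingDoor is an event actor for the father peeping at a door, hidden when play begins.
; Peep reveals the skeletal mesh, spawns a breathing sound and runs a timeline sliding the actor along world Y by MoveLength.
; Returnfrompeep sets a finishing flag and reverses that timeline, whose Finished branch checks the flag to stop the sound and destroy the actor.
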(event `self.ReceiveBeginPlay`
  (`parent.ReceiveBeginPlay`)
  (`SceneComponent.SetVisibility` (`self.SkeletalMesh`) false false))

(event `Peep`
  (bind (_startlocation_x _startlocation_y _startlocation_z) (`KismetMathLibrary.BreakVector` (`self.StartLocation`)))
  (`SceneComponent.SetVisibility` (`self.SkeletalMesh`) true false)
  (`KismetSystemLibrary.DelayUntilNextTick`)
  (bind _output_get (set `self.StartLocation` (`self.K2_GetActorLocation`)))
  (bind _returnvalue (`GameplayStatics.SpawnSoundAtLocation` "/Game/Sounds/sfx_father-breath.sfx_father-breath" _output_get (struct) 0.5 1.0 0.0 "/Game/Sounds/BasketballBounce/SA_ProximitySound.SA_ProximitySound" null))
  (set `self.Sound of Father` _returnvalue)
  (bind (_direction _alpha) (`Timeline|Timeline` :!via `PlayFromStart` :!label _label)
    (:`Update`
      (`self.K2_SetActorLocation` (`KismetMathLibrary.MakeVector` _startlocation_x (`KismetMathLibrary.Lerp` _startlocation_y (+ _startlocation_y (`self.MoveLength`)) _alpha) _startlocation_z)))
    (:`Finished`
      (`self.IsFinishing`
        (:`then`
          (`AudioComponent.Stop` (`self.Sound of Father`))
          (`self.K2_DestroyActor`))
        (:`else`)))))

(event `Return from peep`
  (set `self.IsFinishing` true)
  (goto _label :!via `Reverse`))

(fn `UserConstructionScript`
  (`parent.UserConstructionScript`))