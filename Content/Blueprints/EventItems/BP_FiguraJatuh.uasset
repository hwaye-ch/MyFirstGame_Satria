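; BP_FiguraJatuh is an inspectable photo frame event item that falls when its Enabler fires the drop event.
; The fall briefly enables physics, plays a drop sound, then freezes the item and flags BPSequenceActivator as activated.
; Inspecting triggers delayed auto dialogue through BPDialogueComponent.
; Finishing inspection runs a DoOnce timed sequence that shows an animated WBP_Chat message, removes it, then calls CallEnableBed.
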(event `self.ReceiveBeginPlay`
  (bind _enabler (`self.Enabler`))
  (set `self.Initial Location` (`SceneComponent.K2_GetComponentLocation` (`self.InspectableItem`)))
  (set `self.Initial Rotation` (`SceneComponent.K2_GetComponentRotation` (`self.InspectableItem`)))
  (`/Engine/EditorBlueprintResources/StandardMacros.IsValid` _enabler
    (:`Is Valid`
      (add `/Game/Blueprints/Levels/Trigger_FrameJatuh.DropPhotoFrame` _enabler (delegate `Simulate Photo Physics`))
      (set `self.IsLocationChangedInChild` true))))

(event `Simulate Photo Physics`
  (`PrimitiveComponent.SetSimulatePhysics` (`self.InspectableItem`) true)
  (`KismetSystemLibrary.Delay` 0.5)
  (`GameplayStatics.PlaySound2D` "/Game/Sounds/photo_frame_dropped.photo_frame_dropped" 1.0 1.0 0.0 null null)
  (`KismetSystemLibrary.Delay` 1.0)
  (`PrimitiveComponent.SetSimulatePhysics` (`self.InspectableItem`) false)
  (set `/Game/Blueprints/Components/BP_SequenceActivator.IsSequenceActivated` true (`self.BP_SequenceActivator`)))

(event `self.OnProgressInspecting`
  (`KismetSystemLibrary.Delay` (`self.DelayBeforeDialogue`))
  (message `/Game/Blueprints/Interface/BPI_Dialogue.DisplayAutoDialogue` (`self.BP_DialogueComponent`)))

(event `self.OnFinishedInspecting`
  (`/Engine/EditorBlueprintResources/StandardMacros.DoOnce` false
    (:`Completed`
      (`KismetSystemLibrary.PrintString` "Hao aku sudah selesai inspecting")
      (`KismetSystemLibrary.Delay` 10.0)
      (bind _returnvalue (`|CreateWidget` "/Game/Blueprints/Widgets/WBP_Chat.WBP_Chat_C"))
      (`UserWidget.AddToViewport` _returnvalue 0)
      (`UserWidget.PlayAnimation` _returnvalue (`/Game/Blueprints/Widgets/WBP_Chat.DisplayMessage` _returnvalue) 0.0 1 "Forward" 1.0 false)
      (`KismetSystemLibrary.Delay` 5.0)
      (`Widget.RemoveFromParent` _returnvalue)
      (`KismetSystemLibrary.Delay` 5.0)
      (`self.EnableBed`))))

(fn `UserConstructionScript`
  (`parent.UserConstructionScript`))