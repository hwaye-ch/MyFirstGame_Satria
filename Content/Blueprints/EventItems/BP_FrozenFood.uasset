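; BP_FrozenFood is an event item pickup for frozen food.
; Its PickupObject event sets the item code on BPActivatorComponent to a fixed enum value and prints that code to screen.
; While IsRotating is set, Tick spins the Pickupable component around its local yaw, scaled by frame time and the Rotation variable.
; The construction script only calls the parent's.
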(event `/Game/Blueprints/Interface/BPI_Pickup.PickupObject`
  (bind _output_get (set `/Game/Blueprints/Components/BP_ActivatorComponent.ActivatorItemCode` "NewEnumerator0" (`self.BP_ActivatorComponent`)))
  (`KismetSystemLibrary.PrintString` (`|GetEnumeratorNameAsString` _output_get)))

(event `self.ReceiveTick`
  (params (DeltaSeconds :type "Float (single-precision)"))
  (if (`self.IsRotating`)
    (`SceneComponent.K2_AddLocalRotation` (`self.Pickupable`) (`KismetMathLibrary.MakeRotator` 0.0 0.0 (* DeltaSeconds (`self.Rotation`))) false false)))

(fn `UserConstructionScript`
  (`parent.UserConstructionScript`))