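; BP_HeatedFood is an event item, named as heated food, that the player can pick up and throw.
; SpawnObject runs PickupObject, which copies mesh, scale and activator item code to the player, then destroys the actor or mesh component according to BPSpawnerComponent flags.
; ThrowObject moves the held mesh back onto this actor, launches it with a physics impulse, clears the player's hand and flags the actor for destruction on next pickup.
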(event `Destroy Item`
  (`KismetSystemLibrary.Delay` 0.01)
  (`self.K2_DestroyActor`))

(event `self.SpawnObject`
  (params (PlayerPref :type "/Game/FirstPerson/Blueprints/BP_FirstPersonCharacter Object Reference"))
  (`/Game/Blueprints/Interface/BPI_Pickup.PickupObject` PlayerPref))

(fn `PickupObject`
  (params (PlayerPref :type "/Game/FirstPerson/Blueprints/BP_FirstPersonCharacter Object Reference"))
  (returns (ThrowableActor :type "/Game/Blueprints/ModularItems/BP_PickupableItem Object Reference"))
  (bind _bp_spawnercomponent (`self.BP_SpawnerComponent`))
  (bind _pickupable (`self.Pickupable`))
  (bind _pickupable_position (`/Game/FirstPerson/Blueprints/BP_FirstPersonCharacter.Pickupable Position` PlayerPref))
  (bind _returnvalue (`SceneComponent.K2_GetComponentScale` _pickupable))
  (bind _staticmesh (`StaticMeshComponent.StaticMesh` _pickupable))
  (`/Engine/EditorBlueprintResources/StandardMacros.IsValid` _pickupable
    (:`Is Valid`
      (set `/Game/FirstPerson/Blueprints/BP_FirstPersonCharacter.MeshPickupable` _staticmesh PlayerPref)
      (set `/Game/FirstPerson/Blueprints/BP_FirstPersonCharacter.PickupableVector` _returnvalue PlayerPref)
      (`StaticMeshComponent.SetStaticMesh` _pickupable_position _staticmesh)
      (`SceneComponent.SetWorldScale3D` _pickupable_position _returnvalue)
      (set `/Game/FirstPerson/Blueprints/BP_FirstPersonCharacter.IsHoldingItem` true PlayerPref)
      (set `/Game/FirstPerson/Blueprints/BP_FirstPersonCharacter.ActivatorObjectName` (`/Game/Blueprints/Components/BP_ActivatorComponent.ActivatorItemCode` (`self.BP_ActivatorComponent`)) PlayerPref)
      (if (`/Game/Blueprints/Components/BP_SpawnerComponent.DestroyAfterInteract` _bp_spawnercomponent)
        (`self.Destroy Item`)
        (elif (`/Game/Blueprints/Components/BP_SpawnerComponent.DestroySpawnee` _bp_spawnercomponent)
          (`ActorComponent.K2_DestroyComponent` (`self.Pickupable`))))
      (return null))
    (:`Is Not Valid`
      (`KismetSystemLibrary.PrintString` "Destroyed :("))))

(fn `ThrowObject`
  (params (PlayerPref :type "/Game/FirstPerson/Blueprints/BP_FirstPersonCharacter Object Reference"))
  (bind _pickupable (`self.Pickupable`))
  (bind _bp_spawnercomponent (`self.BP_SpawnerComponent`))
  (bind _meshpickupable (`/Game/FirstPerson/Blueprints/BP_FirstPersonCharacter.MeshPickupable` (`self.PlayerPref`)))
  (set `/Game/Blueprints/Components/BP_SpawnerComponent.DestroyAfterInteract` true _bp_spawnercomponent)
  (set `/Game/Blueprints/Components/BP_SpawnerComponent.DestroySpawnee` true _bp_spawnercomponent)
  (set `self.PlayerPref` PlayerPref)
  (`/Engine/EditorBlueprintResources/StandardMacros.IsValid` _meshpickupable
    (:`Is Valid`
      (`StaticMeshComponent.SetStaticMesh` _pickupable _meshpickupable)
      (`SceneComponent.SetWorldScale3D` _pickupable (`/Game/FirstPerson/Blueprints/BP_FirstPersonCharacter.PickupableVector` (`self.PlayerPref`)))
      (`PrimitiveComponent.SetSimulatePhysics` _pickupable true)
      (`PrimitiveComponent.AddImpulse` _pickupable (* (`self.GetActorForwardVector`) (`/Game/FirstPerson/Blueprints/BP_FirstPersonCharacter.ThrowForce` (`self.PlayerPref`))) "None" true)
      (`StaticMeshComponent.SetStaticMesh` (`/Game/FirstPerson/Blueprints/BP_FirstPersonCharacter.Pickupable Position` (`self.PlayerPref`)) null)
      (set `/Game/FirstPerson/Blueprints/BP_FirstPersonCharacter.IsHoldingItem` false (`self.PlayerPref`))
      (set `/Game/FirstPerson/Blueprints/BP_FirstPersonCharacter.MeshPickupable` null (`self.PlayerPref`))
      (return))))

(fn `UserConstructionScript`)