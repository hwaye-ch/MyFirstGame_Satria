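; BP_HouseTalking is an event item actor that plays people-talking audio at its location.
; PlayPeopleTalking, when enabled, prints a debug string, spawns the cue with proximity attenuation and the Volume multiplier, and stores the resulting audio component.
; When disabled, it stops that stored sound if it is still valid.
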(event `self.ReceiveBeginPlay`
  (`parent.ReceiveBeginPlay`))

(event `Play People Talking`
  (params (Enabled :type Boolean))
  (if Enabled
    (`KismetSystemLibrary.PrintString` "Playing House Talking")
    (bind _returnvalue (`GameplayStatics.SpawnSoundAtLocation` "/Game/Sounds/PeopleTalkingIntheHouse/sfx_people-talking-cue.sfx_people-talking-cue" (`self.K2_GetActorLocation`) (struct) (`self.Volume`) 1.0 0.0 "/Game/Sounds/BasketballBounce/SA_ProximitySound.SA_ProximitySound" null))
    (set `self.Sound` _returnvalue)
    (else
      (bind _sound (`self.Sound`)
        (:`then`
          (`AudioComponent.Stop` _sound))
        (:`else`)))))

(fn `UserConstructionScript`
  (`parent.UserConstructionScript`))