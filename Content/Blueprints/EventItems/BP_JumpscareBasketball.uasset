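; Event item that stages a jumpscare by launching a physics basketball at the player, once, shortly after BeginPlay.
; After a delay it spawns a BP_BasketballSpawner at its PropertyItem location and enables physics on that actor's PropertyItem.
; A mass-independent impulse toward the player then throws it, with the vertical component scaled down.
; An unwired Level Sequence playback of Anim_ch5balljumpscare remains in the graph and never runs.
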(event `self.ReceiveBeginPlay`
  (bind _returnvalue (`SceneComponent.K2_GetComponentLocation` (`self.Property Item`)))
  (`parent.ReceiveBeginPlay`)
  (`KismetSystemLibrary.Delay` 5.0)
  (bind _returnvalue_2 (`|SpawnActorFromClass` "/Game/Blueprints/EventItems/BP_BasketballSpawner.BP_BasketballSpawner_C" (`KismetMathLibrary.Conv_VectorToTransform` _returnvalue) "Undefined" "MultiplyWithRoot" null null))
  (`PrimitiveComponent.SetSimulatePhysics` (`/Game/Blueprints/ModularItems/BP_PropertyItem.Property Item` _returnvalue_2) true)
  (`PrimitiveComponent.AddImpulse` (`/Game/Blueprints/ModularItems/BP_PropertyItem.Property Item` _returnvalue_2) (* (`KismetMathLibrary.Normal` (- (`self.K2_GetActorLocation` (`self.Player Pref`)) _returnvalue)) (1000.0 1000.0 100.0)) "None" true)
  (`KismetSystemLibrary.Delay` 5.0))

(fn `UserConstructionScript`
  (`parent.UserConstructionScript`))