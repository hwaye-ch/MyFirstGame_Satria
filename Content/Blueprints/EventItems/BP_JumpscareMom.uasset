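; Jumpscare actor for a ghostly mom that flies into the player's face, leading into a wake-up-from-nightmare sequence.
; It hides both meshes and waits for the JumpscareEnabler dispatcher, then after a delay shows FlyingMom and timeline-lerps to just before the camera, spawning scare sounds every update.
; Afterwards it restores player control, plays the chapter 4 wake-up sequence, calls WakeUpFromNightmare and destroys itself.
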(event `self.ReceiveBeginPlay`
  (`parent.ReceiveBeginPlay`)
  (bind _jumpscareenabler (`self.JumpscareEnabler`)
    (:`then`
      (add `/Game/Blueprints/EventItems/BP_TriggerJumpscareOnLook.Call Jumpscare` _jumpscareenabler (delegate `/Game/Blueprints/Interface/BPI_Executable.Execute`))
      (set `self.GhostStartLocation` (`self.K2_GetActorLocation` self))
      (`SceneComponent.SetVisibility` (`self.FlyingMom`) false false)
      (`SceneComponent.SetVisibility` (`self.IdleMom`) false false))
    (:`else`)))

(event `/Game/Blueprints/Interface/BPI_Executable.Execute`
  (bind _firstpersoncamera (`/Game/FirstPerson/Blueprints/BP_FirstPersonCharacter.FirstPersonCamera` (`self.Player Pref`)))
  (`KismetSystemLibrary.Delay` 5.0)
  (`SceneComponent.SetVisibility` (`self.IdleMom`) false false)
  (`SceneComponent.SetVisibility` (`self.FlyingMom`) true false)
  (set `self.GhostEndLocation` (+ (`SceneComponent.K2_GetComponentLocation` _firstpersoncamera) (* (`SceneComponent.GetForwardVector` _firstpersoncamera) 20.0)))
  (bind (_direction _newtrack_0) (`Timeline|Timeline` :!via `PlayFromStart`)
    (:`Update`
      (`self.K2_SetActorLocation` (`KismetMathLibrary.VLerp` (`self.GhostStartLocation`) (`self.GhostEndLocation`) _newtrack_0))
      (`GameplayStatics.SpawnSound2D` "/Game/Sounds/sfx_jumpscare.sfx_jumpscare" 1.0 1.0 0.0 null)
      (`GameplayStatics.SpawnSound2D` "/Game/Sounds/sfx_tinnitus.sfx_tinnitus" 0.1 1.0 0.0 null))
    (:`Finished`
      (`KismetSystemLibrary.Delay` 2.0)
      (`SceneComponent.SetVisibility` (`self.FlyingMom`) false false)
      (`/Game/FirstPerson/Blueprints/BP_FirstPersonCharacter.Enable Look and Movement` (`self.Player Pref`))
      (bind (_outactor _returnvalue) (`LevelSequencePlayer.CreateLevelSequencePlayer` "/Game/Animation/Anim_ch4-WakeUpFromNightmare.Anim_ch4-WakeUpFromNightmare"))
      (`MovieSceneSequencePlayer.Play` _returnvalue)
      (add `MovieSceneSequencePlayer.OnFinished` _returnvalue (delegate `Listen to finished sequence`)))))

(event `Listen to finished sequence`
  (`self.WakeUpFromNightmare` (`self.Player Pref`))
  (`KismetSystemLibrary.Delay` 5.0)
  (`self.K2_DestroyActor`))

(fn `UserConstructionScript`
  (`parent.UserConstructionScript`))