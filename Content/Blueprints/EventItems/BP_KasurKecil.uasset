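; BP_KasurKecil is an interactable event item, a small bed ("kasur kecil"), that the player uses to sleep and move on to chapter 5.
; On BeginPlay it binds EnableKasur to the WakeUpFromNightmare event of KasurEnabler, if that reference is valid.
; EnableKasur logs readiness but sets CanInteract to false.
; Interacting passes a DoOnce, then calls the player's CallGoToNextChapter with a fade-in.
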(event `self.ReceiveBeginPlay`
  (bind _kasurenabler (`self.KasurEnabler`)
    (:`then`
      (add `/Game/Blueprints/EventItems/BP_JumpscareMom.WakeUpFromNightmare` _kasurenabler (delegate `Enable Kasur`)))
    (:`else`)))

(event `Enable Kasur`
  (params (PlayerPref :type "/Game/FirstPerson/Blueprints/BP_FirstPersonCharacter Object Reference"))
  (`KismetSystemLibrary.PrintString` "Kasur is ready to interact")
  (set `self.CanInteract?` false))

(event `self.OnInteract`
  (`/Engine/EditorBlueprintResources/StandardMacros.DoOnce` false
    (:`Completed`
      (`KismetSystemLibrary.PrintString` "Executing Sleep and Go to Next Chapter")
      (`/Game/FirstPerson/Blueprints/BP_FirstPersonCharacter.GoToNextChapter` (`self.PlayerRef`) 5 true))))

(fn `UserConstructionScript`
  (`parent.UserConstructionScript`))