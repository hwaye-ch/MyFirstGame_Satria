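; Interactable wall switch that turns a linked CeilingLamp's light on and off.
; Interacting plays an on or off click at the switch and flips its state, but updates the light's visibility and saved last-lit state only when neither lamp-dead flag is set.
; A TurnLamp event lets the light be set directly, bypassing those dead checks and leaving the saved state untouched.
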(event `self.ReceiveBeginPlay`
  (`parent.ReceiveBeginPlay`)
  (set `self.CanInteract?` true))

(event `Turn Lamp`
  (params (`On?` :type Boolean))
  (set `self.IsLightOn` `On?`)
  (bind _ceilinglamp (`self.CeilingLamp` :!label _label)
    (:`then`
      (bind _light (`/Game/Blueprints/Items/CeilingLamp.Light` _ceilinglamp)
        (:`then`
          (`SceneComponent.SetVisibility` _light (`self.IsLightOn`) false))
        (:`else`)))
    (:`else`)))

(event `/Game/Blueprints/Interface/BPI_Actionable.InteractObject`
  (bind _returnvalue (`self.K2_GetActorLocation` self))
  (`self.IsLightOn`
    (:`then`
      (`GameplayStatics.SpawnSoundAtLocation` "/Game/Sounds/sfx_light-off.sfx_light-off" _returnvalue (struct) 1.0 1.0 0.0 null null))
    (:`else`
      (`GameplayStatics.SpawnSoundAtLocation` "/Game/Sounds/sfx_light-on.sfx_light-on" _returnvalue (struct) 1.0 1.0 0.0 null null)))
  (set `self.IsLightOn` (not (`self.IsLightOn`)))
  (`self.IsLampDeadByEvent?`
    (:`then`)
    (:`else`
      (`self.IsLampDead`
        (:`then`)
        (:`else`
          (set `self.IsLastLampStateLit` (`self.IsLightOn`))
          (goto _label))))))

(fn `UserConstructionScript`
  (`parent.UserConstructionScript`))