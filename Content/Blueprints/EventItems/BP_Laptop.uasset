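; BP_Laptop is an interactable laptop that moves the player from one story chapter to the next.
; Bound events from three enabler references make it interactable.
; Interaction switches on the current chapter: chapters 1-3 freeze the player, play a fade widget and timed dialogue, then advance, while chapter 4 is a print-only placeholder.
; A DoOnce blocks repeats; chapter 3 shows dialogue and resets it until EndChapter is set.
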(event `self.ReceiveBeginPlay`
  (bind _enabler (`self.Enabler`))
  (bind _enabler_of_laptop (`self.Enabler of Laptop`))
  (bind _enabler_chapter_2 (`self.Enabler Chapter 2`))
  (`/Engine/EditorBlueprintResources/StandardMacros.IsValid` _enabler
    (:`Is Valid`
      (add `/Game/Blueprints/EventItems/BP_FiguraJatuh.EnableBed` _enabler (delegate `Enable Laptop`)))
    (:`Is Not Valid`
      _))
  (`/Engine/EditorBlueprintResources/StandardMacros.IsValid` _enabler_chapter_2
    (:`Is Valid`
      (add `/Game/Blueprints/Characters/BP_Janitor.ActivateLaptop` _enabler_chapter_2 (delegate `Enable Laptop Chapter 3`)))
    (:`Is Not Valid`
      _))
  (`/Engine/EditorBlueprintResources/StandardMacros.IsValid` _enabler_of_laptop
    (:`Is Valid`
      (add `/Game/Blueprints/Levels/Trigger_BasketballBouncingFromMikey.TriggerMikeyRoomEvent` _enabler_of_laptop (delegate `Enable Interact Laptop`)))))

(event `Enable Laptop`
  (message `/Game/Blueprints/Interface/BPI_Dialogue.DisplayAutoDialogue` (`self.BP_DialogueComponent`))
  (`KismetSystemLibrary.Delay` 5.0)
  (set `/Game/Blueprints/Components/BP_EnablerComponent.IsReadyToInteract` true (`self.BP_EnablerComponent`)))

(event `Enable Interact Laptop`
  (`KismetSystemLibrary.PrintString` "Laptop is activated")
  (set `/Game/Blueprints/Components/BP_EnablerComponent.IsReadyToInteract` true (`self.BP_EnablerComponent`)))

(event `Enable Laptop Chapter 3`
  (set `/Game/Blueprints/Components/BP_EnablerComponent.IsReadyToInteract` true (`self.BP_EnablerComponent`))
  (`self.Activate Object`)
  (set `self.EndChapter` true))

(event `/Game/Blueprints/Interface/BPI_Actionable.OnInteract`
  (bind _bp_dialoguecomponent (`self.BP_DialogueComponent`))
  (bind _bp_dialoguecomponent_2 (`self.BP_DialogueComponent`))
  (bind _bp_dialoguecomponent_3 (`self.BP_DialogueComponent`))
  (`/Engine/EditorBlueprintResources/StandardMacros.DoOnce` false :!label _label
    (:`Completed`
      (switch `int` (`/Game/FirstPerson/Blueprints/BP_FirstPersonCharacter.CurrentChapter` (`self.Player Pref`))
        (:`1`
          (`/Game/FirstPerson/Blueprints/BP_FirstPersonCharacter.Disable Movement and Look` (`self.Player Pref`))
          (bind _returnvalue (`|CreateWidget` "/Game/Blueprints/Widgets/WBP_FadeScreen.WBP_FadeScreen_C"))
          (`UserWidget.AddToViewport` _returnvalue 0)
          (`UserWidget.PlayAnimation` _returnvalue (`/Game/Blueprints/Widgets/WBP_FadeScreen.SleepSequence` _returnvalue) 0.0 1 "Forward" 1.0 false)
          (`KismetSystemLibrary.Delay` (`self.PreparationDuration`))
          (set `/Game/Blueprints/Components/BP_DialogueComponent.DialogueCode` "ch1_belajar" _bp_dialoguecomponent_2)
          (`/Game/Blueprints/Interface/BPI_Dialogue.DisplayAutoDialogue` _bp_dialoguecomponent_2)
          (`KismetSystemLibrary.Delay` (- (`self.SleepDuration`) (`self.PreparationDuration`)))
          (`/Game/FirstPerson/Blueprints/BP_FirstPersonCharacter.Enable Look and Movement` (`self.Player Pref`))
          (`Widget.RemoveFromParent` _returnvalue)
          (`/Game/FirstPerson/Blueprints/BP_FirstPersonCharacter.GoToNextChapter` (`self.Player Pref`) 2 true))
        (:`2`
          (`/Game/FirstPerson/Blueprints/BP_FirstPersonCharacter.Disable Movement and Look` (`self.Player Pref`))
          (bind _returnvalue_2 (`|CreateWidget` "/Game/Blueprints/Widgets/WBP_FadeScreen.WBP_FadeScreen_C"))
          (`UserWidget.AddToViewport` _returnvalue_2 0)
          (`UserWidget.PlayAnimation` _returnvalue_2 (`/Game/Blueprints/Widgets/WBP_FadeScreen.FadeOutSequence` _returnvalue_2) 0.0 1 "Forward" 1.0 false)
          (`KismetSystemLibrary.Delay` (`self.MisuhMisuhDuration`))
          (set `/Game/Blueprints/Components/BP_DialogueComponent.DialogueCode` "ch2_tired_1" _bp_dialoguecomponent_3)
          (set `/Game/Blueprints/Components/BP_DialogueComponent.DialogueTable` "/Game/Dialogue/Chapter2_Dialogue.Chapter2_Dialogue" _bp_dialoguecomponent_3)
          (`/Game/Blueprints/Interface/BPI_Dialogue.DisplayAutoDialogue` _bp_dialoguecomponent_3)
          (`KismetSystemLibrary.Delay` (- (`self.SleepDurationChapter2`) (`self.MisuhMisuhDuration`)))
          (`Widget.RemoveFromParent` _returnvalue_2)
          (`/Game/FirstPerson/Blueprints/BP_FirstPersonCharacter.Enable Look and Movement` (`self.Player Pref`))
          (`/Game/FirstPerson/Blueprints/BP_FirstPersonCharacter.GoToNextChapter` (`self.Player Pref`) 3 true))
        (:`3`
          (if (`self.EndChapter`)
            (`/Game/FirstPerson/Blueprints/BP_FirstPersonCharacter.Disable Movement and Look` (`self.Player Pref`))
            (bind _returnvalue_3 (`|CreateWidget` "/Game/Blueprints/Widgets/WBP_FadeScreen.WBP_FadeScreen_C"))
            (`UserWidget.AddToViewport` _returnvalue_3 0)
            (`UserWidget.PlayAnimation` _returnvalue_3 (`/Game/Blueprints/Widgets/WBP_FadeScreen.FadeOutSequence` _returnvalue_3) 0.0 1 "Forward" 1.0 false)
            (`KismetSystemLibrary.Delay` (`self.MisuhMisuhDuration`))
            (set `/Game/Blueprints/Components/BP_DialogueComponent.DialogueCode` "ch3_tired_0" _bp_dialoguecomponent)
            (set `/Game/Blueprints/Components/BP_DialogueComponent.DialogueTable` "/Game/Dialogue/Chapter3_Dialogue.Chapter3_Dialogue" _bp_dialoguecomponent)
            (`/Game/Blueprints/Interface/BPI_Dialogue.DisplayAutoDialogue` _bp_dialoguecomponent)
            (`KismetSystemLibrary.Delay` (- (`self.SleepDurationChapter2`) (`self.MisuhMisuhDuration`)))
            (`Widget.RemoveFromParent` _returnvalue_3)
            (`/Game/FirstPerson/Blueprints/BP_FirstPersonCharacter.Enable Look and Movement` (`self.Player Pref`))
            (`/Game/FirstPerson/Blueprints/BP_FirstPersonCharacter.GoToNextChapter` (`self.Player Pref`) 4 true)
            (else
              (`/Game/Blueprints/Components/BP_DialogueComponent.Construct Dialogue` (`self.BP_DialogueComponent`) "ch3_disturbed_by_basketball" "/Game/Dialogue/Chapter3_Dialogue.Chapter3_Dialogue" true true)
              (message `/Game/Blueprints/Interface/BPI_Dialogue.ShowDialogue` (`self.BP_DialogueComponent`) (`self.Player Pref`) self)
              (`self.Activate Object`))))
        (:`4`
          (`KismetSystemLibrary.PrintString` "I supposed to be progress bar mechanism"))))))

(event `Activate Object`
  (goto _label :!via `Reset`))

(fn `UserConstructionScript`
  (`parent.UserConstructionScript`))