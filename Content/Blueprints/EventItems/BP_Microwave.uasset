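; BP_Microwave is an event item that turns the player's held item into heated food.
; On combine, it plays a microwaving screen animation, locks movement and look, and clears the held item.
; A chain of delays shows the food, spins it on Tick under the light, then hides it.
; It then attaches a spawned BP_HeatedFood to the player's hold position, restores control, blocks interaction and calls to enable the dining table.
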(event `/Game/Blueprints/Interface/BPI_Combine.OnCombineObject`
  (bind _player_pref (`self.Player Pref`))
  (bind _player_pref_2 (`self.Player Pref`))
  (bind _hold_position (`/Game/FirstPerson/Blueprints/BP_FirstPersonCharacter.Hold Position` (`self.Player Pref`)))
  (`|ExecutionSequence`
    (:`then_0`
      (bind _returnvalue (`|CreateWidget` "/Game/Blueprints/Widgets/WBP_FadeScreen.WBP_FadeScreen_C"))
      (`UserWidget.AddToViewport` _returnvalue 0)
      (`UserWidget.PlayAnimation` _returnvalue (`/Game/Blueprints/Widgets/WBP_FadeScreen.MicrowavingSequence` _returnvalue) 0.0 1 "Forward" 1.0 false)
      (`/Game/FirstPerson/Blueprints/BP_FirstPersonCharacter.Disable Movement and Look` (`self.Player Pref`)))
    (:`then_1`
      (`SceneComponent.SetVisibility` (`self.food`) true false)
      (`KismetSystemLibrary.Delay` (`self.DelayBeforeRotating`))
      (set `self.IsRotating` true)
      (`SceneComponent.SetVisibility` (`self.Light`) true false)
      (`KismetSystemLibrary.Delay` (`self.DelayCookingDuration`))
      (set `self.IsRotating` false)
      (`SceneComponent.SetVisibility` (`self.Light`) false false)
      (`KismetSystemLibrary.Delay` (`self.DelayAfterCooking`))
      (`SceneComponent.SetVisibility` (`self.food`) false false)
      (bind _returnvalue_2 (`|SpawnActorFromClass` "/Game/Blueprints/EventItems/BP_HeatedFood.BP_HeatedFood_C" (`SceneComponent.K2_GetComponentToWorld` _hold_position) "Undefined" "MultiplyWithRoot" null null))
      (`PrimitiveComponent.SetCollisionEnabled` (`/Game/Blueprints/EventItems/BP_HeatedFood.Pickupable` _returnvalue_2) "QueryAndPhysics")
      (`self.K2_AttachToComponent` _returnvalue_2 _hold_position "None" "SnapToTarget" "SnapToTarget" "SnapToTarget" true)
      (`/Game/FirstPerson/Blueprints/BP_FirstPersonCharacter.Enable Look and Movement` _player_pref)
      (set `/Game/FirstPerson/Blueprints/BP_FirstPersonCharacter.IsInteractionBlocked` true _player_pref)
      (`self.EnableDiningTable` _returnvalue_2))
    (:`then_2`
      (set `/Game/FirstPerson/Blueprints/BP_FirstPersonCharacter.IsHoldingItem` false _player_pref_2)
      (set `/Game/FirstPerson/Blueprints/BP_FirstPersonCharacter.MeshPickupable` null _player_pref_2)
      (`StaticMeshComponent.SetStaticMesh` (`/Game/FirstPerson/Blueprints/BP_FirstPersonCharacter.Pickupable Position` _player_pref_2) null))))

(event `self.ReceiveTick`
  (params (DeltaSeconds :type "Float (single-precision)"))
  (if (`self.IsRotating`)
    (`SceneComponent.K2_AddLocalRotation` (`self.food`) (`KismetMathLibrary.MakeRotator` 0.0 0.0 (* DeltaSeconds (`self.Rotation`))) false false)))

(fn `UserConstructionScript`)