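; Event item door for Mikey's room that swings partly open when that room's event fires.
; On BeginPlay it binds to the Mikey room event dispatcher on its Enabler reference, if that reference is valid.
; When triggered, a timeline interpolates the door's relative yaw from closed to a half-open 45 degrees.
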(event `self.ReceiveBeginPlay`
  (bind _enabler (`self.Enabler`))
  (`parent.ReceiveBeginPlay`)
  (`/Engine/EditorBlueprintResources/StandardMacros.IsValid` _enabler
    (:`Is Valid`
      (add `/Game/Blueprints/Levels/Trigger_BasketballBouncingFromMikey.TriggerMikeyRoomEvent` _enabler (delegate `Open Door Half`)))))

(event `Open Door Half`
  (bind (_direction _door_alpha) (`Timeline|Timeline`)
    (:`Update`
      (`SceneComponent.K2_SetRelativeRotation` (`self.Door`) (`KismetMathLibrary.MakeRotator` 0.0 0.0 (`KismetMathLibrary.Lerp` 0.0 45.0 _door_alpha)) false false))))

(fn `UserConstructionScript`
  (`parent.UserConstructionScript`))