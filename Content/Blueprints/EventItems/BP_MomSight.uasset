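; BP_MomSight is an event item actor whose skeletal mesh fades out and is removed when Execute fires.
; Execute swaps each material slot to a dynamic instance of M_FadeOut, restarting a timeline from inside that loop.
; The timeline drives the fadeOut scalar parameter across the mesh's materials and destroys the actor when it finishes.
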(event `/Game/Blueprints/Interface/BPI_Executable.Execute`
  (for _index (range (+ (`PrimitiveComponent.GetNumMaterials` (`self.SkeletalMesh`)) 1))
    (`PrimitiveComponent.CreateDynamicMaterialInstance` (`self.SkeletalMesh`) _index "/Game/Materials/M_FadeOut.M_FadeOut" "None")
    (bind (_direction _newtrack_0) (`Timeline|Timeline` :!via `PlayFromStart`)
      (:`Update`
        (`MeshComponent.SetScalarParameterValueOnMaterials` (`self.SkeletalMesh`) "fadeOut" _newtrack_0))
      (:`Finished`
        (`self.K2_DestroyActor`)))))

(fn `UserConstructionScript`
  (`parent.UserConstructionScript`))