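; Event item that plays a mysterious basketball dribbling sound in the hall in front of a room.
; On BeginPlay it binds to the laptop enabler's basketball trigger and, only if that enabler is valid, to a sound stopper's jumpscare event.
; The trigger spawns an attenuated proximity sound at the item's location and stores it, so the jumpscare event can stop it.
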(event `self.ReceiveBeginPlay`
  (bind _soundstopper (`self.SoundStopper`))
  (bind _laptop_enabler (`self.Laptop Enabler`))
  (`/Engine/EditorBlueprintResources/StandardMacros.IsValid` _laptop_enabler
    (:`Is Valid`
      (add `/Game/Blueprints/EventItems/BP_Laptop.Trigger Mysterious Basket Ball at Hall` _laptop_enabler (delegate `Execute Sound`))
      (`/Engine/EditorBlueprintResources/StandardMacros.IsValid` _soundstopper
        (:`Is Valid`
          (add `/Game/Blueprints/EventItems/BP_RyansDoor.SetJumpscare` _soundstopper (delegate `Stop Sound`)))))))

(event `Execute Sound`
  (bind _returnvalue (`GameplayStatics.SpawnSoundAtLocation` "/Game/Sounds/BasketballBounce/sfx_basketball_dribbling.sfx_basketball_dribbling" (`SceneComponent.GetSocketLocation` (`self.Property Item`) "None") (struct) 1.0 1.0 0.0 "/Game/Sounds/BasketballBounce/SA_ProximitySound.SA_ProximitySound" null))
  (set `self.SoundObject` _returnvalue))

(event `Stop Sound`
  (bind _soundobject (`self.SoundObject`)
    (:`then`
      (`AudioComponent.Stop` _soundobject))
    (:`else`)))

(fn `UserConstructionScript`
  (`parent.UserConstructionScript`))