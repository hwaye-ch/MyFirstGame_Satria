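; BP_NPC is a talkable NPC that starts a dialogue when the first-person character talks to it.
; TalkwithObject registers the NPC as trigger on its BPDialogueComponent, shows the component's configured message, then hands the component, table, next code, widget and end flag to the player.
; FinishDialogue flags the player's dialogue text as complete and prints a debug string.
; InteractObject and ShowDialogue are empty stubs.
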(event `/Game/Blueprints/Interface/BPI_Talk.TalkWithObject`
  (params (TargetActor :type "Actor Object Reference"))
  (bind _bp_dialoguecomponent (`self.BP_DialogueComponent`))
  (bind _dialoguetable (`/Game/Blueprints/Components/BP_DialogueComponent.DialogueTable` _bp_dialoguecomponent))
  (bind _asbp_first_person_character (cast `/Game/FirstPerson/Blueprints/BP_FirstPersonCharacter` TargetActor))
  (bind _output_get (set `self.PlayerPref` _asbp_first_person_character))
  (set `/Game/FirstPerson/Blueprints/BP_FirstPersonCharacter.IsTriggeringDialogue` true _output_get)
  (set `/Game/FirstPerson/Blueprints/BP_FirstPersonCharacter.IsDialogueTextComplete` false (`self.PlayerPref`))
  (set `/Game/Blueprints/Components/BP_DialogueComponent.ActorTrigger` self _bp_dialoguecomponent)
  (bind (_isendofdialogue _nextdialoguecode _dialoguewidget) (message `/Game/Blueprints/Interface/BPI_Dialogue.ShowDialogue` _bp_dialoguecomponent (`/Game/Blueprints/Components/BP_DialogueComponent.DialogueCode` _bp_dialoguecomponent) _dialoguetable))
  (set `/Game/FirstPerson/Blueprints/BP_FirstPersonCharacter.IsDialogueEnded` _isendofdialogue (`self.PlayerPref`))
  (set `/Game/FirstPerson/Blueprints/BP_FirstPersonCharacter.DialogueActorComponent` _bp_dialoguecomponent (`self.PlayerPref`))
  (set `/Game/FirstPerson/Blueprints/BP_FirstPersonCharacter.DialogueCode` _nextdialoguecode (`self.PlayerPref`))
  (set `/Game/FirstPerson/Blueprints/BP_FirstPersonCharacter.DialogueTable` _dialoguetable (`self.PlayerPref`))
  (set `/Game/FirstPerson/Blueprints/BP_FirstPersonCharacter.DialogueWidget` _dialoguewidget (`self.PlayerPref`)))

(event `/Game/Blueprints/Interface/BPI_Dialogue.FinishDialogue`
  (`KismetSystemLibrary.PrintString` "Aku sudah selesai btw")
  (set `/Game/FirstPerson/Blueprints/BP_FirstPersonCharacter.IsDialogueTextComplete` true (`self.PlayerPref`)))

(fn `InteractObject`
  (params (PlayerPref :type "/Game/FirstPerson/Blueprints/BP_FirstPersonCharacter Object Reference"))
  (returns (MeshBentukan :type "StaticMesh Object Reference"))
  (return null))

(fn `ShowDialogue`
  (params (DialogueCode :type Name) (DialogueTable :type "DataTable Object Reference"))
  (returns (isEndOfDialogue :type Boolean) (NextDialogueCode :type Name) (DialogueWidget :type "/Game/Blueprints/Widgets/WBP_Dialogue Object Reference"))
  (return false "None" null))

(fn `UserConstructionScript`)