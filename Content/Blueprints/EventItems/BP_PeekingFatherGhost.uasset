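; BP_PeekingFatherGhost is a one-shot scare: a father ghost that peeks out, then slips away when looked at.
; It starts hidden until FatherEnabler's StartFatherPeeping event reveals it with a breathing sound.
; Tick then checks the player's HitActor for the "Father" tag, firing once to swap breathing for a laugh.
; The MoveFather timeline slides the actor a short distance along world Y, then destroys it.
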(event `self.ReceiveBeginPlay`
  (bind _returnvalue (`self.K2_GetActorLocation` self))
  (`parent.ReceiveBeginPlay`)
  (`SceneComponent.SetVisibility` (`self.Father`) false false)
  (bind _fatherenabler (`self.FatherEnabler`)
    (:`then`
      (add `/Game/Blueprints/EventItems/BP_Laptop.Start Father Peeping` _fatherenabler (delegate `Show father`))
      (set `self.GhostStartLocation` _returnvalue)
      (set `self.GhostEndLocation` (`KismetMathLibrary.MakeVector` (.x _returnvalue) (- (.y _returnvalue) 50.0) (.z _returnvalue))))
    (:`else`)))

(event `Show father`
  (`SceneComponent.SetVisibility` (`self.Father`) true false)
  (set `self.IsReady` true)
  (bind _returnvalue (`GameplayStatics.SpawnSoundAtLocation` "/Game/Sounds/sfx_father-breath.sfx_father-breath" (`self.K2_GetActorLocation` self) (struct) 0.5 1.0 0.0 "/Game/Sounds/BasketballBounce/SA_ProximitySound.SA_ProximitySound" null))
  (set `self.fatherbreathsound` _returnvalue))

(event `self.ReceiveTick`
  (params (DeltaSeconds :type "Float (single-precision)"))
  (bind _hit_actor (`/Game/FirstPerson/Blueprints/BP_FirstPersonCharacter.Hit Actor` (`self.Player Pref`)))
  (if (`self.IsReady`)
    (`/Engine/EditorBlueprintResources/StandardMacros.IsValid` _hit_actor
      (:`Is Valid`
        (if (`self.ActorHasTag` _hit_actor "Father")
          (`/Engine/EditorBlueprintResources/StandardMacros.DoOnce` false
            (:`Completed`
              (`KismetSystemLibrary.PrintString` "Papa is looked at" true true (struct :`R` 0.54207 :`G` 1.0 :`B` 0.554339 :`A` 1.0))
              (`GameplayStatics.SpawnSoundAtLocation` "/Game/Sounds/sfx_father-laugh.sfx_father-laugh" (`self.K2_GetActorLocation` self) (struct) 1.0 1.0 0.0 "/Game/Sounds/BasketballBounce/SA_ProximitySound.SA_ProximitySound" null)
              (bind _fatherbreathsound (`self.fatherbreathsound`)
                (:`then`
                  (`AudioComponent.Stop` _fatherbreathsound)
                  (bind (_direction _alpha) (`Timeline|Move Father` :!via `PlayFromStart` :!label _label)
                    (:`Update`
                      (`self.K2_SetActorLocation` (`KismetMathLibrary.VLerp` (`self.GhostStartLocation`) (`self.GhostEndLocation`) _alpha)))
                    (:`Finished`
                      (`self.K2_DestroyActor`))))
                (:`else`
                  (goto _label :!via `PlayFromStart`))))))))))

(fn `UserConstructionScript`
  (`parent.UserConstructionScript`))