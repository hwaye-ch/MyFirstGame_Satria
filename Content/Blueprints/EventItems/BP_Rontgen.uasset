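; BP_Rontgen is an inspectable event item that plays a Chapter 7 dialogue the first time it is inspected.
; InspectObject passes through a DoOnce, binds the dialogue-ended delegate, then constructs and shows the dialogue via BPDialogueComponent with movement and look blocked.
; When the dialogue ends, the bound event calls DisableMovementAndLook on the player, and nothing in this Blueprint re-enables control.
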(event `/Game/Blueprints/Interface/BPI_Inspect.InspectObject`
  (bind _bp_dialoguecomponent (`self.BP_DialogueComponent`))
  (`/Engine/EditorBlueprintResources/StandardMacros.DoOnce` false
    (:`Completed`
      (add `/Game/Blueprints/Components/BP_DialogueComponent.OnDialogueEnded` _bp_dialoguecomponent (delegate `OnDialogueEnded_Event`))
      (bind _dialoguecomponent (`/Game/Blueprints/Components/BP_DialogueComponent.Construct Dialogue` _bp_dialoguecomponent "ch7_rontgen_1" "/Game/Dialogue/Chapter7_Dialogue.Chapter7_Dialogue" true true))
      (`/Game/Blueprints/Interface/BPI_Dialogue.ShowDialogue` _dialoguecomponent (`self.PlayerRef`) self))))

(event `OnDialogueEnded_Event`
  (`/Game/FirstPerson/Blueprints/BP_FirstPersonCharacter.Disable Movement and Look` (`self.PlayerRef`)))

(fn `UserConstructionScript`
  (`parent.UserConstructionScript`))