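; Ryan's door, an event item that lets the player toggle peeking through a dedicated door camera.
; StartPeeking flips IsPeeking and swaps active cameras, blending the view to the door and disabling player movement and look.
; Exiting switches straight back to the player's first-person camera and restores control.
; A DoOnce triggers CallSetJumpscare on the first peek only.
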(event `self.Start Peeking`
  (if (`self.IsPeeking`)
    (`KismetSystemLibrary.PrintString` "Exit Peeking")
    (set `self.IsPeeking` false)
    (`ActorComponent.SetActive` (`/Game/FirstPerson/Blueprints/BP_FirstPersonCharacter.FirstPersonCamera` (`self.Player Pref`)) true false)
    (`ActorComponent.SetActive` (`self.Camera`) false false)
    (`PlayerController.SetViewTargetWithBlend` (`GameplayStatics.GetPlayerController` 0) (`self.Player Pref`) 0.0 "VTBlend_Linear" 0.0 false)
    (`/Game/FirstPerson/Blueprints/BP_FirstPersonCharacter.Enable Look and Movement` (`self.Player Pref`))
    (else
      (`KismetSystemLibrary.PrintString` "Start Peeking")
      (set `self.IsPeeking` true)
      (`ActorComponent.SetActive` (`/Game/FirstPerson/Blueprints/BP_FirstPersonCharacter.FirstPersonCamera` (`self.Player Pref`)) false false)
      (`ActorComponent.SetActive` (`self.Camera`) true false)
      (`PlayerController.SetViewTargetWithBlend` (`GameplayStatics.GetPlayerController` 0) self 0.3 "VTBlend_Linear" 0.0 false)
      (`/Game/FirstPerson/Blueprints/BP_FirstPersonCharacter.Disable Movement and Look` (`self.Player Pref`))
      (`/Engine/EditorBlueprintResources/StandardMacros.DoOnce` false
        (:`Completed`
          (`self.SetJumpscare`))))))

(fn `UserConstructionScript`
  (`parent.UserConstructionScript`))