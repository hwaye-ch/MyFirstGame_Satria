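; BP_RyansRoomsDoor is a door Blueprint with events to open and close it, including an event-driven open.
; OpenDoorbyEvent sets the EventDoorInteraction flag, plays a 2D opening sound, and runs the SlowOpen timeline to lerp the door's relative yaw into a swing.
; ClosetheDoor instantly resets the door's world rotation to zero and clears IsDoorOpened.
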(event `Open Door by Event`
  (set `self.EventDoorInteraction` true)
  (`GameplayStatics.PlaySound2D` "/Game/Sounds/sfx_door_opened.sfx_door_opened" 1.0 1.0 0.0 null null)
  (bind (_direction _newtrack_0) (`Timeline|Slow Open`)
    (:`Update`
      (`SceneComponent.K2_SetRelativeRotation` (`self.Door`) (`KismetMathLibrary.MakeRotator` 0.0 0.0 (`KismetMathLibrary.Lerp` 0.0 -60.0 _newtrack_0)) false false))))

(event `Close the Door`
  (`SceneComponent.K2_SetWorldRotation` :`self` (`self.Door`))
  (set `self.IsDoorOpened` false))

(fn `UserConstructionScript`
  (`parent.UserConstructionScript`))