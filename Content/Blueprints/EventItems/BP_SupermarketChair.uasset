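; BP_SupermarketChair is an event item chair whose CombineObject event plays an eating moment and moves the player to another map.
; The event starts a long screen fade-out through BPFadeScreenComponent and, in parallel, plays a 2D eating sound after a short delay.
; When the fade reports its exact finish, a bound handler asks the game instance to teleport to a fixed map enum entry.
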(event `/Game/Blueprints/Interface/BPI_Combine.CombineObject`
  (bind _bp_fadescreencomponent (`self.BP_FadeScreenComponent`))
  (`|ExecutionSequence`
    (:`then_0`
      (`/Game/Blueprints/Components/BP_FadeScreenComponent.Fade Out` _bp_fadescreencomponent 17.0 (`self.PlayerRef`))
      (add `/Game/Blueprints/Components/BP_FadeScreenComponent.OnExactFinish` _bp_fadescreencomponent (delegate `OnExactFinish_Event`)))
    (:`then_1`
      (`KismetSystemLibrary.Delay` 3.0)
      (`GameplayStatics.SpawnSound2D` "/Game/Sounds/sfx_eating.sfx_eating" 1.0 1.0 0.0 null))))

(event `OnExactFinish_Event`
  (`/Game/System/HwyGameInstance.Teleport to Map` (`self.Game Instance Ref`) "NewEnumerator0"))

(fn `UserConstructionScript`
  (`parent.UserConstructionScript`))