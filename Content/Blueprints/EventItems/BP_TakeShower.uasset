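; BP_TakeShower is an event item that plays a shower sequence when the player interacts with it.
; InteractItem passes through a DoOnce, so the sequence triggers only on the first interaction.
; It creates a WBP_FadeScreen widget, adds it to the viewport, plays its ShowerSequence animation and prints a debug string.
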(event `/Game/Blueprints/Interface/BPI_Actionable.InteractItem`
  (`/Engine/EditorBlueprintResources/StandardMacros.DoOnce` false
    (:`Completed`
      (bind _returnvalue (`|CreateWidget` "/Game/Blueprints/Widgets/WBP_FadeScreen.WBP_FadeScreen_C"))
      (`UserWidget.AddToViewport` _returnvalue 0)
      (`UserWidget.PlayAnimation` _returnvalue (`/Game/Blueprints/Widgets/WBP_FadeScreen.ShowerSequence` _returnvalue) 0.0 1 "Forward" 1.0 false)
      (`KismetSystemLibrary.PrintString` "Jebur mandi heuheu"))))

(fn `UserConstructionScript`
  (`parent.UserConstructionScript`))