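; BP_Television is a TV prop that switches on at BeginPlay to show a basketball match and can be turned on or off by events.
; Turning on shows the screen and light, plays media and proximity-attenuated audio, and flickers the light through a timeline.
; Turning off hides both and stops the match audio and timeline.
; PlayCrazyDisturbance recursively toggles the TV with shrinking delays, using ShouldStop to end switched on.
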(event `self.ReceiveBeginPlay`
  (bind _mediaplayer (`self.MediaPlayer`))
  (`parent.ReceiveBeginPlay`)
  (`SceneComponent.SetVisibility` (`self.Light`) false false)
  (`SceneComponent.SetVisibility` (`self.Cube`) false false)
  (`SceneComponent.SetVisibility` (`self.Light`) true false :!label _label)
  (`SceneComponent.SetVisibility` (`self.Cube`) true false)
  (`GameplayStatics.SpawnSoundAtLocation` "/Game/Sounds/sfx_tv-turn.sfx_tv-turn" (`SceneComponent.K2_GetComponentLocation` (`self.Property Item`)) (struct) 1.0 0.9 0.0 "/Game/Sounds/BasketballBounce/SA_ProximitySound.SA_ProximitySound" null)
  (`MediaPlayer.OpenSource` _mediaplayer "/Game/Media/nba.nba")
  (`MediaPlayer.Play` _mediaplayer)
  (bind _returnvalue (`GameplayStatics.SpawnSoundAtLocation` "/Game/Sounds/sfx_basketball-match.sfx_basketball-match" (`SceneComponent.K2_GetComponentLocation` (`self.Property Item`)) (struct) 0.3 1.0 0.0 "/Game/Sounds/BasketballBounce/SA_ProximitySound.SA_ProximitySound" null false))
  (set `self.NbaSound` _returnvalue)
  (bind (_direction _light_intensity) (`Timeline|FlashingLightTime` :!label _label_2)
    (:`Update`
      (`LightComponent.SetIntensity` (`self.Light`) (* _light_intensity 200.0)))))

(event `Turn On TV`
  (goto _label))

(event `Turn Off TV`
  (`GameplayStatics.SpawnSoundAtLocation` "/Game/Sounds/sfx_tv-turn.sfx_tv-turn" (`SceneComponent.K2_GetComponentLocation` (`self.Property Item`)) (struct) 1.0 1.0 0.0 "/Game/Sounds/BasketballBounce/SA_ProximitySound.SA_ProximitySound" null)
  (`SceneComponent.SetVisibility` (`self.Light`) false false)
  (`SceneComponent.SetVisibility` (`self.Cube`) false false)
  (`AudioComponent.Stop` (`self.NbaSound`))
  (goto _label_2 :!via `Stop`))

(event `Play Crazy Disturbance`
  (`KismetSystemLibrary.Delay` (`self.Duration`))
  (`self.Turn On TV`)
  (`KismetSystemLibrary.Delay` (`self.Duration`))
  (`self.Turn Off TV`)
  (`self.ShouldStop?`
    (:`then`
      (`self.Turn On TV`))
    (:`else`
      (`self.Play Crazy Disturbance`)
      (if (>= (`self.Duration`) 0.3)
        (set `self.Duration` (- (`self.Duration`) 0.1))
        (else
          (`KismetSystemLibrary.Delay` 5.0)
          (set `self.ShouldStop?` true))))))

(fn `UserConstructionScript`
  (`parent.UserConstructionScript`))