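; BP_Trash is a trash pickup event item, built on a parent class that supplies its base behavior.
; On BeginPlay its Pickupable component stays visible but has collision disabled.
; EnableSampah keeps it visible and turns on query and physics collision.
; OnPickupObject only prints debug text and the activator item code from BPActivatorComponent.
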(event `self.ReceiveBeginPlay`
  (bind _pickupable (`self.Pickupable`))
  (`parent.ReceiveBeginPlay`)
  (`SceneComponent.SetVisibility` _pickupable true false)
  (`PrimitiveComponent.SetCollisionEnabled` _pickupable "NoCollision"))

(event `/Game/Blueprints/Interface/BPI_Pickup.OnPickupObject`
  (`KismetSystemLibrary.PrintString` "BP_Trash - Pickup Trash")
  (`KismetSystemLibrary.PrintString` (`|GetEnumeratorNameAsString` (`/Game/Blueprints/Components/BP_ActivatorComponent.ActivatorItemCode` (`self.BP_ActivatorComponent`)))))

(event `Enable Sampah`
  (bind _pickupable (`self.Pickupable`))
  (`SceneComponent.SetVisibility` _pickupable true false)
  (`PrimitiveComponent.SetCollisionEnabled` _pickupable "QueryAndPhysics"))

(fn `UserConstructionScript`
  (`parent.UserConstructionScript`))