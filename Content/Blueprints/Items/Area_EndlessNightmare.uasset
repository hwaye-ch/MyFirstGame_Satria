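; Area_EndlessNightmare is a self-replicating level segment that builds an endless nightmare path as the player advances.
; Player-triggered, one-shot overlaps spawn the next segment at an Arrow, raise that segment's wall, or destroy the current one.
; BP_ChapterNightmare tracks the spawn count and populates new segments, with specific counts raising a wall or removing Mother.
; The branch that spawns the crawling Mother is hard-wired off.
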(event `self.ReceiveBeginPlay`
  (bind _returnvalue (`GameplayStatics.GetActorOfClass` "/Game/Blueprints/Chapters/BP_ChapterNightmare.BP_ChapterNightmare_C"))
  (set `self.ChapterManager` _returnvalue))

(event `Initialize Nightmare`
  (bind _new_block (`self.SpawnBlock`))
  (bind _wall (`/Game/Blueprints/Items/Area_EndlessNightmare.Wall` _new_block))
  (`SceneComponent.SetVisibility` _wall false true)
  (`PrimitiveComponent.SetCollisionEnabled` _wall "NoCollision"))

(event `self.Spawn.OnComponentBeginOverlap`
  (params (OverlappedComponent :type "PrimitiveComponent Object Reference") (OtherActor :type "Actor Object Reference") (OtherComp :type "PrimitiveComponent Object Reference") (OtherBodyIndex :type Integer) (bFromSweep :type Boolean) (SweepResult :type "HitResult Structure (by ref)"))
  (bind _wall (`/Game/Blueprints/Items/Area_EndlessNightmare.Wall` (`self.New Spawned Area`)))
  (bind _wall_2 (`/Game/Blueprints/Items/Area_EndlessNightmare.Wall` (`self.New Spawned Area`)))
  (cast `/Game/FirstPerson/Blueprints/BP_FirstPersonCharacter` OtherActor)
  (`/Engine/EditorBlueprintResources/StandardMacros.DoOnce` false
    (:`Completed`
      (bind _new_block (`self.SpawnBlock`))
      (bind _output_get (set `self.New Spawned Area` _new_block))
      (`/Game/Blueprints/Chapters/BP_ChapterNightmare.Spawn Stuff` (`self.ChapterManager`) _output_get)
      (`KismetSystemLibrary.PrintString` "Spawn")
      (bind _result (`/Engine/EditorBlueprintResources/StandardMacros.IncrementInt` (`/Game/Blueprints/Chapters/BP_ChapterNightmare.Spawn Count` (`self.ChapterManager`)))
        (:`  `
          (`KismetSystemLibrary.PrintString` (`KismetStringLibrary.Concat_StrStr` "Spawn Count: " (`KismetStringLibrary.Conv_IntToString` _result)))
          (`SceneComponent.SetVisibility` _wall false false)
          (`PrimitiveComponent.SetCollisionEnabled` _wall "NoCollision")
          (if false
            (`self.Spawn Mother`)
            (elif (== (`/Game/Blueprints/Chapters/BP_ChapterNightmare.Spawn Count` (`self.ChapterManager`)) 24)
              (bind _mother (`self.Mother`)
                (:`then`
                  (`self.K2_DestroyActor` _mother))
                (:`else`))
              (elif (== (`/Game/Blueprints/Chapters/BP_ChapterNightmare.Spawn Count` (`self.ChapterManager`)) 10)
                (`SceneComponent.SetVisibility` _wall_2 true true)
                (`PrimitiveComponent.SetCollisionEnabled` _wall_2 "QueryAndPhysics")))))))))

(event `self.Destroy.OnComponentBeginOverlap`
  (params (OverlappedComponent :type "PrimitiveComponent Object Reference") (OtherActor :type "Actor Object Reference") (OtherComp :type "PrimitiveComponent Object Reference") (OtherBodyIndex :type Integer) (bFromSweep :type Boolean) (SweepResult :type "HitResult Structure (by ref)"))
  (cast `/Game/FirstPerson/Blueprints/BP_FirstPersonCharacter` OtherActor)
  (`/Engine/EditorBlueprintResources/StandardMacros.DoOnce` false
    (:`Completed`
      (`self.K2_DestroyActor`)
      (`KismetSystemLibrary.PrintString` "Destroy"))))

(event `self.Wall Builder.OnComponentBeginOverlap`
  (params (OverlappedComponent :type "PrimitiveComponent Object Reference") (OtherActor :type "Actor Object Reference") (OtherComp :type "PrimitiveComponent Object Reference") (OtherBodyIndex :type Integer) (bFromSweep :type Boolean) (SweepResult :type "HitResult Structure (by ref)"))
  (cast `/Game/FirstPerson/Blueprints/BP_FirstPersonCharacter` OtherActor)
  (`/Engine/EditorBlueprintResources/StandardMacros.DoOnce` false
    (:`Completed`
      (bind _new_spawned_area (`self.New Spawned Area`)
        (:`then`
          (bind _wall (`/Game/Blueprints/Items/Area_EndlessNightmare.Wall` _new_spawned_area))
          (`SceneComponent.SetVisibility` _wall true false)
          (`PrimitiveComponent.SetCollisionEnabled` _wall "QueryAndPhysics")
          (`KismetSystemLibrary.PrintString` "Wall Built"))
        (:`else`)))))

(event `Spawn Mother`
  (bind _returnvalue (`|SpawnActorFromClass` "/Game/Blueprints/Characters/BP_MomCrawling.BP_MomCrawling_C" (`SceneComponent.K2_GetComponentToWorld` (`self.SpawnAreaMother`)) "Undefined" "MultiplyWithRoot" null null))
  (`PawnSensingComponent.SetSensingUpdatesEnabled` (`/Game/Blueprints/Characters/BP_MomCrawling.PawnSensing` _returnvalue) true)
  (set `self.Mother` _returnvalue))

(fn `SpawnBlock`
  (returns (`New Block` :type "/Game/Blueprints/Items/Area_EndlessNightmare Object Reference"))
  (bind _returnvalue (`|SpawnActorFromClass` "Area_EndlessNightmare_C" (`SceneComponent.K2_GetComponentToWorld` (`self.Arrow`)) "Undefined" "MultiplyWithRoot" null (`GameplayStatics.GetPlayerCharacter` 0)))
  (return _returnvalue))

(fn `UserConstructionScript`)