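; BP_GroundSpawner is a road segment that extends an endless road as the first-person character moves along it.
; Entering the Spawner trigger spawns a new road actor once, taking X from the Platform's bounds size transformed to world space and Y and Z from the Arrow.
; Entering the Destroyer trigger destroys this segment.
; Both triggers print debug messages, and the PlayEndlessRoad event is an empty stub.
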(event `self.ReceiveBeginPlay`
  (`parent.ReceiveBeginPlay`))

(event `Play Endless Road`)

(event `self.Spawner.OnComponentBeginOverlap`
  (params (OverlappedComponent :type "PrimitiveComponent Object Reference") (OtherActor :type "Actor Object Reference") (OtherComp :type "PrimitiveComponent Object Reference") (OtherBodyIndex :type Integer) (bFromSweep :type Boolean) (SweepResult :type "HitResult Structure (by ref)"))
  (bind (_min _max) (`StaticMeshComponent.GetLocalBounds` (`self.Platform`)))
  (bind (_returnvalue_location _returnvalue_rotation) (`KismetMathLibrary.BreakTransform` (`SceneComponent.K2_GetComponentToWorld` (`self.Platform`))))
  (bind (_returnvalue_x _returnvalue_y _returnvalue_z) (`KismetMathLibrary.BreakVector` (`SceneComponent.K2_GetComponentLocation` (`self.Arrow`))))
  (cast `/Game/FirstPerson/Blueprints/BP_FirstPersonCharacter` OtherActor)
  (`/Engine/EditorBlueprintResources/StandardMacros.DoOnce` false
    (:`Completed`
      (`|SpawnActorFromClass` "BP_GroundSpawner_C" (`KismetMathLibrary.MakeTransform` (`KismetMathLibrary.MakeVector` (.x (`KismetMathLibrary.TransformLocation` (`SceneComponent.K2_GetComponentToWorld` (`self.Platform`)) (- _max _min))) _returnvalue_y _returnvalue_z) _returnvalue_rotation) "Undefined" "MultiplyWithRoot" null null)
      (`KismetSystemLibrary.PrintString` "Spawn New Road"))))

(event `self.Destroyer.OnComponentBeginOverlap`
  (params (OverlappedComponent :type "PrimitiveComponent Object Reference") (OtherActor :type "Actor Object Reference") (OtherComp :type "PrimitiveComponent Object Reference") (OtherBodyIndex :type Integer) (bFromSweep :type Boolean) (SweepResult :type "HitResult Structure (by ref)"))
  (cast `/Game/FirstPerson/Blueprints/BP_FirstPersonCharacter` OtherActor)
  (`self.K2_DestroyActor`)
  (`KismetSystemLibrary.PrintString` "Destroy Road"))

(fn `UserConstructionScript`
  (`parent.UserConstructionScript`))