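; BP_InspectableItem is a world item that the player can bring up for close inspection and rotate with the mouse.
; A once-only Inspect event freezes player movement and look, shows the cursor, and plays a timeline lerping the item to the first-person character's InspectableItem transform.
; While inspecting, Tick and mouse axes feed local rotation.
; Q resets the gate, restores controls and reverses the timeline to return the item.
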(event `self.ReceiveTick`
  (params (DeltaSeconds :type "Float (single-precision)"))
  (if (`self.CanInspect?`) :!label _label
    (`SceneComponent.K2_AddLocalRotation` (`self.InspectableItem`) (`KismetMathLibrary.MakeRotator` (* (stale `InputAxisKey|MouseX` AxisValue) 0.4) (* (stale `InputAxisKey|MouseY` AxisValue) 0.4)) false false)))

(event `self.ReceiveBeginPlay`
  (bind _inspectableitem (`self.InspectableItem`))
  (bind _output_get (set `self.Original Location` (`SceneComponent.K2_GetComponentLocation` _inspectableitem)))
  (bind _output_get_2 (set `self.Original Rotation` (`SceneComponent.K2_GetComponentRotation` _inspectableitem)))
  (`self.EnableInput` (`GameplayStatics.GetPlayerController` 0)))

(event `InputAxisKey|MouseX`
  (params (AxisValue :type "Float (single-precision)"))
  (goto _label))

(event `InputAxisKey|MouseY`
  (params (AxisValue :type "Float (single-precision)"))
  (goto _label))

(event `/Game/Blueprints/Interface/BPI_Inspect.Inspect`
  (`/Engine/EditorBlueprintResources/StandardMacros.DoOnce` false :!label _label_2
    (:`Completed`
      (set `PlayerController.bShowMouseCursor` true (`GameplayStatics.GetPlayerController` 0))
      (set `self.CanInspect?` true)
      (bind _asbp_first_person_character (cast `/Game/FirstPerson/Blueprints/BP_FirstPersonCharacter` (`GameplayStatics.GetPlayerCharacter` 0)))
      (`CharacterMovementComponent.DisableMovement` (`Character.CharacterMovement` (`GameplayStatics.GetPlayerCharacter` 0)))
      (`Controller.SetIgnoreLookInput` (`GameplayStatics.GetPlayerController` 0) true)
      (bind (_direction __) (`Timeline|TL_Inspect` :!label _label_3)
        (:`Update`
          (bind (_returnvalue_location _returnvalue_rotation) (`KismetMathLibrary.BreakTransform` (`SceneComponent.K2_GetComponentToWorld` (`/Game/FirstPerson/Blueprints/BP_FirstPersonCharacter.Inspectable Item` _asbp_first_person_character))))
          (`SceneComponent.K2_SetWorldTransform` (`self.InspectableItem`) (`KismetMathLibrary.MakeTransform` (`KismetMathLibrary.VLerp` (stale `self.ReceiveBeginPlay` _output_get) _returnvalue_location __) (`KismetMathLibrary.RLerp` (stale `self.ReceiveBeginPlay` _output_get_2) _returnvalue_rotation __)) false false))))))

(event `Key|Q`
  (params (Key :type "Key Structure"))
  (bind _returnvalue (`GameplayStatics.GetPlayerController` 0))
  (:`Pressed`
    (`|ExecutionSequence`
      (:`then_0`
        (goto _label_2 :!via `Reset`))
      (:`then_1`
        (set `self.CanInspect?` false)
        (`CharacterMovementComponent.SetMovementMode` (`Character.CharacterMovement` (`GameplayStatics.GetPlayerCharacter` 0)) "MOVE_Walking" 0)
        (set `PlayerController.bShowMouseCursor` false _returnvalue)
        (`Controller.ResetIgnoreLookInput` _returnvalue)
        (`WidgetBlueprintLibrary.SetInputMode_GameOnly` _returnvalue)
        (goto _label_3 :!via `Reverse`)))))

(fn `UserConstructionScript`)