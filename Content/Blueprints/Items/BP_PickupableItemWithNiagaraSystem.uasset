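; Pickupable item Blueprint with a Niagara smoke effect that the player can pick up, hold and throw.
; Pickup copies the mesh, scale, smoke effect and activator item code to the player, flags it as holding, then destroys the actor after a brief delay.
; Throw rebuilds the mesh and scale from the player's stored values, enables physics, applies a mass-independent forward impulse using the player's throw force, and clears the held item.
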(event `Destroy Item`
  (`KismetSystemLibrary.Delay` 0.01)
  (`self.K2_DestroyActor`))

(fn `PickupObject`
  (params (PlayerPref :type "/Game/FirstPerson/Blueprints/BP_FirstPersonCharacter Object Reference"))
  (returns (ThrowableActor :type "/Game/Blueprints/Items/BP_PickupableItem Object Reference"))
  (bind _pickupable (`self.Pickupable`))
  (bind _pickupable_item (`/Game/FirstPerson/Blueprints/BP_FirstPersonCharacter.Pickupable Item` PlayerPref))
  (bind _returnvalue (`SceneComponent.K2_GetComponentScale` _pickupable))
  (bind _staticmesh (`StaticMeshComponent.StaticMesh` _pickupable))
  (set `/Game/FirstPerson/Blueprints/BP_FirstPersonCharacter.MeshPickupable` _staticmesh PlayerPref)
  (set `/Game/FirstPerson/Blueprints/BP_FirstPersonCharacter.PickupableVector` _returnvalue PlayerPref)
  (set `/Game/FirstPerson/Blueprints/BP_FirstPersonCharacter.SmokeEffect` (`self.NS_Smoke`) PlayerPref)
  (`StaticMeshComponent.SetStaticMesh` _pickupable_item _staticmesh)
  (`SceneComponent.SetWorldScale3D` _pickupable_item _returnvalue)
  (set `/Game/FirstPerson/Blueprints/BP_FirstPersonCharacter.IsHoldingItem` true PlayerPref)
  (set `/Game/FirstPerson/Blueprints/BP_FirstPersonCharacter.ActivatorObjectName` (`/Game/Blueprints/Components/BP_ActivatorComponent.ActivatorItemCode` (`self.BP_ActivatorComponent`)) PlayerPref)
  (`self.Destroy Item`)
  (return null))

(fn `ThrowObject`
  (params (PlayerPref :type "/Game/FirstPerson/Blueprints/BP_FirstPersonCharacter Object Reference"))
  (bind _pickupable (`self.Pickupable`))
  (bind _meshpickupable (`/Game/FirstPerson/Blueprints/BP_FirstPersonCharacter.MeshPickupable` (`self.PlayerPref`)))
  (set `self.PlayerPref` PlayerPref)
  (`/Engine/EditorBlueprintResources/StandardMacros.IsValid` _meshpickupable
    (:`Is Valid`
      (`StaticMeshComponent.SetStaticMesh` _pickupable _meshpickupable)
      (`SceneComponent.SetWorldScale3D` _pickupable (`/Game/FirstPerson/Blueprints/BP_FirstPersonCharacter.PickupableVector` (`self.PlayerPref`)))
      (`PrimitiveComponent.SetSimulatePhysics` _pickupable true)
      (`PrimitiveComponent.AddImpulse` _pickupable (* (`self.GetActorForwardVector`) (`/Game/FirstPerson/Blueprints/BP_FirstPersonCharacter.ThrowForce` (`self.PlayerPref`))) "None" true)
      (`StaticMeshComponent.SetStaticMesh` (`/Game/FirstPerson/Blueprints/BP_FirstPersonCharacter.Pickupable Item` (`self.PlayerPref`)) null)
      (set `/Game/FirstPerson/Blueprints/BP_FirstPersonCharacter.IsHoldingItem` false (`self.PlayerPref`))
      (set `/Game/FirstPerson/Blueprints/BP_FirstPersonCharacter.MeshPickupable` null (`self.PlayerPref`))
      (return))))

(fn `UserConstructionScript`)