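; BP_TableCamera is a level camera for the player waking from a nightmare at a table.
; The WakeUpEventEnabler event triggers a fade-in, instant camera switch, teleport to the table spawn point and lamp state restore.
; It then takes interact-button priority, so a press makes the player get up.
; Getting up runs a timed fade, ends the camera mid-fade with a chair sound, repositions the player and releases the priority.
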(event `self.ReceiveBeginPlay`
  (bind _wakeupeventenabler (`self.WakeUpEventEnabler`)
    (:`then`
      (add `/Game/Blueprints/EventItems/BP_JumpscareMom.WakeUpFromNightmare` _wakeupeventenabler (delegate `Wake Up`)))
    (:`else`)))

(event `Wake Up`
  (params (PlayerPref :type "/Game/FirstPerson/Blueprints/BP_FirstPersonCharacter Object Reference"))
  (set `self.Player Pref` PlayerPref)
  (`/Game/Blueprints/Components/BP_FadeScreenComponent.Fade In` (`self.BP_FadeScreenComponent`) (`self.Player Pref`))
  (`self.Initialize Level Camera` (`self.Player Pref`))
  (`self.Move Character near Table`)
  (`/Game/FirstPerson/Blueprints/BP_FirstPersonCharacter.Set Interact Button Priority` (`self.Player Pref`))
  (add `/Game/FirstPerson/Blueprints/BP_FirstPersonCharacter.InteractButtonPressed` (`self.Player Pref`) (delegate `Get Up`))
  (`self.RestoreAllLampState`))

(event `Move Character near Table`
  (bind _property_item (`/Game/Blueprints/ModularItems/BP_PropertyItem.Property Item` (`self.SpawnAreaTable`)))
  (`self.K2_SetActorLocationAndRotation` (`self.Player Pref`) (`SceneComponent.K2_GetComponentLocation` _property_item) (`SceneComponent.K2_GetComponentRotation` _property_item) false true))

(event `self.Initialize Level Camera`
  (params (`Player Pref` :type "/Game/FirstPerson/Blueprints/BP_FirstPersonCharacter Object Reference") (`Blend Time` :type "Float (double-precision)"))
  (`parent.Initialize Level Camera` `Player Pref` `Blend Time`)
  (`self.Move Character near Table`))

(event `Get Up`
  (`/Game/Blueprints/Components/BP_FadeScreenComponent.Fade Event` (`self.BP_FadeScreenComponent`) 4.0 (`self.Player Pref`))
  (`KismetSystemLibrary.Delay` 2.0)
  (`self.End Level Camera`)
  (`GameplayStatics.PlaySound2D` "/Game/Sounds/sfx_moving-chair.sfx_moving-chair" 1.0 1.0 0.0 null null)
  (`self.Move Character near Table`)
  (`/Game/FirstPerson/Blueprints/BP_FirstPersonCharacter.Unset Interact Button Priority` (`self.Player Pref`)))

(fn `UserConstructionScript`
  (`parent.UserConstructionScript`))