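; BP_TeaserCamera is a level camera that takes over as the game starts, judging by its name for teaser shots.
; On BeginPlay, if its Action reference is valid, it casts the player to BP_FirstPersonCharacter and calls InitializeLevelCamera with zero blend time.
; Disconnected leftover nodes would play the merry-go-round sound and enable rain visuals and audio, but never run.
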(event `self.ReceiveBeginPlay`
  (`self.Action?`
    (:`then`
      (`|ExecutionSequence`
        (:`then_0`
          (bind _asbp_first_person_character (cast `/Game/FirstPerson/Blueprints/BP_FirstPersonCharacter` (`GameplayStatics.GetPlayerCharacter` 0)))
          (`self.Initialize Level Camera` _asbp_first_person_character))))
    (:`else`)))

(fn `UserConstructionScript`
  (`parent.UserConstructionScript`))