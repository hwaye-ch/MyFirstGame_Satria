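; Level camera for the toilet that runs the Chapter 1 opening sequence.
; StartChapter1Event cuts to the camera without blending, then after timed delays plays the front door's welcome sound and starts a screen fade.
; When the fade component reports it has finished, the camera plays a flush sound, ends itself and unlocks the first BP_Door tagged "toilet1".
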(event `Start Chapter 1 Event`
  (bind _bp_fadescreencomponent (`self.BP_FadeScreenComponent`))
  (`self.Initialize Level Camera` (`self.Player Ref`))
  (`KismetSystemLibrary.Delay` 10.0)
  (bind _returnvalue (`GameplayStatics.GetActorOfClass` "/Game/Convenience_Store/Blueprints/BP_Front_Door.BP_Front_Door_C"))
  (`/Game/Convenience_Store/Blueprints/BP_Front_Door.Play Welcome Sound` _returnvalue)
  (`KismetSystemLibrary.Delay` 5.0)
  (add `/Game/Blueprints/Components/BP_FadeScreenComponent.OnFadeEventFinished` _bp_fadescreencomponent (delegate `OnFadeEventFinished_Event`))
  (`/Game/Blueprints/Components/BP_FadeScreenComponent.Fade Event` _bp_fadescreencomponent 5.0 (`self.Player Ref`) 2.0))

(event `OnFadeEventFinished_Event`
  (`AudioComponent.Play` (`self.sfx_flush`) 0.0)
  (`self.End Level Camera`)
  (bind _outactors (`GameplayStatics.GetAllActorsWithTag` "toilet1"))
  (bind _asbp_door (cast `/Game/Convenience_Store/Blueprints/BP_Door` (`|GetArrayItem` _outactors)))
  (set `/Game/Convenience_Store/Blueprints/BP_Door.IsLocked?` false _asbp_door))

(fn `UserConstructionScript`
  (`parent.UserConstructionScript`))