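; Chapter 7A window interactable that blends the player's view to its child-actor level camera and ends it on the next interact press.
; When the event is ready, a one-time sequence shows window dialogue and tells the chapter manager to move NPCs, binding the exit input after dialogue ends.
; Otherwise exit input binds immediately with priority.
; The first event exit clears the flag, then plays a sad sound and hides the crutch-tagged actor after a delay.
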(event `self.ReceiveBeginPlay`
  (`parent.ReceiveBeginPlay`)
  (bind _returnvalue (`GameplayStatics.GetActorOfClass` "/Game/Blueprints/Items/BP_Chapter7AManager.BP_Chapter7AManager_C"))
  (set `self.ChapterManager` _returnvalue))

(event `/Game/Blueprints/Interface/BPI_Actionable.InteractObject`
  (bind _playerref (`self.PlayerRef`))
  (bind _bp_dialoguecomponent (`self.BP_DialogueComponent`))
  (bind _asbp_level_camera (cast `/Game/Blueprints/ModularItems/BP_LevelCamera` (`ChildActorComponent.ChildActor` (`self.ChildActor`))))
  (bind _output_get (set `self.As BP Level Camera` _asbp_level_camera))
  (`/Game/Blueprints/ModularItems/BP_LevelCamera.Initialize Level Camera` _output_get (`self.PlayerRef`) 0.4)
  (`self.IsEventReady?`
    (:`then`
      (`/Engine/EditorBlueprintResources/StandardMacros.DoOnce` false
        (:`Completed`
          (`KismetSystemLibrary.Delay` 2.0)
          (bind _dialoguecomponent (`/Game/Blueprints/Components/BP_DialogueComponent.Construct Dialogue` (`self.BP_DialogueComponent`) "ch7_window_1" "/Game/Dialogue/Chapter7_Dialogue.Chapter7_Dialogue" false false))
          (`/Game/Blueprints/Interface/BPI_Dialogue.ShowDialogue` _dialoguecomponent (`self.PlayerRef`) self)
          (add `/Game/Blueprints/Components/BP_DialogueComponent.OnDialogueEnded` _bp_dialoguecomponent (delegate `OnDialogueEnded_Event`))
          (`/Game/Blueprints/Items/BP_Chapter7AManager.MoveNPCs` (`self.ChapterManager`)))))
    (:`else`
      (add `/Game/FirstPerson/Blueprints/BP_FirstPersonCharacter.InteractButtonPressed` _playerref (delegate `InteractButtonPressed_Event`) :!label _label)
      (set `/Game/FirstPerson/Blueprints/BP_FirstPersonCharacter.IsInteractButtonPriority?` true _playerref)
      (clear `/Game/Blueprints/Components/BP_DialogueComponent.OnDialogueEnded` _bp_dialoguecomponent))))

(event `OnDialogueEnded_Event`
  (goto _label))

(event `InteractButtonPressed_Event`
  (`/Game/Blueprints/ModularItems/BP_LevelCamera.End Level Camera` (`self.As BP Level Camera`))
  (set `/Game/FirstPerson/Blueprints/BP_FirstPersonCharacter.IsInteractButtonPriority?` false (`self.PlayerRef`))
  (clear `/Game/FirstPerson/Blueprints/BP_FirstPersonCharacter.InteractButtonPressed` (`self.PlayerRef`))
  (`self.IsEventReady?`
    (:`then`
      (`/Engine/EditorBlueprintResources/StandardMacros.DoOnce` false
        (:`Completed`
          (set `self.IsEventReady?` false)
          (`KismetSystemLibrary.Delay` 2.0)
          (`GameplayStatics.PlaySound2D` "/Game/Sounds/backsound-sad.backsound-sad" 1.0 1.0 0.0 null null)
          (bind _outactors (`GameplayStatics.GetAllActorsWithTag` "crutch"))
          (`self.SetActorHiddenInGame` (`|GetArrayItem` _outactors) true))))
    (:`else`)))

(fn `UserConstructionScript`
  (`parent.UserConstructionScript`))