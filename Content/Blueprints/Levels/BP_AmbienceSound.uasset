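; Level ambience controller actor that plays a night ambience at its location and layers 2D horror sounds over it.
; Custom events start the ambience once, keep its audio component and set its volume directly.
; Timelines lerp that volume down to a low level, reverse to restore it, or fade it from low to silence.
; Starting the horror soundscape drops the ambience to minimum volume, while a second horror ambience plays independently.
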(event `Play Sound Ambience`
  (`self.EnvironmentalSound`
    (:`then`)
    (:`else`
      (bind _returnvalue (`GameplayStatics.SpawnSoundAtLocation` "/Game/Sounds/sfx_night-ambience.sfx_night-ambience" (`self.K2_GetActorLocation` self) (struct) (`self.MaxVolume`) 1.0 0.0 null null))
      (set `self.EnvironmentalSound` _returnvalue))))

(event `Stop the Ambience Sound`
  (bind _environmentalsound (`self.EnvironmentalSound`)
    (:`then`
      (bind (_direction _newtrack_0) (`Timeline|Timeline_0`)
        (:`Update`
          (`AudioComponent.SetVolumeMultiplier` _environmentalsound (`KismetMathLibrary.Lerp` (`self.LowVolume`) 0.0 _newtrack_0)))))
    (:`else`)))

(event `Lower the Volume`
  (bind _environmentalsound (`self.EnvironmentalSound`)
    (:`then`
      (bind (_direction _newtrack_0) (`Timeline|Timeline` :!label _label)
        (:`Update`
          (`AudioComponent.SetVolumeMultiplier` _environmentalsound (`KismetMathLibrary.Lerp` (`self.MaxVolume`) (`self.LowVolume`) _newtrack_0)))))
    (:`else`)))

(event `Increase the Volume`
  (goto _label :!via `Reverse`))

(event `Play Horror Bg Sound`
  (bind _returnvalue (`GameplayStatics.SpawnSound2D` "/Game/Sounds/sfx_soundscapehorror.sfx_soundscapehorror" 0.075 1.0 0.0 null))
  (set `self.HorrorAmbience` _returnvalue)
  (bind _environmentalsound (`self.EnvironmentalSound`)
    (:`then`
      (`AudioComponent.SetVolumeMultiplier` _environmentalsound (`self.MinVolume`)))
    (:`else`)))

(event `Set Ambience Volume`
  (params (Volume :type "Float (double-precision)"))
  (`AudioComponent.SetVolumeMultiplier` (`self.EnvironmentalSound`) Volume))

(event `Set Horror Ambience`
  (`GameplayStatics.SpawnSound2D` "/Game/Sounds/sfx_horror-ambience.sfx_horror-ambience" 0.5 1.0 0.0 null))

(fn `UserConstructionScript`
  (`parent.UserConstructionScript`))