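; BP_AmbienceSoundModifier is a trigger volume that ducks a referenced ambience sound and boosts footstep sound while the first-person character is inside its box.
; Begin overlap lowers the ambience volume and increases the character's footsteps; end overlap restores full ambience and lowers the footsteps.
; BeginPlay waits one tick, then queries the box so a character already inside gets the same effect.
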(event `self.ReceiveBeginPlay`
  (`parent.ReceiveBeginPlay`)
  (`KismetSystemLibrary.DelayUntilNextTick`)
  (bind _asbp_first_person_character (cast `/Game/FirstPerson/Blueprints/BP_FirstPersonCharacter` (`|GetArrayItem` (`PrimitiveComponent.GetOverlappingActors` (`self.Box`) "/Game/FirstPerson/Blueprints/BP_FirstPersonCharacter.BP_FirstPersonCharacter_C"))))
  (`/Game/Blueprints/Levels/BP_AmbienceSound.Set Ambience Volume` (`self.AmbienceSound`) 0.1)
  (`/Game/FirstPerson/Blueprints/BP_FirstPersonCharacter.Increase Footstep Sound` _asbp_first_person_character))

(event `self.Box.OnComponentBeginOverlap`
  (params (OverlappedComponent :type "PrimitiveComponent Object Reference") (OtherActor :type "Actor Object Reference") (OtherComp :type "PrimitiveComponent Object Reference") (OtherBodyIndex :type Integer) (bFromSweep :type Boolean) (SweepResult :type "HitResult Structure (by ref)"))
  (bind _asbp_first_person_character (cast `/Game/FirstPerson/Blueprints/BP_FirstPersonCharacter` OtherActor))
  (bind _ambiencesound (`self.AmbienceSound`)
    (:`then`
      (`/Game/Blueprints/Levels/BP_AmbienceSound.Set Ambience Volume` _ambiencesound 0.1)
      (`/Game/FirstPerson/Blueprints/BP_FirstPersonCharacter.Increase Footstep Sound` _asbp_first_person_character))
    (:`else`)))

(event `self.Box.OnComponentEndOverlap`
  (params (OverlappedComponent :type "PrimitiveComponent Object Reference") (OtherActor :type "Actor Object Reference") (OtherComp :type "PrimitiveComponent Object Reference") (OtherBodyIndex :type Integer))
  (bind _asbp_first_person_character (cast `/Game/FirstPerson/Blueprints/BP_FirstPersonCharacter` OtherActor))
  (bind _ambiencesound (`self.AmbienceSound`)
    (:`then`
      (`/Game/Blueprints/Levels/BP_AmbienceSound.Set Ambience Volume` _ambiencesound 1.0)
      (`/Game/FirstPerson/Blueprints/BP_FirstPersonCharacter.Lower Footstep Sound` _asbp_first_person_character))
    (:`else`)))

(fn `UserConstructionScript`
  (`parent.UserConstructionScript`))