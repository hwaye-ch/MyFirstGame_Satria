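; BP_Chapter5Manager runs the timed scripted sequence for Chapter 5 when PlayChapter5 is called.
; It closes and reopens Ryan's door, plays a cooking sound effect, turns on the television, has the Father peep and return, then turns the television off.
; Delays space the beats in a single chain of nested validity checks, so a missing actor reference stops the rest of the sequence.
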(event `Play Chapter 5`
  ; Door opened mysteriously
  (bind _ryan_sdoor (`self.Ryan'sDoor`)
    (:`then`
      (`/Game/Blueprints/EventItems/BP_RyansRoomsDoor.Close the Door` _ryan_sdoor)
      (`KismetSystemLibrary.Delay` 10.0)
      (`/Game/Blueprints/EventItems/BP_RyansRoomsDoor.Open Door by Event` _ryan_sdoor)
      (`KismetSystemLibrary.Delay` 16.0)
      ; Cooking Sound Effect
      (bind _cookingsfx (`self.CookingSfx`)
        (:`then`
          (`/Game/Blueprints/Interface/BPI_Executable.Execute` _cookingsfx)
          (`KismetSystemLibrary.Delay` 10.0)
          ; Television Segment
          (bind _television (`self.Television`)
            (:`then`
              (`/Game/Blueprints/EventItems/BP_Television.Turn On TV` _television)
              (`KismetSystemLibrary.Delay` 10.0)
              ; Father Peeping
              (bind _father (`self.Father`)
                (:`then`
                  (`/Game/Blueprints/EventItems/BP_FatherPeepingDoor.Peep` _father)
                  (`KismetSystemLibrary.Delay` 10.0)
                  (`/Game/Blueprints/EventItems/BP_FatherPeepingDoor.Return from peep` _father)
                  (`KismetSystemLibrary.Delay` 10.0)
                  (`/Game/Blueprints/EventItems/BP_Television.Turn Off TV` _television))
                (:`else`)))
            (:`else`)))
        (:`else`)))
    (:`else`)))

(fn `UserConstructionScript`
  (`parent.UserConstructionScript`))