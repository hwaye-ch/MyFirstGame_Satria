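; Level trigger actor that starts a dialogue when BP_FirstPersonCharacter enters its TriggerBox.
; On overlap it calls ShowDialogueMessage on its BPI_Dialogue components with the current DialogueCode, then stores and debug-prints the next code.
; It hands the end-of-dialogue flag, next code and first dialogue component to the character.
; Its own ShowDialogue function is a stub returning default values.
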(event `self.TriggerBox.OnComponentBeginOverlap`
  (params (OverlappedComponent :type "PrimitiveComponent Object Reference") (OtherActor :type "Actor Object Reference") (OtherComp :type "PrimitiveComponent Object Reference") (OtherBodyIndex :type Integer) (bFromSweep :type Boolean) (SweepResult :type "HitResult Structure (by ref)"))
  (bind _returnvalue (`self.GetComponentsByInterface` "/Game/Blueprints/Interface/BPI_Dialogue.BPI_Dialogue_C"))
  (bind _asbp_first_person_character (cast `/Game/FirstPerson/Blueprints/BP_FirstPersonCharacter` OtherActor))
  (bind (_isendofdialogue _nextdialoguecode) (message `/Game/Blueprints/Interface/BPI_Dialogue.ShowDialogue` _returnvalue (`self.DialogueCode`)))
  (`KismetSystemLibrary.PrintString` (`KismetStringLibrary.Conv_NameToString` _nextdialoguecode))
  (set `/Game/FirstPerson/Blueprints/BP_FirstPersonCharacter.IsDialogueEnded` _isendofdialogue _asbp_first_person_character)
  (set `/Game/FirstPerson/Blueprints/BP_FirstPersonCharacter.DialogueActor` (`|GetArrayItem` _returnvalue) _asbp_first_person_character)
  (bind _output_get (set `self.DialogueCode` _nextdialoguecode))
  (set `/Game/FirstPerson/Blueprints/BP_FirstPersonCharacter.DialogueCode` _output_get _asbp_first_person_character))

(fn `ShowDialogue`
  (params (DialogueCode :type Name))
  (returns (isEndOfDialogue :type Boolean) (NextDialogueCode :type Name))
  (return false "None"))

(fn `UserConstructionScript`)