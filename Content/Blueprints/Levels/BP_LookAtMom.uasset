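; Level trigger actor that fires a one-time jumpscare when the player's hit actor is tagged "Mom".
; Once ready, it checks the player's hit actor on tick, then sets the player's panic flag.
; A timeline rotates the bed camera toward the mom-on-bed actor's item, then turns off that camera's look state.
; Alongside this, it plays a loud 2D sting and calls ShowDanOnBed on the father-on-bed actor.
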(event `self.ReceiveBeginPlay`
  (`parent.ReceiveBeginPlay`))

(event `self.ReceiveTick`
  (params (DeltaSeconds :type "Float (single-precision)"))
  (`KismetSystemLibrary.DelayUntilNextTick`)
  (`self.IsReady?`
    (:`then`
      (bind _hit_actor (`/Game/FirstPerson/Blueprints/BP_FirstPersonCharacter.Hit Actor` (`self.Player Pref`))
        (:`then`
          (if (`self.ActorHasTag` _hit_actor "Mom")
            (`/Engine/EditorBlueprintResources/StandardMacros.DoOnce` false
              (:`Completed`
                (`|ExecutionSequence`
                  (:`then_0`
                    (bind _returnvalue (`GameplayStatics.GetActorOfClass` "/Game/Blueprints/EventItems/BP_MomOnBed.BP_MomOnBed_C"))
                    (bind _returnvalue_2 (`GameplayStatics.GetActorOfClass` "/Game/Blueprints/LevelCameras/BP_BedCamera.BP_BedCamera_C"))
                    (set `/Game/FirstPerson/Blueprints/BP_FirstPersonCharacter.IsPanic` true (`self.Player Pref`))
                    (bind (_direction _newtrack_0) (`Timeline|Timeline` :!via `PlayFromStart`)
                      (:`Update`
                        (bind _camera (`/Game/Blueprints/ModularItems/BP_LevelCamera.Camera` _returnvalue_2))
                        (`SceneComponent.K2_SetWorldRotation` _camera (`KismetMathLibrary.RLerp` (`SceneComponent.K2_GetComponentRotation` _camera) (`KismetMathLibrary.FindLookAtRotation` (`SceneComponent.K2_GetComponentLocation` _camera) (`SceneComponent.K2_GetComponentLocation` (`/Game/Blueprints/ModularItems/BP_PropertyItem.Property Item` _returnvalue))) _newtrack_0) false false))
                      (:`Finished`
                        (`/Game/Blueprints/ModularItems/BP_LevelCamera.Set Look` _returnvalue_2 false))))
                  (:`then_1`
                    (`GameplayStatics.SpawnSound2D` "/Game/Sounds/sfx_jumpscare-mom.sfx_jumpscare-mom" 3.0 1.0 0.0 null)
                    (bind _returnvalue_3 (`GameplayStatics.GetActorOfClass` "/Game/Blueprints/EventItems/BP_FatherOnBed.BP_FatherOnBed_C"))
                    (`/Game/Blueprints/EventItems/BP_FatherOnBed.Show Dan on Bed` _returnvalue_3)))))))
        (:`else`)))
    (:`else`)))

(fn `UserConstructionScript`
  (`parent.UserConstructionScript`))