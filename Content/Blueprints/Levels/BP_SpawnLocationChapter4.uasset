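; BP_SpawnLocationChapter4 is a Chapter 4 level actor acting as a fixed, clamped-look camera for the player, apparently at a table with a laptop.
; TeleportPlayer switches the view to this actor, disables controller input and registers it as the player's TableCamera.
; LookInput applies clamped yaw and pitch, while MoveCamera polls the player's action values in a self-recalling Delay loop.
; The actual teleport, look-at-laptop and fade-in chain is disconnected.
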(event `Teleport Player`
  (params (BP_Laptop :type "/Game/Blueprints/EventItems/BP_Laptop Object Reference"))
  (bind _returnvalue (`GameplayStatics.GetPlayerController` 0))
  (bind _player_pref (`self.Player Pref`))
  (set `self.BP Laptop` BP_Laptop)
  (`PlayerController.SetViewTargetWithBlend` _returnvalue self 0.0 "VTBlend_Linear" 0.0 false)
  (`self.DisableInput` _returnvalue null)
  (set `/Game/FirstPerson/Blueprints/BP_FirstPersonCharacter.IsCameraChanged?` true _player_pref)
  (set `/Game/FirstPerson/Blueprints/BP_FirstPersonCharacter.TableCamera` self _player_pref))

(event `LookInput`
  (params (Yaw :type "Float (double-precision)") (Pitch :type "Float (double-precision)"))
  (bind (_relativerotation_roll _relativerotation_pitch _relativerotation_yaw) (`KismetMathLibrary.BreakRotator` (`SceneComponent.RelativeRotation` (`self.Camera`))))
  (`SceneComponent.K2_SetRelativeRotation` (`self.Camera`) (`KismetMathLibrary.MakeRotator` 0.0 (`KismetMathLibrary.FClamp` (+ _relativerotation_pitch (* Pitch -1.0)) -60.0 60.0) (`KismetMathLibrary.FClamp` (+ _relativerotation_yaw Yaw) -60.0 60.0)) false false)
  (`KismetSystemLibrary.Delay` 0.0001))

(event `Move Camera`
  (bind _output_get (set `self.Pitch` (`KismetMathLibrary.FClamp` (+ (`self.Pitch`) (`/Game/FirstPerson/Blueprints/BP_FirstPersonCharacter.Action Value X` (`self.Player Pref`))) -45.0 45.0)))
  (bind _output_get_2 (set `self.Yaw` (`KismetMathLibrary.FClamp` (+ (`/Game/FirstPerson/Blueprints/BP_FirstPersonCharacter.Action Value Y` (`self.Player Pref`)) (`self.Yaw`)) -60.0 60.0)))
  (`SceneComponent.K2_SetRelativeRotation` (`self.Camera`) (`KismetMathLibrary.MakeRotator` 0.0 (* _output_get -1.0) _output_get_2) false false)
  (`KismetSystemLibrary.Delay` 0.0001)
  (`self.Move Camera`))

(fn `UserConstructionScript`
  (`parent.UserConstructionScript`))