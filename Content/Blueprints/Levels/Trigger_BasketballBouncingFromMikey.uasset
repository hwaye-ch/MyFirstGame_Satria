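; Level trigger for the Mikey room event, which its name ties to a bouncing basketball.
; On BeginPlay it binds to the Enabler's ActivateMikeyRoomEvent, if the Enabler is valid, so its overlap area is armed only when that event fires.
; An overlap then calls TriggerMikeyRoomEvent to start the event, with debug prints at both the arming and trigger steps.
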(event `self.ReceiveBeginPlay`
  (bind _enabler (`self.Enabler`))
  (`parent.ReceiveBeginPlay`)
  (`/Engine/EditorBlueprintResources/StandardMacros.IsValid` _enabler
    (:`Is Valid`
      (add `/Game/Blueprints/EventItems/BP_Dumpster.ActivateMikeyRoomEvent` _enabler (delegate `Enable Trigger Area`)))))

(event `Enable Trigger Area`
  (`KismetSystemLibrary.PrintString` "Mikey Event Trigger is ready")
  (`self.Activate Overlap Trigger`))

(event `/Game/Blueprints/Interface/BPI_Trigger.OnOverlapTrigger`
  (`KismetSystemLibrary.PrintString` "Mikey Event is executed")
  (`self.TriggerMikeyRoomEvent`))

(fn `UserConstructionScript`
  (`parent.UserConstructionScript`))