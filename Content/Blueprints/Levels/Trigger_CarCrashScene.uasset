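; Level trigger that stages the car crash cutscene when overlapped, playing the basketball scene sequence.
; On overlap it disables player movement and look, teleports the player to the basketball court, sets control rotation and spawns an explosion starter at the explosion area.
; When the sequence finishes, it re-enables look only and moves the chasing car to the explosion area.
; A separate SpawnExplossion event activates the explosion, then its SFX after a delay.
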(event `self.ReceiveBeginPlay`
  (`parent.ReceiveBeginPlay`)
  (bind _returnvalue (`GameplayStatics.GetActorOfClass` "/Game/Objects/BP_ChasingCar.BP_ChasingCar_C"))
  (set `self.The Car` _returnvalue)
  (bind _returnvalue_2 (`GameplayStatics.GetActorOfClass` "/Game/Blueprints/Levels/SpawnArea_Explossion.SpawnArea_Explossion_C"))
  (set `self.ExplossionArea` _returnvalue_2))

(event `/Game/Blueprints/Interface/BPI_Trigger.OnOverlapTrigger`
  (`KismetSystemLibrary.PrintString` "Playing Cutscene" true true (struct :`R` 1.0 :`B` 0.175299 :`A` 1.0))
  (bind (_outactor _returnvalue) (`LevelSequencePlayer.CreateLevelSequencePlayer` "/Game/Animation/Anim_BasketballScene.Anim_BasketballScene"))
  (`MovieSceneSequencePlayer.Play` _returnvalue)
  (`/Game/FirstPerson/Blueprints/BP_FirstPersonCharacter.Disable Movement and Look` (`self.PlayerRef`))
  (add `MovieSceneSequencePlayer.OnFinished` _returnvalue (delegate `OnFinishedCutscene`))
  (bind _returnvalue_2 (`GameplayStatics.GetActorOfClass` "/Game/Blueprints/Levels/SpawnArea_BasketballCourt.SpawnArea_BasketballCourt_C"))
  (`self.K2_SetActorLocation` (`self.PlayerRef`) (`self.K2_GetActorLocation` _returnvalue_2) false false)
  (`Controller.SetControlRotation` (`GameplayStatics.GetPlayerController` 0) (`KismetMathLibrary.FindLookAtRotation` (`SceneComponent.GetForwardVector` (`/Game/FirstPerson/Blueprints/BP_FirstPersonCharacter.FirstPersonCamera` (`self.PlayerRef`))) (`self.K2_GetActorLocation` (`self.ExplossionArea`))))
  (bind _returnvalue_3 (`|SpawnActorFromClass` "/Game/Blueprints/EventItems/BP_ExplossionAnimationStarter.BP_ExplossionAnimationStarter_C" (`self.GetTransform` (`self.ExplossionArea`)) "Undefined" "MultiplyWithRoot" null null))
  (set `self.Explossion` _returnvalue_3))

(event `OnFinishedCutscene`
  (`/Game/FirstPerson/Blueprints/BP_FirstPersonCharacter.Enable Look` (`self.PlayerRef`))
  (`self.K2_SetActorLocation` (`self.The Car`) (`self.K2_GetActorLocation` (`self.ExplossionArea`)) false true))

(event `SpawnExplossion`
  (bind _explossion (`self.Explossion`)
    (:`then`
      (`/Game/Blueprints/EventItems/BP_ExplossionAnimationStarter.Activate` _explossion)
      (`KismetSystemLibrary.Delay` 2.0)
      (`ActorComponent.Activate` (`/Game/Blueprints/Levels/SpawnArea_Explossion.sfx_explossion` (`self.ExplossionArea`)) false))
    (:`else`)))

(fn `UserConstructionScript`
  (`parent.UserConstructionScript`))