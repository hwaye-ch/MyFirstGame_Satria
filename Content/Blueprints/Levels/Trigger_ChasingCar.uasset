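; Level trigger that starts a car chase, with a cinematic intro, suspense music and panic camera shake.
; On overlap it reveals the car's Mikey mesh, plays the chase-start level sequence and locks player movement and look.
; When the sequence finishes it turns the player toward the car, starts music, calls the chase and restores control.
; Tick then repeats the camera shake at the player, while the car's PlayerDead event stops the music.
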(event `/Game/Blueprints/Interface/BPI_Trigger.OnOverlapTrigger`
  (bind (_outactor _returnvalue) (`LevelSequencePlayer.CreateLevelSequencePlayer` "/Game/Animation/Anim_CarStartedToChase.Anim_CarStartedToChase"))
  (`SceneComponent.SetVisibility` (`/Game/Objects/BP_ChasingCar.MikeyMesh` (`self.CarToLookAt`)) true true)
  (set `self.SequencePlayer` _returnvalue)
  (`MovieSceneSequencePlayer.Play` (`self.SequencePlayer`))
  (add `MovieSceneSequencePlayer.OnFinished` _returnvalue (delegate `On Finished Animation`))
  (`/Game/FirstPerson/Blueprints/BP_FirstPersonCharacter.Disable Movement and Look` (`self.PlayerRef`))
  (add `/Game/Objects/BP_ChasingCar.Player Dead` (`self.CarToLookAt`) (delegate `Stop Music`)))

(event `On Finished Animation`
  (`KismetSystemLibrary.PrintString` "Animation Finished, Player look at the car! \n")
  (`Controller.SetControlRotation` (`GameplayStatics.GetPlayerController` 0) (`KismetMathLibrary.FindLookAtRotation` (`self.K2_GetActorLocation` (`self.PlayerRef`)) (`self.K2_GetActorLocation` (`self.CarToLookAt`))))
  (`AudioComponent.Play` (`self.SuspensefulMusic`) 0.0)
  (`self.CarStartChasing`)
  (`/Game/FirstPerson/Blueprints/BP_FirstPersonCharacter.Enable Look and Movement` (`self.PlayerRef`))
  (set `self.Is Event Starting?` true))

(event `Stop Music`
  (`AudioComponent.Stop` (`self.SuspensefulMusic`)))

(event `self.ReceiveTick`
  (params (DeltaSeconds :type "Float (single-precision)"))
  (`self.Is Event Starting?`
    (:`then`
      (`GameplayStatics.PlayWorldCameraShake` "/Game/FirstPerson/Blueprints/CameraShake/CameraShake_Panic.CameraShake_Panic_C" (`self.K2_GetActorLocation` (`self.PlayerRef`)) 0.0 1000.0))
    (:`else`)))

(fn `UserConstructionScript`
  (`parent.UserConstructionScript`))