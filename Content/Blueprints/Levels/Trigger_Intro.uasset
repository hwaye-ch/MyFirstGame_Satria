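; Level trigger Blueprint that plays the Chapter 6 intro dialogue when its overlap event fires.
; When the player's current chapter is 6, it builds the intro dialogue from the Chapter 6 dialogue table with movement and look blocked, then shows it.
; In any other chapter, it has the dialogue component display its automatic message instead.
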(event `/Game/Blueprints/Interface/BPI_Trigger.OnOverlapTrigger`
  (if (== (`/Game/FirstPerson/Blueprints/BP_FirstPersonCharacter.CurrentChapter` (`self.PlayerPref`)) 6)
    (bind _dialoguecomponent (`/Game/Blueprints/Components/BP_DialogueComponent.Construct Dialogue` (`self.BP_DialogueComponent`) "ch6_intro_0" "/Game/Dialogue/Chapter6_Dialogue.Chapter6_Dialogue" true true))
    (`/Game/Blueprints/Interface/BPI_Dialogue.ShowDialogue` _dialoguecomponent (`self.PlayerPref`) self)
    (else
      (message `/Game/Blueprints/Interface/BPI_Dialogue.DisplayAutoDialogue` (`self.BP_DialogueComponent`)))))

(fn `UserConstructionScript`
  (`parent.UserConstructionScript`))