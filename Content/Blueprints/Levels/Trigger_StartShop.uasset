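; Level trigger that starts the convenience store sequence when its overlap event fires.
; It plays the store cinematic, activates the red car's audio, calls SetCollisionSetting(true) on the shop barrier and unlocks the front door.
; The car and door are cached on BeginPlay via GetActorOfClass, while the barrier is looked up on overlap.
; When the cinematic finishes, the red car is destroyed if still valid.
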(event `self.ReceiveBeginPlay`
  (`parent.ReceiveBeginPlay`)
  (bind _returnvalue (`GameplayStatics.GetActorOfClass` "/Game/Blueprints/EventItems/BP_RedCar.BP_RedCar_C"))
  (set `self.RedCar` _returnvalue)
  (bind _returnvalue_2 (`GameplayStatics.GetActorOfClass` "/Game/Convenience_Store/Blueprints/BP_Front_Door.BP_Front_Door_C"))
  (set `self.FrontDoor` _returnvalue_2))

(event `/Game/Blueprints/Interface/BPI_Trigger.OnOverlapTrigger`
  (`|ExecutionSequence`
    (:`then_0`
      (bind (_outactor _returnvalue) (`LevelSequencePlayer.CreateLevelSequencePlayer` "/Game/Animation/Anim_ConvenienceStoreCinematic.Anim_ConvenienceStoreCinematic"))
      (add `MovieSceneSequencePlayer.OnFinished` _returnvalue (delegate `OnFinished_Event`))
      (`MovieSceneSequencePlayer.Play` _returnvalue)
      (`ActorComponent.Activate` (`/Game/Blueprints/EventItems/BP_RedCar.Audio` (`self.RedCar`)) false))
    (:`then_1`
      (bind _returnvalue_2 (`GameplayStatics.GetActorOfClass` "/Game/Blueprints/Levels/Barrier_Shop.Barrier_Shop_C"))
      (`self.Set Collision Setting` _returnvalue_2 true))
    (:`then_2`
      (set `/Game/Convenience_Store/Blueprints/BP_Front_Door.IsLocked` false (`self.FrontDoor`)))))

(event `OnFinished_Event`
  (bind _redcar (`self.RedCar`)
    (:`then`
      (`self.K2_DestroyActor` _redcar))
    (:`else`)))

(fn `UserConstructionScript`
  (`parent.UserConstructionScript`))