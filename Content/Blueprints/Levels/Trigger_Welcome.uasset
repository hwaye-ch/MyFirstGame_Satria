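; Welcome trigger that plays an introductory dialogue on overlap, chosen by the player's current chapter.
; Chapter 1 shows the dialogue component's own dialogue and fires EnableKulkas.
; Chapter 2 builds its dialogue from that chapter's table, blocking movement and look.
; Chapter 3 fires StartCountingTrash, then displays a table-built auto message after a one-tick delay.
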(event `/Game/Blueprints/Interface/BPI_Trigger.OnOverlapTrigger`
  (switch `int` (`/Game/FirstPerson/Blueprints/BP_FirstPersonCharacter.CurrentChapter` (`self.PlayerPref`))
    (:`1`
      (`/Game/Blueprints/Interface/BPI_Dialogue.ShowDialogue` (`self.BP_DialogueComponent`) (`self.PlayerPref`) self)
      (`self.EnableKulkas`))
    (:`2`
      (bind _dialoguecomponent (`/Game/Blueprints/Components/BP_DialogueComponent.Construct Dialogue` (`self.BP_DialogueComponent`) "ch2_welcome" "/Game/Dialogue/Chapter2_Dialogue.Chapter2_Dialogue" true true))
      (`/Game/Blueprints/Components/BP_DialogueComponent.ShowDialogue` _dialoguecomponent (`self.PlayerPref`) self))
    (:`3`
      (`self.StartCountingTrash`)
      (bind _dialoguecomponent_2 (`/Game/Blueprints/Components/BP_DialogueComponent.Construct Dialogue` (`self.BP_DialogueComponent`) "ch3_welcome" "/Game/Dialogue/Chapter3_Dialogue.Chapter3_Dialogue" false false))
      (`KismetSystemLibrary.DelayUntilNextTick`)
      (message `/Game/Blueprints/Interface/BPI_Dialogue.DisplayAutoDialogue` _dialoguecomponent_2))))

(fn `ShowDialogue`
  (params (PlayerPref :type "/Game/FirstPerson/Blueprints/BP_FirstPersonCharacter Object Reference") (DialogueActorTrigger :type "Actor Object Reference"))
  (return))

(fn `UserConstructionScript`)