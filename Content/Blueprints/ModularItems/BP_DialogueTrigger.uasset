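; Modular trigger actor that starts dialogue when the first-person character enters its trigger box.
; The overlap stores the player and hands it to BPDialogueComponent to show the message, then destroys the trigger box unless KeepActor is set.
; An optional barrier box gets blocking collision from EnableCollision at construction and BeginPlay.
; FinishDialogue flags the player's dialogue text as complete; the local ShowDialogue function is empty.
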(event `self.ReceiveBeginPlay`
  (if (`self.EnableCollision`)
    (`PrimitiveComponent.SetCollisionEnabled` (`self.BarrierBox`) "QueryAndPhysics")
    (else
      (`PrimitiveComponent.SetCollisionEnabled` (`self.BarrierBox`) "NoCollision"))))

(event `self.TriggerBox.OnComponentBeginOverlap`
  (params (OverlappedComponent :type "PrimitiveComponent Object Reference") (OtherActor :type "Actor Object Reference") (OtherComp :type "PrimitiveComponent Object Reference") (OtherBodyIndex :type Integer) (bFromSweep :type Boolean) (SweepResult :type "HitResult Structure (by ref)"))
  (bind _asbp_first_person_character (cast `/Game/FirstPerson/Blueprints/BP_FirstPersonCharacter` OtherActor))
  (bind _output_get (set `self.PlayerPref` _asbp_first_person_character))
  (message `/Game/Blueprints/Interface/BPI_Dialogue.ShowDialogue` (`self.BP_DialogueComponent`) _output_get self)
  (if (not (`/Game/Blueprints/Components/BP_DialogueComponent.KeepActor` (`self.BP_DialogueComponent`)))
    (`ActorComponent.K2_DestroyComponent` (`self.TriggerBox`))))

(event `/Game/Blueprints/Interface/BPI_Dialogue.FinishDialogue`
  (`KismetSystemLibrary.PrintString` "Aku sudah selesai btw")
  (set `/Game/FirstPerson/Blueprints/BP_FirstPersonCharacter.IsDialogueTextComplete` true (`self.PlayerPref`)))

(fn `ShowDialogue`
  (params (PlayerPref :type "/Game/FirstPerson/Blueprints/BP_FirstPersonCharacter Object Reference") (DialogueActorTrigger :type "Actor Object Reference"))
  (return))

(fn `UserConstructionScript`
  (if (`self.EnableCollision`)
    (`PrimitiveComponent.SetCollisionEnabled` (`self.BarrierBox`) "QueryAndPhysics")
    (`PrimitiveComponent.SetCollisionResponseToChannel` (`self.BarrierBox`) "ECC_Pawn" "ECR_Block")
    (else
      (`PrimitiveComponent.SetCollisionEnabled` (`self.BarrierBox`) "NoCollision"))))