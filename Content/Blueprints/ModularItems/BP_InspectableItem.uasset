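; BP_InspectableItem is an item the player can bring up to inspect, rotate with IA_Look, and put back.
; OnBeginInspecting toggles inspection, using TL_Inspect to lerp between the item's original transform and the player's InspectablePosition, reversing on exit.
; While inspecting, player movement and camera look are disabled.
; Progress and finish events fire when BPSequenceActivator's sequence is active, and a child flag can override the return transform.
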(event `EnhancedInput|/Game/FirstPerson/Input/Actions/IA_Look`
  (params (ActionValue :type "Vector2D Structure") (ElapsedSeconds :type "Float (double-precision)") (TriggeredSeconds :type "Float (double-precision)") (InputAction :type "InputAction Object Reference" :default "/Game/FirstPerson/Input/Actions/IA_Look.IA_Look"))
  (:`Triggered`
    (if (`self.CanInspect?`)
      (`SceneComponent.K2_AddLocalRotation` (`self.InspectableItem`) (`KismetMathLibrary.MakeRotator` (* ActionValue_X 0.4) 0.0 (* ActionValue_Y 0.4)) false false))))

(event `/Game/Blueprints/Interface/BPI_Inspect.OnBeginInspecting`
  (params (PlayerPref :type "/Game/FirstPerson/Blueprints/BP_FirstPersonCharacter Object Reference"))
  (bind _returnvalue (`GameplayStatics.GetPlayerController` 0))
  (bind _inspectableitem (`self.InspectableItem`))
  (bind _player_pref (`self.Player Pref`))
  (bind _player_pref_2 (`self.Player Pref`))
  (set `self.Player Pref` PlayerPref)
  (`/Game/Blueprints/Interface/BPI_Inspect.OnStartInspecting`)
  (if (`self.CanInspect?`)
    (`|ExecutionSequence`
      (:`then_0`
        (goto _label_2 :!via `Reset`))
      (:`then_1`
        (set `self.CanInspect?` false)
        (set `/Game/FirstPerson/Blueprints/BP_FirstPersonCharacter.ActiveInspectableItem` null _player_pref)
        (set `/Game/FirstPerson/Blueprints/BP_FirstPersonCharacter.IsInspecting` false _player_pref)
        (`CharacterMovementComponent.SetMovementMode` (`Character.CharacterMovement` (`GameplayStatics.GetPlayerCharacter` 0)) "MOVE_Walking" 0)
        (set `PlayerController.bShowMouseCursor` false _returnvalue)
        (`Controller.ResetIgnoreLookInput` _returnvalue)
        (`WidgetBlueprintLibrary.SetInputMode_GameOnly` _returnvalue)
        (if (`/Game/Blueprints/Components/BP_SequenceActivator.IsSequenceActivated` (`self.BP_SequenceActivator`))
          (`self.OnFinishedInspecting`)
          (bind (_direction __) (`Timeline|TL_Inspect` :!via `Reverse` :!label _label)
            (:`Update`
              (`SceneComponent.K2_SetWorldTransform` (`self.InspectableItem`) (`KismetMathLibrary.MakeTransform` (`KismetMathLibrary.VLerp` (`self.Original Location`) (`self.InspectableLocation`) __) (`KismetMathLibrary.RLerp` (`self.Original Rotation`) (`self.InspectableRotation`) __) (`SceneComponent.K2_GetComponentScale` (`self.InspectableItem`))) false false)
              (`KismetSystemLibrary.Delay` 0.31)
              (if (`self.IsLocationChangedInChild`)
                (set `self.Original Location` (`self.Initial Location`))
                (set `self.Original Rotation` (`self.Initial Rotation`)))))
          (else
            (goto _label :!via `Reverse`)))))
    (else
      (set `self.Original Location` (`SceneComponent.K2_GetComponentLocation` _inspectableitem))
      (set `self.Original Rotation` (`SceneComponent.K2_GetComponentRotation` _inspectableitem))
      (`self.EnableInput` (`GameplayStatics.GetPlayerController` 0))
      (`/Engine/EditorBlueprintResources/StandardMacros.DoOnce` false :!label _label_2
        (:`Completed`
          (set `PlayerController.bShowMouseCursor` false (`GameplayStatics.GetPlayerController` 0))
          (if (`/Game/Blueprints/Components/BP_SequenceActivator.IsSequenceActivated` (`self.BP_SequenceActivator`))
            (`self.OnProgressInspecting`))
          (set `self.CanInspect?` true)
          (set `/Game/FirstPerson/Blueprints/BP_FirstPersonCharacter.ActiveInspectableItem` self _player_pref_2)
          (set `/Game/FirstPerson/Blueprints/BP_FirstPersonCharacter.IsInspecting` true _player_pref_2)
          (`CharacterMovementComponent.DisableMovement` (`Character.CharacterMovement` (`GameplayStatics.GetPlayerCharacter` 0)))
          (`Controller.SetIgnoreLookInput` (`GameplayStatics.GetPlayerController` 0) true)
          (goto _label))))))

(event `/Game/Blueprints/Interface/BPI_Inspect.OnStartInspecting`
  (bind (_returnvalue_location _returnvalue_rotation) (`KismetMathLibrary.BreakTransform` (`SceneComponent.K2_GetComponentToWorld` (`/Game/FirstPerson/Blueprints/BP_FirstPersonCharacter.Inspectable Position` (`self.Player Pref`)))))
  (set `self.InspectableLocation` _returnvalue_location)
  (set `self.InspectableRotation` _returnvalue_rotation))

(fn `UserConstructionScript`)