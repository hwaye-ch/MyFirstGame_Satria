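; BP_InteractableDoor is a modular interactable door that swings open and closed, with lock and peek-mode options.
; Interact stores the player, then either calls the empty StartPeeking event or, if unlocked and not moving, toggles the door with a sound.
; Timelines lerp the door's yaw toward a direction-dependent angle, and SetDoorClosed reverses a separate timeline.
; BeginPlay reveals the peephole sphere and mesh when ShowPeepHole is set.
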(event `self.ReceiveBeginPlay`
  (if (`self.ShowPeepHole`)
    (`SceneComponent.SetVisibility` (`self.Sphere`) true false)
    (`SceneComponent.SetVisibility` (`self.StaticMesh`) true false)))

(event `/Game/Blueprints/Interface/BPI_Engageable.Interact`
  (params (PlayerRef :type "/Game/FirstPerson/Blueprints/BP_FirstPersonCharacter Object Reference"))
  (set `self.Player Pref` PlayerRef)
  (if (`self.IsPeekMode`)
    (`self.Start Peeking`)
    (elif (`self.IsLocked`)
      _
      (elif (not (`self.IsOpening`))
        (set `self.IsOpening` true)
        (if (`self.OpenForward`)
          (set `self.YawValue` (`self.OpenBackwardValue`))
          (else
            (set `self.YawValue` (`self.OpenForwardValue`))))
        (bind _output_get (set `self.IsDoorOpened` (not (`self.IsDoorOpened`))))
        (if _output_get
          (`GameplayStatics.PlaySound2D` "/Game/Sounds/sfx_door_opened.sfx_door_opened" 1.0 1.0 0.0 null null)
          (bind (_direction _door_alpha) (`Timeline|TL_Doors` :!label _label)
            (:`Update`
              (`SceneComponent.K2_SetRelativeRotation` (`self.Door`) (`KismetMathLibrary.MakeRotator` 0.0 0.0 (`KismetMathLibrary.Lerp` 0.0 (`self.YawValue`) _door_alpha)) false false))
            (:`Finished`
              (set `self.IsOpening` false)))
          (else
            (`GameplayStatics.PlaySound2D` "/Game/Sounds/sfx_door_closed.sfx_door_closed" 1.0 1.0 0.0 null null)
            (goto _label :!via `Reverse`)))))))

(event `Set Door Closed`
  (`self.IsDoorOpened`
    (:`then`
      (bind (_direction _door_alpha) (`Timeline|Timeline` :!via `Reverse`)
        (:`Update`
          (`SceneComponent.K2_SetRelativeRotation` (`self.Door`) (`KismetMathLibrary.MakeRotator` 0.0 0.0 (`KismetMathLibrary.Lerp` 0.0 (`self.YawValue`) _door_alpha)) false false))
        (:`Finished`
          (set `self.IsOpening` false))))
    (:`else`)))

(event `Start Peeking`)

(fn `UserConstructionScript`)