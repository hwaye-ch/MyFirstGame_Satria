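; BP_LevelCamera is a fixed camera that temporarily takes over the player's view.
; Initialize and End events switch the view target, set the player's camera override state and toggle their movement and look.
; Look input adjusts the camera's relative rotation, with yaw and inverted pitch clamped to a limited range.
; GetCameraTrace supplies trace endpoints from the camera along its forward vector, out to the maximum interact range.
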(event `Initialize Level Camera`
  (params (`Player Pref` :type "/Game/FirstPerson/Blueprints/BP_FirstPersonCharacter Object Reference"))
  (set `self.Player Pref` `Player Pref`)
  (`PlayerController.SetViewTargetWithBlend` (`GameplayStatics.GetPlayerController` 0) self 0.0 "VTBlend_Linear" 0.0 false)
  (set `/Game/FirstPerson/Blueprints/BP_FirstPersonCharacter.IsViewingThroughLevelCam?` true (`self.Player Pref`))
  (set `/Game/FirstPerson/Blueprints/BP_FirstPersonCharacter.OverridedCamera` self (`self.Player Pref`))
  (`/Game/FirstPerson/Blueprints/BP_FirstPersonCharacter.Disable Movement and Look` (`self.Player Pref`)))

(event `End Level Camera`
  (set `/Game/FirstPerson/Blueprints/BP_FirstPersonCharacter.IsViewingThroughLevelCam?` false (`self.Player Pref`))
  (`PlayerController.SetViewTargetWithBlend` (`GameplayStatics.GetPlayerController` 0) (`self.Player Pref`) 0.0 "VTBlend_Linear" 0.0 false)
  (set `/Game/FirstPerson/Blueprints/BP_FirstPersonCharacter.OverridedCamera` null (`self.Player Pref`))
  (`/Game/FirstPerson/Blueprints/BP_FirstPersonCharacter.Enable Look and Movement` (`self.Player Pref`)))

(event `Look Through Level Camera`
  (params (Yaw :type "Float (double-precision)") (Pitch :type "Float (double-precision)"))
  (bind (_relativerotation_roll _relativerotation_pitch _relativerotation_yaw) (`KismetMathLibrary.BreakRotator` (`SceneComponent.RelativeRotation` (`self.Camera`))))
  (`SceneComponent.K2_SetRelativeRotation` (`self.Camera`) (`KismetMathLibrary.MakeRotator` 0.0 (`KismetMathLibrary.FClamp` (+ _relativerotation_pitch (* Pitch -1.0)) -60.0 60.0) (`KismetMathLibrary.FClamp` (+ _relativerotation_yaw Yaw) -60.0 60.0)) false false))

(fn `Get Camera Trace`
  (returns (Start :type "Vector Structure") (End :type "Vector Structure"))
  (bind _camera (`self.Camera`))
  (bind _returnvalue (`SceneComponent.K2_GetComponentLocation` _camera))
  (return _returnvalue (+ (* (`SceneComponent.GetForwardVector` _camera) (`self.MaxInteractRange`)) _returnvalue)))

(fn `UserConstructionScript`
  (`parent.UserConstructionScript`))