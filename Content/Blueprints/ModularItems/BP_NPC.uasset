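; BP_NPC is an interactable NPC that starts talking when a player interacts with it.
; On BeginPlay it binds to its dialogue component's start and end events and caches the HwyGameInstance.
; Those dialogue events toggle an idle/talk state through CallToggleIdleAndTalk.
; Interact stores the player reference and calls TalkWithObject, while InteractObject and ShowDialogue are empty stubs.
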(event `self.ReceiveBeginPlay`
  (bind _bp_dialoguecomponent (`self.BP_DialogueComponent`))
  (add `/Game/Blueprints/Components/BP_DialogueComponent.OnDialogStarted` _bp_dialoguecomponent (delegate `Handle Dialogue Started`))
  (add `/Game/Blueprints/Components/BP_DialogueComponent.OnDialogueEnded` _bp_dialoguecomponent (delegate `Handle Dialogue Ended`))
  (bind _ashwy_game_instance (cast `/Game/System/HwyGameInstance` (`GameplayStatics.GetGameInstance`)))
  (set `self.Game Instance Ref` _ashwy_game_instance))

(event `Handle Dialogue Started`
  (`self.ToggleIdleAndTalk` true))

(event `Handle Dialogue Ended`
  (`self.ToggleIdleAndTalk` false))

(event `/Game/Blueprints/Interface/BPI_Engageable.Interact`
  (params (PlayerRef :type "/Game/FirstPerson/Blueprints/BP_FirstPersonCharacter Object Reference"))
  (set `self.PlayerRef` PlayerRef)
  (`/Game/Blueprints/Interface/BPI_Talk.TalkWithObject`))

(fn `InteractObject`
  (params (PlayerPref :type "/Game/FirstPerson/Blueprints/BP_FirstPersonCharacter Object Reference"))
  (returns (MeshBentukan :type "StaticMesh Object Reference"))
  (return null))

(fn `ShowDialogue`
  (params (PlayerPref :type "/Game/FirstPerson/Blueprints/BP_FirstPersonCharacter Object Reference") (DialogueActorTrigger :type "Actor Object Reference"))
  (return))

(fn `UserConstructionScript`)