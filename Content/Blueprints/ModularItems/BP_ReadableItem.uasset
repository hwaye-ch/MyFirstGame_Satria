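; BP_ReadableItem is an interactable actor the player can read, showing a description widget from its readable component.
; Interact toggles between Read Item and Dismiss Item, flipping the player's IsReading state.
; Reading plays a widget animation, registers the item on the player and disables movement and look before calling ReadObject.
; Dismissing plays the closing animation, waits briefly, removes the widget and restores control.
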(event `self.ReceiveBeginPlay`
  (set `self.OriginalLocation` (`self.GetTransform`)))

(event `/Game/Blueprints/Interface/BPI_Engageable.Interact`
  (params (PlayerRef :type "/Game/FirstPerson/Blueprints/BP_FirstPersonCharacter Object Reference"))
  (bind _widget (`self.Widget`))
  (bind _output_get (set `self.Player Ref` PlayerRef))
  (bind _isreading (`/Game/FirstPerson/Blueprints/BP_FirstPersonCharacter.IsReading` _output_get)
    (:`then`
      (bind _widget_2 (`self.Widget`)
        (:`then`
          (`UserWidget.PlayAnimation` _widget_2 (`/Game/Blueprints/Widgets/WBP_ReadItemDescription.DoneReading` _widget_2) 0.0 1 "Forward" 1.0 false)
          (set `/Game/FirstPerson/Blueprints/BP_FirstPersonCharacter.Active Readable Item` null (`self.Player Ref`))
          (`KismetSystemLibrary.Delay` 0.5)
          (`Widget.RemoveFromParent` (`self.Widget`))
          (`/Game/FirstPerson/Blueprints/BP_FirstPersonCharacter.Enable Look and Movement` (`self.Player Ref`)))
        (:`else`)))
    (:`else`
      (bind _returnvalue (`/Game/Blueprints/Components/BP_TextRelatedComponent.Show Object Description` (`self.BP_ReadableComponent`)))
      (set `self.Widget` _returnvalue)
      (`UserWidget.PlayAnimation` _widget (`/Game/Blueprints/Widgets/WBP_ReadItemDescription.Reading` _widget) 0.0 1 "Forward" 1.0 false)
      (`/Game/FirstPerson/Blueprints/BP_FirstPersonCharacter.Disable Movement and Look` (`self.Player Ref`))
      (set `/Game/FirstPerson/Blueprints/BP_FirstPersonCharacter.Active Readable Item` self (`self.Player Ref`))
      (`/Game/Blueprints/Interface/BPI_Readable.Read Object`)))
  (set `/Game/FirstPerson/Blueprints/BP_FirstPersonCharacter.IsReading` (not _isreading) (`self.Player Ref`)))

(fn `UserConstructionScript`)