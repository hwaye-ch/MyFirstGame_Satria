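; BP_ThrowableItem is a modular item actor that handles throwing the player's held item and removes itself when picked up.
; ThrowObject spawns a BP_PickupableItem at the held mesh's transform, copying the player's stored mesh and scale.
; It enables physics, applies a velocity-change impulse along this actor's forward vector, then clears the player's held state.
; PickupObject only triggers a briefly delayed self-destroy.
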(event `Destroy Item`
  (`KismetSystemLibrary.Delay` 0.01)
  (`self.K2_DestroyActor`))

(event `/Game/Blueprints/Interface/BPI_Pickup.ThrowObject`
  (params (PlayerPref :type "/Game/FirstPerson/Blueprints/BP_FirstPersonCharacter Object Reference"))
  (bind _meshpickupable (`/Game/FirstPerson/Blueprints/BP_FirstPersonCharacter.MeshPickupable` (`self.Player Pref`)))
  (set `self.Player Pref` PlayerPref)
  (bind _returnvalue (`|SpawnActorFromClass` "/Game/Blueprints/ModularItems/BP_PickupableItem.BP_PickupableItem_C" (`SceneComponent.GetSocketTransform` (`/Game/FirstPerson/Blueprints/BP_FirstPersonCharacter.Pickupable Item` PlayerPref) "None" "RTS_World") "Undefined" "MultiplyWithRoot" null null))
  (`/Engine/EditorBlueprintResources/StandardMacros.IsValid` _meshpickupable
    (:`Is Valid`
      (bind _pickupable (`/Game/Blueprints/ModularItems/BP_PickupableItem.Pickupable` _returnvalue))
      (`StaticMeshComponent.SetStaticMesh` _pickupable _meshpickupable)
      (`SceneComponent.SetWorldScale3D` _pickupable (`/Game/FirstPerson/Blueprints/BP_FirstPersonCharacter.PickupableVector` (`self.Player Pref`)))
      (`PrimitiveComponent.SetSimulatePhysics` _pickupable true)
      (`PrimitiveComponent.AddImpulse` _pickupable (* (`self.GetActorForwardVector`) (`/Game/FirstPerson/Blueprints/BP_FirstPersonCharacter.ThrowForce` (`self.Player Pref`))) "None" true)
      (`StaticMeshComponent.SetStaticMesh` (`/Game/FirstPerson/Blueprints/BP_FirstPersonCharacter.Pickupable Item` (`self.Player Pref`)) null)
      (set `/Game/FirstPerson/Blueprints/BP_FirstPersonCharacter.IsHoldingItem` false (`self.Player Pref`))
      (set `/Game/FirstPerson/Blueprints/BP_FirstPersonCharacter.MeshPickupable` null (`self.Player Pref`)))))

(fn `PickupObject`
  (params (PlayerPref :type "/Game/FirstPerson/Blueprints/BP_FirstPersonCharacter Object Reference"))
  (returns (ThrowableActor :type "/Game/Blueprints/ModularItems/BP_PickupableItem Object Reference"))
  (`self.Destroy Item`)
  (return null))

(fn `UserConstructionScript`)