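; BP_TriggerArea is a modular trigger volume that reacts when the first-person character walks into it, with a barrier box whose collision is set at BeginPlay.
; Overlap passes a DoOnce gate, reset by ActivateTrigger, then checks BPEnablerComponent's readiness.
; When ready, it stores the player, calls OnTriggerMessage and destroys the collision box unless KeepTrigger is set.
; OnTrigger itself only prints a debug string.
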(event `self.ReceiveBeginPlay`
  (if (`self.EnableCollision`)
    (`PrimitiveComponent.SetCollisionEnabled` (`self.BarrierBox`) "QueryAndPhysics")
    (else
      (`PrimitiveComponent.SetCollisionEnabled` (`self.BarrierBox`) "NoCollision"))))

(event `self.CollisionBox.OnComponentBeginOverlap`
  (params (OverlappedComponent :type "PrimitiveComponent Object Reference") (OtherActor :type "Actor Object Reference") (OtherComp :type "PrimitiveComponent Object Reference") (OtherBodyIndex :type Integer) (bFromSweep :type Boolean) (SweepResult :type "HitResult Structure (by ref)"))
  (bind _asbp_first_person_character (cast `/Game/FirstPerson/Blueprints/BP_FirstPersonCharacter` OtherActor))
  (`/Engine/EditorBlueprintResources/StandardMacros.DoOnce` true :!label _label
    (:`Completed`
      (if (`/Game/Blueprints/Components/BP_EnablerComponent.IsReadyToInteract` (`self.BP_EnablerComponent`))
        (set `self.PlayerPref` _asbp_first_person_character)
        (message `/Game/Blueprints/Interface/BPI_Trigger.OnTrigger` self)
        (if (not (`/Game/Blueprints/Components/BP_EnablerComponent.KeepTrigger?` (`self.BP_EnablerComponent`)))
          (`ActorComponent.K2_DestroyComponent` (`self.CollisionBox`)))
        (else
          (`KismetSystemLibrary.PrintString` "Trigger Area is not set ready"))))))

(event `Activate Trigger`
  (goto _label :!via `Reset`))

(event `/Game/Blueprints/Interface/BPI_Trigger.OnTrigger`
  (`KismetSystemLibrary.PrintString` "Kamu sudah di sini"))

(fn `UserConstructionScript`)