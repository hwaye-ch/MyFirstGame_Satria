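; BP_Mikey is a character Blueprint for Mikey, an NPC that reacts to dialogue and extends a parent class.
; Dialogue start prints a debug string and toggles the talk state on through CallToggleIdleAndTalk.
; Dialogue end prints, calls CallUnblockBarrier and toggles the talk state off.
; The end handler invokes the parent's HandleDialogueStarted rather than a parent end handler.
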(event `self.ReceiveBeginPlay`
  (`parent.ReceiveBeginPlay`))

(event `self.Handle Dialogue Started`
  (`parent.Handle Dialogue Started`)
  (`KismetSystemLibrary.PrintString` "Start Dialogue wih Mikey")
  (`self.ToggleIdleAndTalk` true))

(event `self.Handle Dialogue Ended`
  (`parent.Handle Dialogue Started`)
  (`KismetSystemLibrary.PrintString` "End Dialogue with Mikey")
  (`self.UnblockBarrier`)
  (`self.ToggleIdleAndTalk` false))

(fn `UserConstructionScript`
  (`parent.UserConstructionScript`))