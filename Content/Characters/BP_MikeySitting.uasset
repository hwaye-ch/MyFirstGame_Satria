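; Seated Mikey NPC for Chapter 7A who relocates and becomes talkable when the chapter's move-NPCs event fires.
; On BeginPlay he hides his crutch and registers that event with BP_Chapter7AManager.
; The event snaps him to SpawnArea_Mikey, applies the sick AnimBP, shows the crutch and builds his movement- and look-blocking dialogue.
; Talking, gated on event readiness, shows the dialogue and notifies the manager once to enable dialogue.
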(event `self.ReceiveBeginPlay`
  (`parent.ReceiveBeginPlay`)
  (bind _returnvalue (`GameplayStatics.GetActorOfClass` "/Game/Blueprints/Items/BP_Chapter7AManager.BP_Chapter7AManager_C"))
  (bind _output_get (set `self.ChapterManager` _returnvalue))
  (add `/Game/Blueprints/Items/BP_Chapter7AManager.MoveNPCs` _output_get (delegate `MoveNPCs_Event`))
  (`SceneComponent.SetVisibility` (`self.Crutch`) false true))

(event `MoveNPCs_Event`
  (bind _returnvalue (`GameplayStatics.GetActorOfClass` "/Game/Blueprints/Levels/SpawnArea_Mikey.SpawnArea_Mikey_C"))
  (`self.K2_SetActorLocationAndRotation` (`self.K2_GetActorLocation` _returnvalue) (`self.K2_GetActorRotation` _returnvalue))
  (`SkeletalMeshComponent.SetAnimationMode` (`self.Mesh`) "AnimationSingleNode" true)
  (`SkeletalMeshComponent.SetAnimInstanceClass` (`self.Mesh`) "/Game/Blueprints/Characters/ABP_MikeySick.ABP_MikeySick_C")
  (`SceneComponent.SetVisibility` (`self.Crutch`) true true)
  (set `self.IsEventReady?` true)
  (`/Game/Blueprints/Components/BP_DialogueComponent.Construct Dialogue` (`self.BP_DialogueComponent`) "ch7_mikey_0" "/Game/Dialogue/Chapter7_Dialogue.Chapter7_Dialogue" true true))

(event `/Game/Blueprints/Interface/BPI_Talk.TalkWithObject`
  (`self.IsEventReady?`
    (:`then`
      (`/Game/Blueprints/Interface/BPI_Dialogue.ShowDialogue` (`self.BP_DialogueComponent`) (`self.PlayerRef`) self)
      (`/Engine/EditorBlueprintResources/StandardMacros.DoOnce` false
        (:`Completed`
          (`/Game/Blueprints/Items/BP_Chapter7AManager.EnableDialogue` (`self.ChapterManager`) "NewEnumerator1"))))
    (:`else`)))

(fn `UserConstructionScript`
  (`parent.UserConstructionScript`))