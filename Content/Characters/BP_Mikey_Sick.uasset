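; BP_Mikey_Sick is a talkable character Blueprint for Mikey in his sick state.
; Its chapter 2 setup event builds movement- and look-blocking dialogue from the Chapter 2 table and swaps in the sick mesh and anim Blueprint.
; Dialogue start and end toggle idle/talk, and ending also unblocks a barrier.
; The end handler calls the parent's dialogue-started handler rather than an ended one.
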(event `self.ReceiveBeginPlay`
  (`parent.ReceiveBeginPlay`))

(event `self.Handle Dialogue Started`
  (`parent.Handle Dialogue Started`)
  (`KismetSystemLibrary.PrintString` "Start Dialogue wih Mikey")
  (`self.ToggleIdleAndTalk` true))

(event `self.Handle Dialogue Ended`
  (`parent.Handle Dialogue Started`)
  (`KismetSystemLibrary.PrintString` "End Dialogue with Mikey")
  (`self.UnblockBarrier`)
  (`self.ToggleIdleAndTalk` false))

(event `Setup event for chapter 2`
  (`/Game/Blueprints/Components/BP_DialogueComponent.Construct Dialogue` (`self.BP_DialogueComponent`) "ch2_ryan1" "/Game/Dialogue/Chapter2_Dialogue.Chapter2_Dialogue" true true)
  (`SkeletalMeshComponent.SetSkeletalMeshAsset` (`self.Mesh`) "/Game/Objects/Mikey/MikeySick/Mikey_sick.Mikey_sick")
  (`SkeletalMeshComponent.SetAnimInstanceClass` (`self.Mesh`) "/Game/Blueprints/Characters/ABP_MikeySick.ABP_MikeySick_C"))

(fn `UserConstructionScript`
  (`parent.UserConstructionScript`))