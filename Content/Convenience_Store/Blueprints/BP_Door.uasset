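; Modular convenience store wall-and-door Blueprint that swings the door open or closed on interaction.
; The construction script picks wall, wallpaper, frame, trim, sign and metal plate from type settings, destroying unwanted components.
; Door removal is limited to one wall type; the others use a fixed frame, reposition the door and drop the sign.
; InteractObject plays or reverses a yaw Timeline over 90 degrees, using flags to block re-triggering and track open state.
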(event `/Game/Blueprints/Interface/BPI_Actionable.InteractObject`
  (`self.IsOpening?`
    (:`then`)
    (:`else`
      (set `self.IsOpening?` true)
      (`self.IsDoorOpened?`
        (:`then`
          (bind (_direction _newtrack_0) (`Timeline|Timeline` :!via `Reverse` :!label _label)
            (:`Update`
              (`SceneComponent.K2_SetRelativeRotation` (`self.Door`) (`KismetMathLibrary.MakeRotator` 0.0 0.0 (`KismetMathLibrary.Lerp` 0.0 90.0 _newtrack_0)) false false))
            (:`Finished`
              (set `self.IsOpening?` false)
              (set `self.IsDoorOpened?` (not (`self.IsDoorOpened?`))))))
        (:`else`
          (goto _label))))))

(fn `UserConstructionScript`
  (locals (Wall_Meshes :type "Array of StaticMesh Object Reference") (Wall_Inside_Choice :type Boolean) (Wall_Materials :type "Array of MaterialInstance Object Reference") (Door_Frame_Meshes :type "Array of StaticMesh Object Reference") (Door_Choice :type Integer) (Sign_Meshes :type "Array of StaticMesh Object Reference") (Trim_Meshes :type "Array of StaticMesh Object Reference") (Trim_Meshes_Inside :type "Array of StaticMesh Object Reference") (Sign_Disabled :type Boolean) (Door_Disabled :type Boolean) (Metalplate_Disabled :type Boolean))
  (bind _door (`self.Door`))
  (bind _returnvalue (`KismetMathLibrary.Conv_ByteToInt` (`self.Wall_Type`)))
  (if (`self.Door_is_present`)
    (set `local.Door_Choice` 0)
    (else
      (set `local.Door_Choice` 1)))
  ;[1 0.9963 0.9853] Wall
  (`StaticMeshComponent.SetStaticMesh` (`self.Wall`) (`|GetArrayItem` (`local.Wall_Meshes`) _returnvalue))
  (set `local.Wall_Inside_Choice` (== _returnvalue 1))
  (`PrimitiveComponent.SetMaterial` (`self.Wall`) 0 (`|GetArrayItem` (`local.Wall_Materials`) (`KismetMathLibrary.Conv_ByteToInt` (`self.Wallpaper_Type`))))
  ;[1 1 1] Door Frame
  (if (`local.Wall_Inside_Choice`)
    (`StaticMeshComponent.SetStaticMesh` (`self.Door_Frame`) (`|GetArrayItem` (`local.Door_Frame_Meshes`) (`local.Door_Choice`)))
    ;[1 1 1] Door
    (`StaticMeshComponent.SetStaticMesh` (`self.Door`) "/Game/Convenience_Store/Meshes/SM_Door.SM_Door")
    (if (`self.Door_is_present`)
      ;[1 1 1] Signs
      (`StaticMeshComponent.SetStaticMesh` (`self.Sign`) (`|GetArrayItem` (`local.Sign_Meshes`) (`KismetMathLibrary.Conv_ByteToInt` (`self.Sign_Type`))))
      ;[1 1 1] Metalplate
      (`StaticMeshComponent.SetStaticMesh` (`self.Metal_Plate`) "/Game/Convenience_Store/Meshes/SM_Door_Metalplate.SM_Door_Metalplate" :!label _label)
      (else
        (`ActorComponent.K2_DestroyComponent` (`self.Door`))))
    (else
      (`StaticMeshComponent.SetStaticMesh` (`self.Door_Frame`) (`|GetArrayItem` (`local.Door_Frame_Meshes`) 2))
      (`StaticMeshComponent.SetStaticMesh` _door "/Game/Convenience_Store/Meshes/SM_Door.SM_Door")
      (`SceneComponent.K2_SetRelativeLocation` _door (-44.197281 -22.365051 107.84288) false false)
      (`ActorComponent.K2_DestroyComponent` (`self.Sign`))
      (goto _label)))
  ;[1 1 1] Wall Trims
  (if (`local.Wall_Inside_Choice`)
    (`StaticMeshComponent.SetStaticMesh` (`self.Wall_Trim`) (`|GetArrayItem` (`local.Trim_Meshes_Inside`) (`KismetMathLibrary.Conv_ByteToInt` (`self.Wall_Trim_Type`))))
    (else
      (`StaticMeshComponent.SetStaticMesh` (`self.Wall_Trim`) (`|GetArrayItem` (`local.Trim_Meshes`) (`KismetMathLibrary.Conv_ByteToInt` (`self.Wall_Trim_Type`))))))
  ;[1 1 1] Disable Signs
  (set `local.Sign_Disabled` (== (`KismetMathLibrary.Conv_ByteToInt` (`self.Sign_Type`)) 0))
  (if (`local.Sign_Disabled`)
    (`ActorComponent.K2_DestroyComponent` (`self.Sign`)))
  ;[1 1 1] Disable Metalplate
  (set `local.Metalplate_Disabled` (== (`KismetMathLibrary.Conv_ByteToInt` (`self.Metalplate`)) 0))
  (if (`local.Metalplate_Disabled`)
    (`ActorComponent.K2_DestroyComponent` (`self.Metal_Plate`))))