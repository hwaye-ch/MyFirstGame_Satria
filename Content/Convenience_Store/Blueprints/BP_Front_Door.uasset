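; BP_Front_Door is the convenience store's interactable front door, swinging a leaf open or closed.
; InteractObject skips locked or moving doors, then plays or reverses the OpenDoor timeline to lerp the left leaf's yaw toward a forward or back angle.
; Opening plays a door sound and welcome audio, while closing plays a delayed close sound.
; The construction script picks the Front mesh from an array by FrontType.
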(event `/Game/Blueprints/Interface/BPI_Actionable.InteractObject`
  (bind _returnvalue (`self.K2_GetActorLocation`))
  (`self.IsLocked`
    (:`then`)
    (:`else`
      (`self.IsOpening?`
        (:`then`)
        (:`else`
          (set `self.IsOpening?` true)
          (`self.IsDoorOpenedForward?`
            (:`then`
              (set `self.DefaultOpenValue` (`self.OpenForwardValue`)))
            (:`else`
              (set `self.DefaultOpenValue` (`self.OpenBackValue`))))
          (`self.IsDoorOpened?`
            (:`then`
              (`|ExecutionSequence`
                (:`then_0`
                  (`KismetSystemLibrary.Delay` 0.5)
                  (`GameplayStatics.PlaySoundAtLocation` "/Game/Sounds/sfx_close-shop-door.sfx_close-shop-door" _returnvalue (struct) 0.2 1.0 0.0 "/Game/Sounds/BasketballBounce/SA_ProximitySound.SA_ProximitySound" null null null))
                (:`then_1`
                  (bind (_direction _newtrack_0) (`Timeline|Open Door` :!via `Reverse` :!label _label)
                    (:`Update`
                      (`SceneComponent.K2_SetWorldRotation` (`self.Door_Leaf_Left`) (`KismetMathLibrary.MakeRotator` 0.0 0.0 (`KismetMathLibrary.Lerp` 0.0 (`self.DefaultOpenValue`) _newtrack_0)) false false))
                    (:`Finished`
                      (set `self.IsOpening?` false)
                      (set `self.IsDoorOpened?` (not (`self.IsDoorOpened?`))))))))
            (:`else`
              (`GameplayStatics.PlaySoundAtLocation` "/Game/Sounds/sfx_open-shop-door.sfx_open-shop-door" _returnvalue (struct) 0.4 1.0 0.0 "/Game/Sounds/BasketballBounce/SA_ProximitySound.SA_ProximitySound" null null null)
              (`self.Play Welcome Sound`)
              (goto _label))))))))

(event `Play Welcome Sound`
  (`AudioComponent.Play` (`self.sfx_welcome-convenience-store`) 0.0))

(fn `UserConstructionScript`
  (locals (Meshes :type "Array of StaticMesh Object Reference"))
  (`StaticMeshComponent.SetStaticMesh` (`self.Front`) (`|GetArrayItem` (`local.Meshes`) (`KismetMathLibrary.Conv_ByteToInt` (`self.Front_Type`)))))