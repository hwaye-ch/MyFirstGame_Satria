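; BP_Gondola_Shelf is a convenience store gondola shelf prop with a configurable mesh on each of its two sides.
; The construction script converts the ShelfSide1 and ShelfSide2 selections to indices into the shared ShelfMeshes array, setting the static meshes on ShelfSideA and ShelfSideB.
; It has no runtime logic, as the event graph holds only disabled default events.
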(fn `UserConstructionScript`
  (locals (Shelf_Meshes :type "Array of StaticMesh Object Reference"))
  (`StaticMeshComponent.SetStaticMesh` (`self.Shelf_Side_A`) (`|GetArrayItem` (`local.Shelf_Meshes`) (`KismetMathLibrary.Conv_ByteToInt` (`self.Shelf_Side_1`))))
  (`StaticMeshComponent.SetStaticMesh` (`self.Shelf_Side_B`) (`|GetArrayItem` (`local.Shelf_Meshes`) (`KismetMathLibrary.Conv_ByteToInt` (`self.Shelf_Side_2`)))))