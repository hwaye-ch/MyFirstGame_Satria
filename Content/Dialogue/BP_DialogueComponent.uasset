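; Dialogue component that shows data-table-driven dialogue lines in an on-screen WBP_Dialogue widget.
; ShowDialogue looks up the given row, creates or updates the widget, stores the row's next table and returns its next code and end flag.
; A call made after an end-flagged row closes the widget instead of showing a line.
; ClearDialogue removes the widget and destroys the passed dialogue actor.
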(event `/Game/Blueprints/Interface/BPI_Dialogue.ClearDialogue`
  (params (DialogueActor :type "Actor Object Reference"))
  (bind _dialoguewidget (`self.DialogueWidget`))
  (`/Engine/EditorBlueprintResources/StandardMacros.IsValid` _dialoguewidget
    (:`Is Valid`
      (`Widget.RemoveFromParent` _dialoguewidget)
      (set `self.EndDialogue` false))
    (:`Is Not Valid`
      _))
  (set `self.DialogueWidget` null)
  (`/Engine/EditorBlueprintResources/StandardMacros.IsValid` DialogueActor
    (:`Is Valid`
      (`Actor.K2_DestroyActor` DialogueActor))))

(fn `ShowDialogue`
  (params (DialogueCode :type Name) (DialogueTable :type "DataTable Object Reference"))
  (returns (isEndOfDialogue :type Boolean) (NextDialogueCode :type Name))
  (set `self.Data Table` DialogueTable)
  (set `self.Row Name` DialogueCode)
  (if (`self.EndDialogue`)
    (`Widget.RemoveFromParent` (`self.DialogueWidget`))
    (set `self.EndDialogue` false)
    (set `self.DialogueWidget` null)
    (else
      (`/Engine/EditorBlueprintResources/StandardMacros.IsValid` (`self.DialogueWidget`)
        (:`Is Valid`
          (bind _returnvalue (`|GetDataTableRow` (`self.Data Table`) (`self.Row Name`))
            (:`then`
              (bind (_dialogue _row _datatable _enddialogue_) (break `/Game/Dialogue/Dialogue_Structure` _returnvalue))
              (`/Game/Dialogue/WBP_Dialogue.Update Dialogue` (`self.DialogueWidget`) _dialogue)
              (set `self.Row Name` _row)
              (set `self.Data Table` _datatable)
              (bind _output_get (set `self.EndDialogue` _enddialogue_))
              (return _output_get (stale _output_get_3)))
            (:`RowNotFound`
              (`KismetSystemLibrary.PrintString` "Row Not Found"))))
        (:`Is Not Valid`
          (bind _returnvalue_2 (`|GetDataTableRow` (`self.Data Table`) (`self.Row Name`))
            (:`then`
              (bind (_dialogue_2 _row_2 _datatable_2 _enddialogue__2) (break `/Game/Dialogue/Dialogue_Structure` _returnvalue_2))
              (bind _returnvalue_3 (`|CreateWidget` "/Game/Dialogue/WBP_Dialogue.WBP_Dialogue_C" null (`KismetTextLibrary.Conv_NameToText` (`self.Name`)) _dialogue_2))
              (bind _output_get_2 (set `self.DialogueWidget` _returnvalue_3))
              (`UserWidget.AddToViewport` _output_get_2 0)
              (bind _output_get_3 (set `self.Row Name` _row_2))
              (set `self.Data Table` _datatable_2)
              (set `self.EndDialogue` _enddialogue__2)
              (return _output_get _output_get_3))))))))