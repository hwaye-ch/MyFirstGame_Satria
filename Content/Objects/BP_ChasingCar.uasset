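; BP_ChasingCar is an AI car that stays dormant until triggered, then chases pawns it sees.
; A linked CarStartEnabler fires ActivateCar, which sets the chase flag and turns on two spotlights that are switched off at start.
; PawnSensing then drives AIMoveTo toward the seen pawn, while a sphere overlap with the first-person character only prints a hit message once.
; A looping random-roam event exists but is never triggered.
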(event `self.ReceiveBeginPlay`
  (bind _carstartenabler (`self.CarStartEnabler`))
  (`/Engine/EditorBlueprintResources/StandardMacros.IsValid` _carstartenabler
    (:`Is Valid`
      (add `/Game/Blueprints/Levels/Trigger_ChasingCar.CarStartChasing` _carstartenabler (delegate `Activate Car!`))
      (`self.Nyalakan Lampu` false))))

(event `Activate Car!`
  (bind _output_get (set `self.IsStartChasing` true))
  (`self.Nyalakan Lampu` _output_get))

(event `self.PawnSensing.OnSeePawn`
  (params (Pawn :type "Pawn Object Reference"))
  (if (`self.IsStartChasing`)
    (`|ExecutionSequence`
      (:`then_0`
        (`|AIMoveTo` self (0.0 0.0 0.0) Pawn)))))

(event `Random Roam`
  (`|AIMoveTo` self (`NavigationSystemV1.K2_GetRandomReachablePointInRadius` (`self.K2_GetActorLocation`) 2500.0 null null) null
    (:`OnSuccess`
      (`self.Random Roam`))))

(event `Nyalakan Lampu`
  (params (`Light On?` :type Boolean))
  (`SceneComponent.SetVisibility` (`self.SpotLight`) `Light On?` false)
  (`SceneComponent.SetVisibility` (`self.SpotLight2`) `Light On?` false))

(event `self.Sphere.OnComponentBeginOverlap`
  (params (OverlappedComponent :type "PrimitiveComponent Object Reference") (OtherActor :type "Actor Object Reference") (OtherComp :type "PrimitiveComponent Object Reference") (OtherBodyIndex :type Integer) (bFromSweep :type Boolean) (SweepResult :type "HitResult Structure (by ref)"))
  (cast `/Game/FirstPerson/Blueprints/BP_FirstPersonCharacter` OtherActor)
  (set `self.IsStartChasing` (`self.IsStartChasing`))
  (`/Engine/EditorBlueprintResources/StandardMacros.DoOnce` false
    (:`Completed`
      (`KismetSystemLibrary.PrintString` "the player is hit"))))

(fn `UserConstructionScript`)