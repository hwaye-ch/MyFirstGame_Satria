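; BP_InteractableDoor is a door actor that swings open and closed through its OpenDoor event.
; Each call flips the opened state, then plays or reverses the TL_Doors timeline, which interpolates the Door component's relative yaw between closed and a quarter turn.
; An IsOpening flag ignores repeat calls until the timeline finishes.
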(event `/Game/Blueprints/Interface/BPI_Interact.OpenDoor`
  (if (not (`self.IsOpening`))
    (set `self.IsOpening` true)
    (bind _output_get (set `self.IsDoorOpened` (not (`self.IsDoorOpened`))))
    (if _output_get
      (bind (_direction _door_alpha) (`Timeline|TL_Doors` :!label _label)
        (:`Update`
          (`SceneComponent.K2_SetRelativeRotation` (`self.Door`) (`KismetMathLibrary.MakeRotator` 0.0 0.0 (`KismetMathLibrary.Lerp` 0.0 90.0 _door_alpha)) false false))
        (:`Finished`
          (set `self.IsOpening` false)))
      (else
        (goto _label :!via `Reverse`)))))

(fn `UserConstructionScript`)